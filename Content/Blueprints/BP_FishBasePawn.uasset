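; Base fish pawn that rolls a random fish from DT_FishParameters and takes on its identity, mesh and material.
; GetFish filters rows by depth, map area, time and player fishing level, then picks randomly among those matching a curve-weighted rarity.
; CreateFish fills the stats and marks the local data copy as caught.
; Weight/length, sell value and CatchFish events are empty here.
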(event Custom|Create%20Fish
  (params (Row%20name :type Name) (Depth :type Integer))
  ;[1 1 1] Fills In fish Stats
  (Variables|Default|SetDepth Depth)
  (bind _returnvalue (Utilities|GetDataTableRow "/Game/DataAssets/DT_FishParameters.DT_FishParameters" Row%20name)
    (:then
      (bind _output_get (Variables|Default|SetFish%20Data _returnvalue))
      (Components|StaticMesh|SetStaticMesh (Variables|Default|GetFIsh%20Mesh) (.FIshMesh (Utilities|Struct|BreakS_Fish _output_get)))
      (Rendering|Material|SetMaterial (Variables|Default|GetFIsh%20Mesh) 0 (.FishMaterial (Utilities|Struct|BreakS_Fish _output_get)))
      (Variables|Default|SetFish%20Name (.Name (Utilities|Struct|BreakS_Fish _output_get)))
      (Variables|Default|SetRarity (.Rarity (Utilities|Struct|BreakS_Fish _output_get)))
      (Variables|Default|SetFishing%20Level (.FishingLevel (Utilities|Struct|BreakS_Fish _output_get)))
      (Variables|Default|SetDifficulty (.Difficulty (Utilities|Struct|BreakS_Fish _output_get)))
      (CallFunction|GenerateWeightandLength (.MinLength (Utilities|Struct|BreakS_Fish _output_get)) (.MaxLength (Utilities|Struct|BreakS_Fish _output_get)) (.MinWeight (Utilities|Struct|BreakS_Fish _output_get)) (.MaxWeight (Utilities|Struct|BreakS_Fish _output_get)))
      (CallFunction|CalculateSellValue)
      (if (not (.Caught (Utilities|Struct|BreakS_Fish _output_get)))
        (Variables|Default|SetFish%20Data (Utilities|Struct|MakeS_Fish (.ID (Utilities|Struct|BreakS_Fish _output_get)) (.FIshMesh (Utilities|Struct|BreakS_Fish _output_get)) (.FishMaterial (Utilities|Struct|BreakS_Fish _output_get)) (.FishIcon (Utilities|Struct|BreakS_Fish _output_get)) (.Name (Utilities|Struct|BreakS_Fish _output_get)) (.Rarity (Utilities|Struct|BreakS_Fish _output_get)) (.Depth (Utilities|Struct|BreakS_Fish _output_get)) (.MapArea (Utilities|Struct|BreakS_Fish _output_get)) (.Time (Utilities|Struct|BreakS_Fish _output_get)) (.FishingLevel (Utilities|Struct|BreakS_Fish _output_get)) (.Difficulty (Utilities|Struct|BreakS_Fish _output_get)) (.MinLength (Utilities|Struct|BreakS_Fish _output_get)) (.MinWeight (Utilities|Struct|BreakS_Fish _output_get)) (.MaxLength (Utilities|Struct|BreakS_Fish _output_get)) (.MaxWeight (Utilities|Struct|BreakS_Fish _output_get)) true))))))

(event Custom|Catch%20Fish)

(event Custom|Get%20Fish
  (params (Depth :type Integer) (Area :type Integer) (Time :type Integer) (Fishing%20Level :type Integer))
  ;[1 1 1] Creates an array of fish that will spawn in a specified depth, area, and time as well as under the players fishing level
  (bind _outrownames (DataTable|GetDataTableRowNames "/Game/DataAssets/DT_FishParameters.DT_FishParameters"))
  (Utilities|Array|Clear (Variables|Default|GetFishTypeRowNameArr))
  (for _array_element _outrownames
    (bind _returnvalue (Utilities|GetDataTableRow "/Game/DataAssets/DT_FishParameters.DT_FishParameters" _array_element)
      (:then
        (if (Math|Boolean|ANDBoolean (Utilities|Array|Get(acopy) (.Depth (Utilities|Struct|BreakS_Fish _returnvalue)) Depth) (Utilities|Array|Get(acopy) (.MapArea (Utilities|Struct|BreakS_Fish _returnvalue)) Area) (Utilities|Array|Get(acopy) (.Time (Utilities|Struct|BreakS_Fish _returnvalue)) Time) (<= (.FishingLevel (Utilities|Struct|BreakS_Fish _returnvalue)) Fishing%20Level))
          (Utilities|Array|Add (Variables|Default|GetFishTypeRowNameArr) _array_element)))))
  ;[1 1 1] Compiles an array of a random rarity selected from a curve
  (Variables|Default|SetRandomRarity (Math|Float|Round (Math|Curves|GetFloatValue (Variables|Default|GetFIshCurve) (Math|Random|RandomFloat))))
  (Utilities|Array|Clear (Variables|Default|GetFishRarityArr))
  (for _array_element_2 (Variables|Default|GetFishTypeRowNameArr)
    (bind _returnvalue_2 (Utilities|GetDataTableRow "/Game/DataAssets/DT_FishParameters.DT_FishParameters" _array_element_2)
      (:then
        (if (== (Variables|Default|GetRandomRarity) (.Rarity (Utilities|Struct|BreakS_Fish _returnvalue_2)))
          (Utilities|Array|Add (Variables|Default|GetFishRarityArr) _array_element_2)))))
  ;[1 1 1] Chooses a random fish from an array of specified fish
  (CallFunction|CreateFish (Utilities|Array|Get(acopy) (Variables|Default|GetFishRarityArr) (Math|Random|RandomIntegerinRange 0 (- (Utilities|Array|Length (Variables|Default|GetFishRarityArr)) 1)))))

(event Custom|Generate%20Weight%20and%20Length
  (params (MinLength :type Float%20%28double-precision%29) (MaxLength :type Float%20%28double-precision%29) (MinWeight :type Float%20%28double-precision%29) (MaxWeight :type Float%20%28double-precision%29)))

(event Custom|Calculate%20Sell%20Value)

(fn ConstructionScript)