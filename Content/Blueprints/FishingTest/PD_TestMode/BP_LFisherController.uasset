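; Player controller for the fishing game that owns the player's UI and menu input.
; BeginPlay adds the boat input context, then after a short delay creates pause, shop, player menu, sell and weekly quota widgets, passing the quota HUD to BP_WeeklyQuotaManager.
; Enhanced Input opens pause and toggles inventory; placeholder hard-coded keys toggle map, Fishopedia and options tabs or open the shop.
; Minigame context switching and actual game pausing are unconnected.
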(event Input|EnhancedActionEvents|EnhancedInputActionIA_Pause
  (params (ActionValue :type Boolean) (ElapsedSeconds :type Float%20%28double-precision%29) (TriggeredSeconds :type Float%20%28double-precision%29) (InputAction :type Input%20Action%20Object%20Reference :default "/Game/Input/IA_Pause.IA_Pause"))
  ;[1 1 1] Pause
  (:Started
    (UserInterface|Viewport|AddtoViewport (Variables|Default|GetPauseMenuUI) 0)))

(event Input|EnhancedActionEvents|EnhancedInputActionIA_InputSequenceTest
  (params (ActionValue :type Boolean) (ElapsedSeconds :type Float%20%28double-precision%29) (TriggeredSeconds :type Float%20%28double-precision%29) (InputAction :type Input%20Action%20Object%20Reference :default "/Game/Input/SequenceMinigame/IA_InputSequenceTest.IA_InputSequenceTest"))
  ;[1 1 1] Input Sequence Minigame
)

(event Input|EnhancedActionEvents|EnhancedInputActionIA_InventoryToggle
  (params (ActionValue :type Boolean) (ElapsedSeconds :type Float%20%28double-precision%29) (TriggeredSeconds :type Float%20%28double-precision%29) (InputAction :type Input%20Action%20Object%20Reference :default "/Game/Input/Boat/IA_InventoryToggle.IA_InventoryToggle"))
  (bind _playermenuui (Variables|Default|GetPlayerMenuUI))
  (:Started
    ;[1 1 1] Player Menu (Switching to correct canvas panel when opening widget)
    ;;[1 1 1] Inventory Widget
    (Utilities|IsValid _playermenuui
      (:Is%20Valid
        (Utilities|FlowControl|FlipFlop
          (:A
            (Widget|RemovefromParent _playermenuui))
          (:B
            (UserInterface|Viewport|AddtoViewport _playermenuui 0)
            ;;;[1 1 1] Tab 0 = Inventory
            (Default|SwitchTab _playermenuui))))
      (:Is%20Not%20Valid
        (Development|PrintString "Player Menus Widget Creation Invalid")))))

(event EventBeginPlay
  (bind _returnvalue (PlayerController|LocalPlayerSubsystems|GetEnhancedInputLocalPlayerSubsystem))
  (bind _self self)
  ;[1 1 1] Setup
  (Utilities|IsValid _returnvalue
    (:Is%20Valid
      (Input|AddMappingContext _returnvalue "/Game/Input/Boat/IMC_Boat.IMC_Boat" 0 "(bIgnoreAllPressedKeysUntilRelease=True,bForceImmediately=False,bNotifyUserSettings=False)")
      (Utilities|FlowControl|Delay 0.2)
      (Utilities|FlowControl|Sequence
        (:then_0
          (bind _returnvalue_2 (UserInterface|CreateWidget "/Game/UI/MenuPrototypes/WBP_PauseMenu.WBP_PauseMenu_C" _self))
          (Variables|Default|SetPauseMenuUI _returnvalue_2))
        (:then_1
          (bind _returnvalue_3 (UserInterface|CreateWidget "/Game/UI/Shop/WBP_ShopMenu.WBP_ShopMenu_C" _self))
          (bind _output_get (Variables|Default|SetShopUI _returnvalue_3))
          (UserInterface|Viewport|AddtoViewport _output_get 0)
          (Widget|SetVisibility _output_get "Hidden")
          (Default|Initialise _output_get))
        (:then_2
          (bind _returnvalue_4 (UserInterface|CreateWidget "/Game/UI/MenuPrototypes/WBP_PlayerMenu.WBP_PlayerMenu_C" _self))
          (bind _output_get_2 (Variables|Default|SetPlayerMenuUI _returnvalue_4))
          (Default|Initialize _output_get_2 self))
        (:then_3
          (bind _returnvalue_5 (UserInterface|CreateWidget "/Game/Blueprints/WeeklyQuota/WBP_WeeklyQuotaHUD.WBP_WeeklyQuotaHUD_C" _self))
          (bind _output_get_3 (Variables|Default|SetWeeklyQuotaUI _returnvalue_5))
          (UserInterface|Viewport|AddtoViewport _output_get_3 0)
          (bind _returnvalue_6 (Actor|GetActorOfClass "/Game/Blueprints/WeeklyQuota/BP_WeeklyQuotaManager.BP_WeeklyQuotaManager_C"))
          (Default|Initialise _returnvalue_6 _output_get_3))
        (:then_4
          (bind _returnvalue_7 (UserInterface|CreateWidget "/Game/UI/Shop/WBP_SellUI.WBP_SellUI_C" _self))
          (bind _output_get_4 (Variables|Default|SetSellUI _returnvalue_7))
          (UserInterface|Viewport|AddtoViewport _output_get_4 0)
          (Widget|SetVisibility _output_get_4 "Hidden")
          (Default|Initialise _output_get_4 self))))
    (:Is%20Not%20Valid
      (Development|PrintString "EILPS Not Valid"))))

(event Input|KeyboardEvents|Q
  (params (Key :type Key%20Structure :default "None"))
  (bind _shopui (Variables|Default|GetShopUI))
  ;[0 1 0] Open Shop - USE THIS LOGIC FOR OPENING SHOP WHEN ENTERING TOWN
  (:Pressed
    (Widget|SetVisibility _shopui "Visible")
    (Input|SetInputModeUIOnly self _shopui "DoNotLock" true)
    (Variables|Default|SetbShowMouseCursor true)))

(event Input|KeyboardEvents|M
  (params (Key :type Key%20Structure :default "None"))
  (bind _playermenuui (Variables|Default|GetPlayerMenuUI))
  ;[1 1 1] Player Menu (Switching to correct canvas panel when opening widget)
  ;;[1 1 1] Map Widget
  ;;;[1 0.2594 0.2594] Replace with IMC input
  (:Pressed
    (Utilities|IsValid _playermenuui
      (:Is%20Valid
        (if (UserInterface|Viewport|IsinViewport _playermenuui)
          (Widget|RemovefromParent _playermenuui)
          (else
            (UserInterface|Viewport|AddtoViewport _playermenuui 0)
            ;;;[1 1 1] Tab 1 = Map
            (Default|SwitchTab _playermenuui 1))))
      (:Is%20Not%20Valid
        (Development|PrintString "Player Menus Widget Creation Invalid")))))

(event Input|KeyboardEvents|O
  (params (Key :type Key%20Structure :default "None"))
  (bind _playermenuui (Variables|Default|GetPlayerMenuUI))
  ;[1 1 1] Player Menu (Switching to correct canvas panel when opening widget)
  ;;[1 1 1] Options Widget
  ;;;[1 0.2594 0.2594] Replace with IMC input
  (:Pressed
    (Utilities|IsValid _playermenuui
      (:Is%20Valid
        (if (UserInterface|Viewport|IsinViewport _playermenuui)
          (Widget|RemovefromParent _playermenuui)
          (else
            (UserInterface|Viewport|AddtoViewport _playermenuui 0)
            ;;;[1 1 1] Tab 4 = Options
            (Default|SwitchTab _playermenuui 3))))
      (:Is%20Not%20Valid
        (Development|PrintString "Player Menus Widget Creation Invalid")))))

(event Input|KeyboardEvents|B
  (params (Key :type Key%20Structure :default "None"))
  (bind _playermenuui (Variables|Default|GetPlayerMenuUI))
  ;[1 1 1] Player Menu (Switching to correct canvas panel when opening widget)
  ;;[1 1 1] Fishopedia Widget
  ;;;[1 0.2594 0.2594] Replace with IMC input
  (:Pressed
    (Utilities|IsValid _playermenuui
      (:Is%20Valid
        (if (UserInterface|Viewport|IsinViewport _playermenuui)
          (Widget|RemovefromParent _playermenuui)
          (else
            (UserInterface|Viewport|AddtoViewport _playermenuui 0)
            ;;;[1 1 1] Tab 3 = Fishopedia
            (Default|SwitchTab _playermenuui 2))))
      (:Is%20Not%20Valid
        (Development|PrintString "Player Menus Widget Creation Invalid")))))

(event Input|KeyboardEvents|I
  (params (Key :type Key%20Structure :default "None"))
  ;[1 1 1] Player Menu (Switching to correct canvas panel when opening widget)
  ;;[1 1 1] Inventory Widget
  ;;;[1 0.2594 0.2594] Replace with IMC input
)

(fn ConstructionScript)