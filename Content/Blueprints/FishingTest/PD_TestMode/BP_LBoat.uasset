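; Player-controlled boat pawn for the fishing test mode that spawns and carries a fishing manager pawn at its attach point.
; Enhanced Input drives movement and yaw steering, flipping steering when reversing, while a timeline eases clamped spring-arm zoom.
; Switching perspective blends the view to the fisher, then possesses it and swaps the boat mapping context for the fishing one.
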(event Input|EnhancedActionEvents|EnhancedInputActionIA_SwitchPerspective
  (params (ActionValue :type Boolean) (ElapsedSeconds :type Float%20%28double-precision%29) (TriggeredSeconds :type Float%20%28double-precision%29) (InputAction :type Input%20Action%20Object%20Reference :default "/Game/Input/IA_SwitchPerspective.IA_SwitchPerspective"))
  (bind _returnvalue (Game|GetPlayerController 0))
  (bind _fisher (Variables|Default|GetFisher))
  (bind _returnvalue_2 (PlayerController|LocalPlayerSubsystems|GetEnhancedInputLocalPlayerSubsystem _returnvalue))
  ;[1 1 1] Change to Fisher Perspective
  (Utilities|IsValid _returnvalue
    (:Is%20Valid
      (Game|Player|SetViewTargetwithBlend _returnvalue _fisher 0.5 "VTBlend_EaseInOut" 2.0 false)
      (Utilities|FlowControl|Delay 0.5)
      (Pawn|Possess _returnvalue _fisher)
      (Utilities|IsValid _returnvalue_2
        (:Is%20Valid
          (Input|RemoveMappingContext _returnvalue_2 "/Game/Input/Boat/IMC_Boat.IMC_Boat" "(bIgnoreAllPressedKeysUntilRelease=True,bForceImmediately=False,bNotifyUserSettings=False)")
          (Input|AddMappingContext _returnvalue_2 "/Game/Input/Fishing/IMC_Fishing.IMC_Fishing" 0 "(bIgnoreAllPressedKeysUntilRelease=True,bForceImmediately=False,bNotifyUserSettings=False)"))))))

(event Input|EnhancedActionEvents|EnhancedInputActionIA_BoatZoom
  (params (ActionValue :type Float%20%28double-precision%29) (ElapsedSeconds :type Float%20%28double-precision%29) (TriggeredSeconds :type Float%20%28double-precision%29) (InputAction :type Input%20Action%20Object%20Reference :default "/Game/Input/Boat/IA_BoatZoom.IA_BoatZoom"))
  ;[1 1 1] Camera Zoom
  (if (not (Variables|Default|GetZoomInProgress?))
    (Variables|Default|SetZoomInProgress? true)
    (bind _alpha (Timeline|Zoom PlayFromStart)
      (:Update
        (Variables|/Script/Engine.SpringArmComponent|SetTargetArmLength (Variables|Default|GetSpringArm) (Math|Float|Lerp (Variables|/Script/Engine.SpringArmComponent|GetTargetArmLength (Variables|Default|GetSpringArm)) (Math|Float|Clamp(Float) (- (Variables|/Script/Engine.SpringArmComponent|GetTargetArmLength (Variables|Default|GetSpringArm)) (Variables|Default|GetZoomMultiplier)) (Variables|Default|GetMinCamLength) (Variables|Default|GetMaxCamLength)) _alpha)))
      (:Finished
        (Variables|Default|SetZoomInProgress? false)))))

(event Input|EnhancedActionEvents|EnhancedInputActionIA_BoatMove
  (params (ActionValue :type Float%20%28double-precision%29) (ElapsedSeconds :type Float%20%28double-precision%29) (TriggeredSeconds :type Float%20%28double-precision%29) (InputAction :type Input%20Action%20Object%20Reference :default "/Game/Input/Boat/IA_BoatMove.IA_BoatMove"))
  ;[1 1 1] Forward/Backward Movement
  (Pawn|Input|AddMovementInput (Math|Vector|RotateVector (Math|Vector|MakeVector ActionValue 0.0 0.0) (Transformation|GetActorRotation)) (* (Variables|Default|GetMovementMultiplier) (Utilities|Time|GetWorldDeltaSeconds)) false)
  (Variables|Default|SetReversing (< ActionValue 0.0)))

(event Input|EnhancedActionEvents|EnhancedInputActionIA_BoatLook
  (params (ActionValue :type Float%20%28double-precision%29) (ElapsedSeconds :type Float%20%28double-precision%29) (TriggeredSeconds :type Float%20%28double-precision%29) (InputAction :type Input%20Action%20Object%20Reference :default "/Game/Input/Boat/IA_BoatLook.IA_BoatLook"))
  ;[1 1 1] Left/Right Turning
  (Pawn|Input|AddControllerYawInput (* ActionValue (Variables|Default|GetSteeringMultiplier) (Utilities|Time|GetWorldDeltaSeconds) (Math|Float|SelectFloat -1.0 1.0 (Variables|Default|GetReversing)))))

(event EventBeginPlay
  (bind _fisherattachpoint (Variables|Default|GetFisherAttachPoint))
  ;[1 1 1] Spawn Fisher
  (Utilities|FlowControl|Sequence
    (:then_0
      (bind _returnvalue (Game|SpawnActorfromClass "/Game/Blueprints/FishingTest/BP_FishingMgr5.BP_FishingMgr5_C" (Transformation|GetWorldTransform _fisherattachpoint) "AlwaysSpawn" "MultiplyWithRoot" 0 0))
      (bind _output_get (Variables|Default|SetFisher _returnvalue))
      (Transformation|AttachComponentToComponent _output_get _fisherattachpoint "None" "SnapToTarget" "SnapToTarget" "SnapToTarget" true)
      (Variables|/Game/Blueprints/FishingTest/BP_FishingMgr5.BP_FishingMgr5_C|SetBoat _output_get self))
    (:then_1
      (Variables|/Game/Blueprints/FishingTest/Components/BPC_FishingCamera.BPC_FishingCamera_C|SetCameraArm (Variables|Default|GetFishingCamera) (Variables|Default|GetSpringArm)))))

(fn ConstructionScript)