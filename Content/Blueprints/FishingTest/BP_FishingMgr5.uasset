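; BP_FishingMgr5 runs the player's fishing mode: aiming, casting and recalling a bobber, with a switch back to possessing the boat.
; A FishingState machine and a timed transition lock gate Enhanced Input actions.
; Holding cast drives a meter timeline that places the target indicator by downward trace.
; Release launches the bobber along a runtime-built spline; impact enables fish overlap colliders, and recall reverses the flight.
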(event Custom|Bobber%20Impact
  (bind _fishinterestcollider (Variables|Default|GetFishInterestCollider))
  ;[0.3341 0.3003 1 1 56] Bobber hits water
  (Utilities|FlowControl|Sequence
    (:then_0
      (Niagara|SpawnSystematLocation "/Game/VFX/NS_Sploosh.NS_Sploosh" (Transformation|GetWorldLocation (Variables|Default|GetFishTargetIndicator))) ; Visual fx/anims
      (Audio|Components|Audio|Play (Variables|Default|GetBobberAudio) 0.0)
      (Audio|PlaySound2D "/Game/Audio/WaterSplish.WaterSplish" 1.0 1.0 0.0 0 0))
    (:then_1
      (Variables|States|SetFishing%20State "NewEnumerator4")
      (Transformation|SetWorldLocation _fishinterestcollider (Transformation|GetWorldLocation (Variables|Default|GetBobber)) false false)
      (Variables|/Script/Engine.PrimitiveComponent|SetbGenerateOverlapEvents _fishinterestcollider true)
      (Variables|/Script/Engine.PrimitiveComponent|SetbGenerateOverlapEvents (Variables|Default|GetFishBiteCollider) true))))

(event Custom|Begin%20Transitioning
  (params (Duration :type Float%20%28double-precision%29))
  ;[0.424 0.07502 0.08093] [ Input disable transitions ]
  (Variables|States|SetMidTransition true)
  (Utilities|Time|SetTimerbyEvent (delegate Custom|End%20Transition) Duration))

(event Custom|CastRod
  (bind _bobberspline (Variables|Default|GetBobberSpline))
  ;[0.2147 0.3632 1] Casting away
  (if (Variables|States|GetValidRodPos) ; TODO: ensure cursor is in valid position
    (Variables|States|SetFishing%20State "NewEnumerator1")
    (Utilities|FlowControl|Sequence
      (:then_0
        (Spline|ClearSplinePoints _bobberspline true)
        (Spline|AddSplinePoint _bobberspline (Math|Vector|MakeVector 0.0 0.0 0.0) "Local" true)
        (Spline|AddSplinePoint _bobberspline (Transformation|GetWorldLocation (Variables|Default|GetFishTargetIndicator)) "World" true)
        (Spline|SetTangentatSplinePoint _bobberspline 0 (Math|Vector|MakeVector 0.0 0.0 6e+02) "World" true)
        (Spline|SetTangentatSplinePoint _bobberspline 1 (Math|Vector|MakeVector 0.0 0.0 0.0) "World" true))
      (:then_1
        (CallFunction|StopAiming)
        (CallFunction|AnimateBobberLaunch false))
      (:then_2
        (CallFunction|BeginTransitioning 1.0)
        (Audio|PlaySound2D "/Game/Audio/RodSwoosh.RodSwoosh" 1.0 1.0 0.0 0 0)))))

(event Custom|RecallRod
  ;[0.6769 0.31 1] Recalling rod
  (Variables|/Script/Engine.PrimitiveComponent|SetbGenerateOverlapEvents (Variables|Default|GetFishBiteCollider) false)
  (Variables|/Script/Engine.PrimitiveComponent|SetbGenerateOverlapEvents (Variables|Default|GetFishInterestCollider) false)
  (CallFunction|BeginTransitioning 1.0)
  (CallFunction|AnimateBobberLaunch true)
  (Variables|States|SetFishing%20State "NewEnumerator0")
  (Transformation|SetRelativeLocation (Variables|Default|GetFishTargetIndicator) "0, 0, 0" false false))

(event Custom|AnimateBobberLaunch
  (params (Backwards :type Boolean))
  (if Backwards
    (bind (_direction _dist) (Timeline|Launch%20Bobber%20on%20Spline ReverseFromEnd)
      (:Update
        (Transformation|SetWorldLocation (Variables|Default|GetBobber) (Spline|GetLocationatTime (Variables|Default|GetBobberSpline) _dist "World" false) false false))
      (:Finished
        (if (Utilities|Enum|Equal(Enum) _direction "Forward")
          (CallFunction|BobberImpact)
          (else
            (Audio|Components|Audio|Stop (Variables|Default|GetBobberAudio))))))
    (else
      (Timeline|Launch%20Bobber%20on%20Spline PlayFromStart))))

(event Custom|StartAiming
  (bind _camera (Variables|Default|GetCamera))
  ;[0.3338 1 0.7006] Selecting a fishing spot
  (Widget|SetVisibility (Variables|UI|GetCastMeter) "Visible")
  (bind _scale (Timeline|Choose%20Fishing%20Distance PlayFromStart)
    (:Update
      (Default|SetGaugePercent (Variables|UI|GetCastMeter) _scale)
      (bind (_outhit _returnvalue) (Collision|LineTraceByChannel (+ (* (Math|Vector|GetForwardVector _camera) (Math|Float|Lerp (Variables|FishCatching|GetMinimum%20Cast%20Range) (Variables|FishCatching|GetMaximum%20Cast%20Range) _scale)) "0.000000,0.000000,5000.000000" (Transformation|GetWorldLocation _camera)) (- (+ (* (Math|Vector|GetForwardVector _camera) (Math|Float|Lerp (Variables|FishCatching|GetMinimum%20Cast%20Range) (Variables|FishCatching|GetMaximum%20Cast%20Range) _scale)) "0.000000,0.000000,5000.000000" (Transformation|GetWorldLocation _camera)) "0.000000,0.000000,10000.000000") "TraceTypeQuery1" false 0 "None" true "(R=50.000000,G=22.712761,B=0.000000,A=1.000000)" "(R=0.000000,G=0.000000,B=0.000000,A=0.000000)"))
      (Variables|States|SetValidRodPos _returnvalue) ; TODO: rewrite to ensure the surface is fishable
      (Transformation|SetWorldLocation (Variables|Default|GetFishTargetIndicator) (+ (.Location (Collision|BreakHitResult _outhit)) "0.000000,0.000000,1.000000") false false))))

(event Custom|FishShowoff
  (params (Fish :type BP%20Fish%20Pawn%20Object%20Reference))
  (Variables|States|SetFishing%20State "NewEnumerator6")
  (Development|PrintString "well done!")
  (Utilities|FlowControl|Delay 2.0)
  (Actor|DestroyActor Fish)
  (Variables|States|SetFishing%20State "NewEnumerator0"))

(event Custom|FishEscape
  (params (Fish :type BP%20Fish%20Pawn%20Object%20Reference))
  (Variables|States|SetFishing%20State "NewEnumerator5")
  (Development|PrintString "you fucked up")
  (Utilities|FlowControl|Delay 2.0)
  (Variables|States|SetFishing%20State "NewEnumerator0"))

(event Custom|End%20Transition
  ;[0.424 0.07502 0.08093] [ Input disable transitions ]
  (Variables|States|SetMidTransition false))

(event Custom|SetCameraMode
  (params (IsOverhead :type Boolean))
  (bind _springarm (Variables|Default|GetSpringArm))
  (bind _relativerotation (Variables|/Script/Engine.SceneComponent|GetRelativeRotation _springarm))
  (if IsOverhead
    (bind (_direction _springarmlength _springarmangle) (Timeline|TransitionCameraPerspective PlayFromStart)
      (:Update
        (Variables|/Script/Engine.SpringArmComponent|SetTargetArmLength _springarm _springarmlength)
        (Transformation|SetRelativeRotation _springarm (Math|Rotator|MakeRotator (.roll _relativerotation) _springarmangle (.yaw _relativerotation)) false false)))
    (else
      (Timeline|TransitionCameraPerspective ReverseFromEnd))))

(event Custom|StopAiming
  (bind _camera (Variables|Default|GetCamera))
  ;[0.3338 1 0.7006] Selecting a fishing spot
  (Widget|SetVisibility (Variables|UI|GetCastMeter) "Hidden")
  (bind _scale (Timeline|Choose%20Fishing%20Distance Stop)
    (:Update
      (Default|SetGaugePercent (Variables|UI|GetCastMeter) _scale)
      (bind (_outhit _returnvalue) (Collision|LineTraceByChannel (+ (* (Math|Vector|GetForwardVector _camera) (Math|Float|Lerp (Variables|FishCatching|GetMinimum%20Cast%20Range) (Variables|FishCatching|GetMaximum%20Cast%20Range) _scale)) "0.000000,0.000000,5000.000000" (Transformation|GetWorldLocation _camera)) (- (+ (* (Math|Vector|GetForwardVector _camera) (Math|Float|Lerp (Variables|FishCatching|GetMinimum%20Cast%20Range) (Variables|FishCatching|GetMaximum%20Cast%20Range) _scale)) "0.000000,0.000000,5000.000000" (Transformation|GetWorldLocation _camera)) "0.000000,0.000000,10000.000000") "TraceTypeQuery1" false 0 "None" true "(R=50.000000,G=22.712761,B=0.000000,A=1.000000)" "(R=0.000000,G=0.000000,B=0.000000,A=0.000000)"))
      (Variables|States|SetValidRodPos _returnvalue) ; TODO: rewrite to ensure the surface is fishable
      (Transformation|SetWorldLocation (Variables|Default|GetFishTargetIndicator) (+ (.Location (Collision|BreakHitResult _outhit)) "0.000000,0.000000,1.000000") false false))))

(event Input|EnhancedActionEvents|EnhancedInputActionIA_FishCast
  (params (ActionValue :type Boolean) (ElapsedSeconds :type Float%20%28double-precision%29) (TriggeredSeconds :type Float%20%28double-precision%29) (InputAction :type Input%20Action%20Object%20Reference :default "/Game/Input/Fishing/IA_FishCast.IA_FishCast"))
  (bind _midtransition (Variables|States|GetMidTransition))
  (bind _returnvalue (not _midtransition))
  ;[0.08179 1 0.06473 1 56] Casting rod (left click)
  (:Started
    (if _returnvalue
      (switch Utilities|FlowControl|Switch|SwitchonE_FishingStates (Variables|States|GetFishing%20State)
        (:NewEnumerator0
          (Variables|States|SetFishing%20State "NewEnumerator7")
          (CallFunction|StartAiming))
        (:NewEnumerator4
          (CallFunction|RecallRod)))))
  (:Completed
    (if _returnvalue
      (switch Utilities|FlowControl|Switch|SwitchonE_FishingStates (Variables|States|GetFishing%20State)
        (:NewEnumerator7
          (CallFunction|StopAiming)
          (CallFunction|CastRod))))))

(event Input|EnhancedActionEvents|EnhancedInputActionIA_FishLook
  (params (ActionValue :type Vector%202D%20Structure) (ElapsedSeconds :type Float%20%28double-precision%29) (TriggeredSeconds :type Float%20%28double-precision%29) (InputAction :type Input%20Action%20Object%20Reference :default "/Game/Input/Fishing/IA_FishLook.IA_FishLook"))
  (bind _fishing_state (Variables|States|GetFishing%20State))
  (bind _camera (Variables|Default|GetCamera))
  (bind _campivot (Variables|Default|GetCamPivot))
  (bind _returnvalue (Utilities|CalculateLookAmount _campivot (.x ActionValue)))
  ;[0.3338 1 0.7006] Selecting a fishing spot
  (if (or (Utilities|Enum|Equal(Enum) _fishing_state "NewEnumerator7") (Utilities|Enum|Equal(Enum) _fishing_state "NewEnumerator0"))
    (Pawn|Input|AddControllerYawInput _returnvalue)
    (Transformation|AddRelativeRotation _campivot (Math|Rotator|MakeRotator 0.0 0.0 _returnvalue) false false)
    (bind (_outhit _returnvalue_2) (Collision|LineTraceByChannel (+ (* (Math|Vector|GetForwardVector _camera) (Math|Float|Lerp (Variables|FishCatching|GetMinimum%20Cast%20Range) (Variables|FishCatching|GetMaximum%20Cast%20Range) (stale Custom|StartAiming _scale))) "0.000000,0.000000,5000.000000" (Transformation|GetWorldLocation _camera)) (- (+ (* (Math|Vector|GetForwardVector _camera) (Math|Float|Lerp (Variables|FishCatching|GetMinimum%20Cast%20Range) (Variables|FishCatching|GetMaximum%20Cast%20Range) (stale Custom|StartAiming _scale))) "0.000000,0.000000,5000.000000" (Transformation|GetWorldLocation _camera)) "0.000000,0.000000,10000.000000") "TraceTypeQuery1" false 0 "None" true "(R=50.000000,G=22.712761,B=0.000000,A=1.000000)" "(R=0.000000,G=0.000000,B=0.000000,A=0.000000)"))
    (Variables|States|SetValidRodPos _returnvalue_2) ; TODO: rewrite to ensure the surface is fishable
    (Transformation|SetWorldLocation (Variables|Default|GetFishTargetIndicator) (+ (.Location (Collision|BreakHitResult _outhit)) "0.000000,0.000000,1.000000") false false)))

(event Input|EnhancedActionEvents|EnhancedInputActionIA_SwitchPerspective
  (params (ActionValue :type Boolean) (ElapsedSeconds :type Float%20%28double-precision%29) (TriggeredSeconds :type Float%20%28double-precision%29) (InputAction :type Input%20Action%20Object%20Reference :default "/Game/Input/IA_SwitchPerspective.IA_SwitchPerspective"))
  (bind _returnvalue (Game|GetPlayerController 0))
  (bind _boat (Variables|Default|GetBoat))
  (bind _returnvalue_2 (PlayerController|LocalPlayerSubsystems|GetEnhancedInputLocalPlayerSubsystem _returnvalue))
  ;[1 1 1] Switch Perspective back to Boat
  (:Started
    (if (and (Utilities|Enum|Equal(Enum) (Variables|States|GetFishing%20State) "NewEnumerator0") (not (Variables|States|GetMidTransition)))
      (Utilities|IsValid _returnvalue
        (:Is%20Valid
          (Game|Player|SetViewTargetwithBlend _returnvalue _boat 0.5 "VTBlend_EaseInOut" 2.0 false)
          (Utilities|FlowControl|Delay 0.5)
          (Pawn|Possess _returnvalue _boat)
          (Utilities|IsValid _returnvalue_2
            (:Is%20Valid
              (Input|RemoveMappingContext _returnvalue_2 "/Game/Input/Fishing/IMC_Fishing.IMC_Fishing" "(bIgnoreAllPressedKeysUntilRelease=True,bForceImmediately=False,bNotifyUserSettings=False)")
              (Input|AddMappingContext _returnvalue_2 "/Game/Input/Boat/IMC_Boat.IMC_Boat" 0 "(bIgnoreAllPressedKeysUntilRelease=True,bForceImmediately=False,bNotifyUserSettings=False)"))))))))

(event EventBeginPlay
  (Utilities|FlowControl|Sequence
    (:then_0
      (bind _returnvalue (Game|ConstructObjectfromClass "/Game/UI/WB_CastMeter.WB_CastMeter_C"))
      (bind _output_get (Variables|UI|SetCastMeter _returnvalue))
      (UserInterface|Viewport|AddtoViewport _output_get 0)
      (Widget|SetVisibility _output_get "Hidden")
      (Input|SetInputModeGameOnly (Game|GetPlayerController 0) false))
    (:then_1
      (bind _returnvalue_2 (Audio|CreateSound2D "/Game/Audio/Loop_Bobbing.Loop_Bobbing" 1.0 1.0 0.0 0 false false))
      (bind _output_get_2 (Variables|Default|SetBobberAudio _returnvalue_2))
      (Audio|Components|Audio|Stop _output_get_2)
      (Class|GameplayStatics|PrimeSound "/Game/Audio/RodSwoosh.RodSwoosh")
      (Class|GameplayStatics|PrimeSound "/Game/Audio/WaterSplish.WaterSplish"))
    (:then_2
      (Development|PrintString "I am fishingmanager5!" true true "(R=1.000000,G=0.039631,B=0.689501,A=1.000000)"))))

(fn ConstructionScript)