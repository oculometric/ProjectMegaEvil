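; Prototype fisher pawn for testing fishing: aim, cast, wait for a bite, fight the fish, or switch back to the boat.
; A timeline drives the cast meter and range, and a downward trace places the target indicator.
; The bobber flies along a runtime-built spline, then a random timer triggers the bite.
; The placeholder minigame swaps cameras and moves a draining gauge by clicks, scored on indicator-bobber overlap, until catch or failure.
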(event OnComponentBeginOverlap(FishDetectorCol)
  (params (OverlappedComponent :type Primitive%20Component%20Object%20Reference) (OtherActor :type Actor%20Object%20Reference) (OtherComp :type Primitive%20Component%20Object%20Reference) (OtherBodyIndex :type Integer) (bFromSweep :type Boolean) (SweepResult :type Hit%20Result%20Structure%20%28by%20ref%29))
  (Utilities|Casting|CastToBP_FishPawn OtherActor)
  (Development|PrintString "FISJ!") ; Overlapping a fish!
)

(event Custom|Bobber%20Impact
  ;[0.3341 0.3003 1 1 56] Bobber hits water
  (Utilities|FlowControl|Sequence
    (:then_0
      (Niagara|SpawnSystematLocation "/Game/VFX/NS_Sploosh.NS_Sploosh" (Transformation|GetWorldLocation (Variables|Default|GetFishTargetIndicator))) ; Visual fx/anims
      (Variables|/Script/Engine.PrimitiveComponent|SetbGenerateOverlapEvents (Variables|Default|GetFishDetectorCol) true) ; Allow bobber to pick up fish
    )
    (:then_1
      (bind _returnvalue (Utilities|Time|SetTimerbyEvent (delegate Custom|Received%20Bite) (Math|Random|RandomFloatinRange 3.0 6.0))) ; Fish finding timer\nultimately this will depend on things like the current lure, fish zone, etc\nthese current params are placeholders
      (Variables|Default|SetFish%20Timer _returnvalue))
    (:then_2
      (Audio|Components|Audio|Play (Variables|Default|GetBobberAudio) 0.0)
      (Audio|PlaySound2D "/Game/Audio/WaterSplish.WaterSplish" 1.0 1.0 0.0 0 0))))

(event Custom|Begin%20Transitioning
  (params (Duration :type Float%20%28double-precision%29))
  ;[0.424 0.07502 0.08093] [ Input disable transitions ]
  (Variables|States|SetMidTransition true)
  (Utilities|Time|SetTimerbyEvent (delegate Custom|End%20Transition) Duration))

(event Custom|End%20Transition
  ;[0.424 0.07502 0.08093] [ Input disable transitions ]
  (Variables|States|SetMidTransition false))

(event Custom|Received%20Bite
  ;[0.9308 0.2421 1 1 63] Bite!
  (Variables|States|SetBite true)
  (CallFunction|StartMinigame)
  (Development|PrintString "BITE!!!!!!!!" true true "(R=1.000000,G=0.254621,B=0.672049,A=1.000000)") ; some kinda official notification feedback\ni.e. UI/VFX response
)

(event Custom|Gauge%20Catch%20Progress
  (params (Change%20in%20Prog :type Float%20%28double-precision%29))
  ;[0.1676 0.3687 1 1 58] Update gauge while catching fish
  (bind _output_get (Variables|FishCatching|SetCatch%20Progress (+ Change%20in%20Prog (Variables|FishCatching|GetCatch%20Progress))))
  (Default|SetGaugePercent (Variables|UI|GetCatchingUI) _output_get)
  (if (>= _output_get 1.0) ; Are we done yet?
    (CallFunction|CatchComplete true)
    (elif (<= _output_get 0.0)
      (CallFunction|CatchComplete false))))

(event Custom|Catch%20Complete
  (params (Success :type Boolean))
  ;[0.08327 1 0.1783] Fish caught (or not)
  (CallFunction|SwapCameras true)
  (Widget|RemovefromParent (Variables|UI|GetCatchingUI))
  (Variables|States|SetFishing%20State "NewEnumerator0")
  (CallFunction|BeginTransitioning 1.5)
  (Utilities|FlowControl|Sequence
    (:then_0
      ;[0.6769 0.31 1] Reeling in
      (bind (_direction _dist) (Timeline|Launch%20Bobber%20on%20Spline ReverseFromEnd)
        (:Update
          (Transformation|SetWorldLocation (Variables|Default|GetBobber) (Spline|GetLocationatTime (Variables|Default|GetBobberSpline) _dist "World" false) false false))
        (:Finished
          (if (Utilities|Enum|Equal(Enum) _direction "Forward")
            (CallFunction|BobberImpact)
            (else
              (Audio|Components|Audio|Stop (Variables|Default|GetBobberAudio)))))))
    (:then_1
      (Development|PrintString (Utilities|String|SelectString "You caught a fish!" "You failed to catch the fish..." Success)))
    (:then_2
      (CallFunction|SelectingFishingSpotState true))))

(event Custom|Change%20Controlled%20State
  (params (Enabling :type Boolean))
  (CallFunction|SelectingFishingSpotState Enabling)
  (Rendering|SetVisibility (Variables|Default|GetNS_CrosshairLine) Enabling false)
  (Input|SetInputModeGameOnly (Game|GetPlayerController 0) false))

(event Custom|StartMinigame
  (Variables|States|SetFishing%20State "NewEnumerator2") ; We are now fighting the fish
  ;[1 0 0] This is all to do with the prototype minigame. Proper minigame code should replace this.
  (bind _returnvalue (UserInterface|CreateWidget "/Game/UI/WB_CatchingGauge.WB_CatchingGauge_C"))
  (bind _output_get (Variables|UI|SetCatchingUI _returnvalue))
  (UserInterface|Viewport|AddtoViewport _output_get 0)
  (CallFunction|SwapCameras false)
  (Variables|FishCatching|SetCatch%20Progress 0.99)
  (Transformation|SetWorldLocation (Variables|Default|GetFishDetectorCol) (Transformation|GetWorldLocation (Variables|Default|GetBobber)) false false))

(event Custom|Selecting%20Fishing%20Spot%20State
  (params (Enabling :type Boolean))
  (bind _camera (Variables|Default|GetCamera))
  ;[0.1214 0.85 1] Determines if the casting gauge should be visible or not
  (Widget|SetVisibility (Variables|UI|GetCast%20Meter) (select Enabling "Visible" "Hidden"))
  (if Enabling
    ;[0.3338 1 0.7006] Selecting a fishing spot
    (bind _scale (Timeline|Choose%20Fishing%20Distance PlayFromStart)
      (:Update
        (Utilities|FlowControl|Sequence
          (:then_0
            (Development|PrintString (Utilities|String|ToString(Float) (Math|Float|Lerp (Variables|FishCatching|GetMinimum%20Cast%20Range) (Variables|FishCatching|GetMaximum%20Cast%20Range) _scale)) true true "(R=0.018557,G=1.000000,B=0.000000,A=1.000000)" 2.0 "FishDistance")
            (Default|SetGaugePercent (Variables|UI|GetCast%20Meter) _scale))
          (:then_1
            (if (Utilities|Enum|NotEqual(Enum) (Variables|States|GetFishing%20State) "NewEnumerator1")
              (Utilities|FlowControl|Sequence
                (:then_0
                  (bind (_outhit _returnvalue) (Collision|LineTraceByChannel (+ (* (Math|Vector|GetForwardVector _camera) (Math|Float|Lerp (Variables|FishCatching|GetMinimum%20Cast%20Range) (Variables|FishCatching|GetMaximum%20Cast%20Range) _scale)) "0.000000,0.000000,5000.000000" (Transformation|GetWorldLocation _camera)) (- (+ (* (Math|Vector|GetForwardVector _camera) (Math|Float|Lerp (Variables|FishCatching|GetMinimum%20Cast%20Range) (Variables|FishCatching|GetMaximum%20Cast%20Range) _scale)) "0.000000,0.000000,5000.000000" (Transformation|GetWorldLocation _camera)) "0.000000,0.000000,10000.000000") "TraceTypeQuery1" false 0 "ForOneFrame" true "(R=50.000000,G=22.712761,B=0.000000,A=1.000000)" "(R=0.000000,G=0.000000,B=0.000000,A=0.000000)"))
                  (Variables|States|SetValidRodPos _returnvalue) ; TODO: rewrite to ensure the surface is fishable
                  (Transformation|SetWorldLocationAndRotation (Variables|Default|GetFishTargetIndicator) (.Location (Collision|BreakHitResult _outhit)) "0, 0, 0" false false))))))))
    (else
      (Timeline|Choose%20Fishing%20Distance Stop))))

(event Custom|Swap%20Cameras
  (params (Set%20Main%20Active :type Boolean))
  (Components|Activation|SetActive (Variables|Default|GetCamera) Set%20Main%20Active false)
  (Components|Activation|SetActive (Variables|Default|GetFishView) (not Set%20Main%20Active) false))

(event Input|EnhancedActionEvents|EnhancedInputActionIA_FishLook
  (params (ActionValue :type Vector%202D%20Structure) (ElapsedSeconds :type Float%20%28double-precision%29) (TriggeredSeconds :type Float%20%28double-precision%29) (InputAction :type Input%20Action%20Object%20Reference :default "/Game/Input/Fishing/IA_FishLook.IA_FishLook"))
  (bind _camera (Variables|Default|GetCamera))
  ;[0.3338 1 0.7006] Selecting a fishing spot
  (Pawn|Input|AddControllerYawInput (.x ActionValue))
  (if (Utilities|Enum|NotEqual(Enum) (Variables|States|GetFishing%20State) "NewEnumerator1")
    (Utilities|FlowControl|Sequence
      (:then_0
        (bind (_outhit _returnvalue) (Collision|LineTraceByChannel (+ (* (Math|Vector|GetForwardVector _camera) (Math|Float|Lerp (Variables|FishCatching|GetMinimum%20Cast%20Range) (Variables|FishCatching|GetMaximum%20Cast%20Range) (stale Custom|Selecting%20Fishing%20Spot%20State _scale))) "0.000000,0.000000,5000.000000" (Transformation|GetWorldLocation _camera)) (- (+ (* (Math|Vector|GetForwardVector _camera) (Math|Float|Lerp (Variables|FishCatching|GetMinimum%20Cast%20Range) (Variables|FishCatching|GetMaximum%20Cast%20Range) (stale Custom|Selecting%20Fishing%20Spot%20State _scale))) "0.000000,0.000000,5000.000000" (Transformation|GetWorldLocation _camera)) "0.000000,0.000000,10000.000000") "TraceTypeQuery1" false 0 "ForOneFrame" true "(R=50.000000,G=22.712761,B=0.000000,A=1.000000)" "(R=0.000000,G=0.000000,B=0.000000,A=0.000000)"))
        (Variables|States|SetValidRodPos _returnvalue) ; TODO: rewrite to ensure the surface is fishable
        (Transformation|SetWorldLocationAndRotation (Variables|Default|GetFishTargetIndicator) (.Location (Collision|BreakHitResult _outhit)) "0, 0, 0" false false)))))

(event Input|EnhancedActionEvents|EnhancedInputActionIA_SwitchPerspective
  (params (ActionValue :type Boolean) (ElapsedSeconds :type Float%20%28double-precision%29) (TriggeredSeconds :type Float%20%28double-precision%29) (InputAction :type Input%20Action%20Object%20Reference :default "/Game/Input/IA_SwitchPerspective.IA_SwitchPerspective"))
  (bind _returnvalue (Game|GetPlayerController 0))
  (bind _returnvalue_2 (PlayerController|LocalPlayerSubsystems|GetEnhancedInputLocalPlayerSubsystem _returnvalue))
  ;[1 1 1] Switch Perspective back to Boat
  (:Started
    (if (and (Utilities|Enum|Equal(Enum) (Variables|States|GetFishing%20State) "NewEnumerator0") (not (Variables|States|GetMidTransition)))
      (Utilities|IsValid _returnvalue
        (:Is%20Valid
          (Pawn|Possess _returnvalue (Variables|Default|GetBoat))
          (Utilities|IsValid _returnvalue_2
            (:Is%20Valid
              (Input|RemoveMappingContext _returnvalue_2 "/Game/Input/Fishing/IMC_Fishing.IMC_Fishing" "(bIgnoreAllPressedKeysUntilRelease=True,bForceImmediately=False,bNotifyUserSettings=False)")
              (Input|AddMappingContext _returnvalue_2 "/Game/Input/Boat/IMC_Boat.IMC_Boat" 0 "(bIgnoreAllPressedKeysUntilRelease=True,bForceImmediately=False,bNotifyUserSettings=False)")
              (CallFunction|ChangeControlledState false))))))))

(event Input|EnhancedActionEvents|EnhancedInputActionIA_FishCast
  (params (ActionValue :type Boolean) (ElapsedSeconds :type Float%20%28double-precision%29) (TriggeredSeconds :type Float%20%28double-precision%29) (InputAction :type Input%20Action%20Object%20Reference :default "/Game/Input/Fishing/IA_FishCast.IA_FishCast"))
  (bind _bobber (Variables|Default|GetBobber))
  (bind _fishtargetindicator (Variables|Default|GetFishTargetIndicator))
  (bind _bobber_2 (Variables|Default|GetBobber))
  (bind _defaultsceneroot (Variables|Default|GetDefaultSceneRoot))
  (bind _bobberspline (Variables|Default|GetBobberSpline))
  (bind _fishtargetindicator_2 (Variables|Default|GetFishTargetIndicator))
  (bind _bobberspline_2 (Variables|Default|GetBobberSpline))
  (bind _returnvalue (Transformation|GetWorldLocation _fishtargetindicator_2))
  (bind _returnvalue_2 (Transformation|GetWorldLocation _bobber))
  (bind _returnvalue_3 (Class|PrimitiveComponent|IsOverlappingComponent _fishtargetindicator _bobber_2))
  (bind _returnvalue_4 (Transformation|GetWorldRotation _defaultsceneroot))
  (bind _returnvalue_5 (Class|KismetMathLibrary|NegateRotator _returnvalue_4))
  (bind _returnvalue_6 (- _returnvalue _returnvalue_2))
  (bind _returnvalue_7 (Math|Vector|RotateVector _returnvalue_6 _returnvalue_5))
  ;[0.08179 1 0.06473 1 56] Casting rod (left click)
  (:Started
    (if (not (Variables|States|GetMidTransition))
      (if (not (Utilities|Enum|Equal(Enum) (Variables|States|GetFishing%20State) "NewEnumerator2"))
        (Utilities|RodIsCast
          (:Is%20Cast
            (if (not (Variables|States|GetBite)) ; Branch if bitten or not
              (CallFunction|BeginTransitioning 1.0)
              ;[0.6769 0.31 1] Reeling in
              (Utilities|FlowControl|Sequence
                (:then_0
                  (bind (_direction _dist) (Timeline|Launch%20Bobber%20on%20Spline ReverseFromEnd)
                    (:Update
                      (Transformation|SetWorldLocation (Variables|Default|GetBobber) (Spline|GetLocationatTime (Variables|Default|GetBobberSpline) _dist "World" false) false false))
                    (:Finished
                      (if (Utilities|Enum|Equal(Enum) _direction "Forward")
                        (CallFunction|BobberImpact)
                        (else
                          (Audio|Components|Audio|Stop (Variables|Default|GetBobberAudio)))))))
                (:then_1
                  (Variables|States|SetFishing%20State "NewEnumerator0")
                  (Utilities|Time|ClearandInvalidateTimerbyHandle (Variables|Default|GetFish%20Timer)) ; Clear bait timer cus we are no longer baiting
                  (Variables|/Script/Engine.PrimitiveComponent|SetbGenerateOverlapEvents (Variables|Default|GetFishDetectorCol) true) ; Prevent bobber from picking up fish\n(we'll also need to get all fish to \nlose interest)
                )
                (:then_2
                  (Transformation|SetWorldLocation (Variables|Default|GetFishTargetIndicator) "0, 0, 0" false false)
                  (CallFunction|SelectingFishingSpotState true)))
              (else
                (CallFunction|StartMinigame))))
          (:Isn't%20Cast
            ;[0.2147 0.3632 1] Casting away
            (if (Variables|States|GetValidRodPos) ; TODO: ensure cursor is in valid position
              (Variables|States|SetFishing%20State "NewEnumerator1")
              (Utilities|FlowControl|Sequence
                (:then_0
                  (Spline|ClearSplinePoints _bobberspline true)
                  (Spline|AddSplinePoint _bobberspline (Math|Vector|MakeVector 0.0 0.0 0.0) "Local" true)
                  (Development|PrintString (Utilities|String|ToString(Vector) _returnvalue_7))
                  (Spline|AddSplinePoint _bobberspline _returnvalue_7 "Local" true)
                  (Spline|SetTangentatSplinePoint _bobberspline_2 0 (Math|Vector|MakeVector 0.0 0.0 6e+02) "World" true)
                  (Spline|SetTangentatSplinePoint _bobberspline_2 1 (Math|Vector|MakeVector 0.0 0.0 0.0) "World" true))
                (:then_1
                  (Timeline|Launch%20Bobber%20on%20Spline PlayFromStart))
                (:then_2
                  (CallFunction|BeginTransitioning 1.0)
                  (CallFunction|SelectingFishingSpotState false)
                  (Audio|PlaySound2D "/Game/Audio/RodSwoosh.RodSwoosh" 1.0 1.0 0.0 0 0))))))
        (else
          ;[0.2854 0.6346 1] Click when currently fighting fish
          (CallFunction|GaugeCatchProgress (Math|Float|SelectFloat 0.1 -0.07 _returnvalue_3))
          (Niagara|SpawnSystematLocation (select _returnvalue_3 "/Game/VFX/NS_SuccessfulSplash.NS_SuccessfulSplash" "/Game/VFX/NS_FailSplash.NS_FailSplash") (Transformation|GetWorldLocation (Variables|Default|GetBobber))))))))

(event EventTick
  (params (DeltaSeconds :type Float%20%28single-precision%29))
  (bind _defaultsceneroot (Variables|Default|GetDefaultSceneRoot))
  (bind _returnvalue (Transformation|GetWorldLocation _defaultsceneroot))
  (Utilities|FlowControl|Sequence
    (:then_0
      (if (Utilities|Enum|Equal(Enum) (Variables|States|GetFishing%20State) "NewEnumerator2")
        (CallFunction|GaugeCatchProgress (* DeltaSeconds -0.01))
        (bind _output_get (Variables|FishCatching|SetRodSteerAngle (Class|KismetMathLibrary|DegAcos (Math|Vector|DotProduct (Math|Vector|Normalize (- (Transformation|GetWorldLocation (Variables|Default|GetFishTargetIndicator)) _returnvalue)) (Math|Vector|Normalize (- (Transformation|GetWorldLocation (Variables|Default|GetBobber)) _returnvalue))))))
        (Development|PrintString (Utilities|String|ToString(Float) _output_get) true true "(R=1.000000,G=0.630471,B=0.000000,A=1.000000)" 2.0 "divide")
        (Development|PrintString (Utilities|String|SelectString "Steering away!" "Failing to control!" (>= _output_get 1.4e+02)) true true (Math|Color|SelectColor "(R=0.000000,G=1.000000,B=0.745748,A=1.000000)" "(R=1.000000,G=0.085407,B=0.306603,A=1.000000)" (>= _output_get 1.4e+02)) 2.0 "steer")))
    (:then_1
      (Development|PrintString (Utilities|String|ToString(Float) (.yaw (Transformation|GetWorldRotation (Variables|Default|GetDefaultSceneRoot)))) true true "(R=0.327742,G=1.000000,B=0.446522,A=1.000000)" 2.0 "Rotation"))))

(event EventBeginPlay
  (Utilities|FlowControl|Sequence
    (:then_0
      (bind _returnvalue (Game|ConstructObjectfromClass "/Game/UI/WB_CastMeter.WB_CastMeter_C"))
      (bind _output_get (Variables|UI|SetCast%20Meter _returnvalue))
      (UserInterface|Viewport|AddtoViewport _output_get 0)
      (Widget|SetVisibility _output_get "Hidden"))
    (:then_1
      (bind _returnvalue_2 (Audio|CreateSound2D "/Game/Audio/Loop_Bobbing.Loop_Bobbing" 1.0 1.0 0.0 0 false false))
      (bind _output_get_2 (Variables|Default|SetBobberAudio _returnvalue_2))
      (Audio|Components|Audio|Stop _output_get_2)
      (Class|GameplayStatics|PrimeSound "/Game/Audio/RodSwoosh.RodSwoosh")
      (Class|GameplayStatics|PrimeSound "/Game/Audio/WaterSplish.WaterSplish"))
    (:then_2
      (CallFunction|SwapCameras true))))

(fn ConstructionScript)