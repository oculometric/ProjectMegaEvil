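; Actor component on BP_FishingMgr that runs the fish-catching minigame from start to end.
; Starting shows the catching gauge, swaps cameras and moves the fish detector to the bobber.
; GameTick advances progress over time and debug-prints rod steering from a dot-product angle against a placeholder fish target, without affecting progress.
; Either progress limit ends the game, currently always as a failure, restoring camera and spot selection.
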(event Custom|Start%20Fishing%20Game
  (bind _fishingmgr (Variables|Default|GetFishingMgr))
  (bind _fishingmgr_2 (Variables|Default|GetFishingMgr))
  (Variables|/Game/Blueprints/FishingTest/BP_FishingMgr5.BP_FishingMgr5_C|SetFishing%20State _fishingmgr_2 "NewEnumerator2")
  (bind _returnvalue (UserInterface|CreateWidget "/Game/UI/WB_CatchingGauge.WB_CatchingGauge_C"))
  (bind _output_get (Variables|/Game/Blueprints/FishingTest/BP_FishingMgr5.BP_FishingMgr5_C|SetCatchingUI _fishingmgr_2 _returnvalue))
  (UserInterface|Viewport|AddtoViewport _output_get 0)
  (Default|SwapCameras (Variables|Default|GetFishingMgr) false)
  (Variables|/Game/Blueprints/FishingTest/BP_FishingMgr5.BP_FishingMgr5_C|SetCatch%20Progress _fishingmgr 0.99)
  (Variables|/Script/Engine.PlayerController|SetbShowMouseCursor (Game|GetPlayerController 0) true)
  (Transformation|SetWorldLocation (Variables|/Game/Blueprints/FishingTest/BP_FishingMgr5.BP_FishingMgr5_C|GetFishDetectorCol _fishingmgr) (Transformation|GetWorldLocation (Variables|/Game/Blueprints/FishingTest/BP_FishingMgr5.BP_FishingMgr5_C|GetBobber _fishingmgr)) false false))

(event Custom|Game%20Tick
  (params (Delta :type Float%20%28double-precision%29))
  (bind _fishingmgr (Variables|Default|GetFishingMgr))
  (bind _defaultsceneroot (Variables|/Game/Blueprints/FishingTest/BP_FishingMgr5.BP_FishingMgr5_C|GetDefaultSceneRoot _fishingmgr))
  (bind _returnvalue (Transformation|GetWorldLocation _defaultsceneroot))
  (CallFunction|CatchProgression (* Delta 0.01))
  (bind _output_get (Variables|/Game/Blueprints/FishingTest/BP_FishingMgr5.BP_FishingMgr5_C|SetRodSteerAngle (Variables|Default|GetFishingMgr) (Class|KismetMathLibrary|DegAcos (Math|Vector|DotProduct (Math|Vector|Normalize (- (Transformation|GetWorldLocation (Variables|/Game/Blueprints/FishingTest/BP_FishingMgr5.BP_FishingMgr5_C|GetFishTargetIndicator _fishingmgr)) _returnvalue)) (Math|Vector|Normalize (- (Transformation|GetWorldLocation (Variables|/Game/Blueprints/FishingTest/BP_FishingMgr5.BP_FishingMgr5_C|GetBobber _fishingmgr)) _returnvalue))))))
  (Development|PrintString (Utilities|String|ToString(Float) _output_get) true true "(R=1.000000,G=0.630471,B=0.000000,A=1.000000)" 2.0 "divide")
  (Development|PrintString (Utilities|String|SelectString "Steering away!" "Failing to control!" (>= _output_get 1.4e+02)) true true (Math|Color|SelectColor "(R=0.000000,G=1.000000,B=0.745748,A=1.000000)" "(R=1.000000,G=0.085407,B=0.306603,A=1.000000)" (>= _output_get 1.4e+02)) 2.0 "steer"))

(event Custom|Game%20End
  (params (Success :type Boolean))
  (bind _fishingmgr (Variables|Default|GetFishingMgr))
  (Default|SwapCameras _fishingmgr true)
  (Widget|RemovefromParent (Variables|/Game/Blueprints/FishingTest/BP_FishingMgr5.BP_FishingMgr5_C|GetCatchingUI _fishingmgr))
  (Variables|/Game/Blueprints/FishingTest/BP_FishingMgr5.BP_FishingMgr5_C|SetFishing%20State _fishingmgr "NewEnumerator0")
  (Default|BeginTransitioning _fishingmgr 1.0)
  (Utilities|FlowControl|Sequence
    (:then_1
      (Development|PrintString (Utilities|String|SelectString "You caught a fish!" "You failed to catch the fish..." Success)))
    (:then_2
      (Default|SelectingFishingSpotState _fishingmgr true))))

(event Custom|Catch%20Progression
  (params (Change%20in%20Prog :type Float%20%28double-precision%29))
  (bind _fishingattributescomp (Variables|Default|GetFishingAttributesComp))
  (bind _output_get (Variables|/Game/Blueprints/FishingTest/Components/BPC_FishingAttributes.BPC_FishingAttributes_C|SetProgressPercentage _fishingattributescomp (+ Change%20in%20Prog (Variables|/Game/Blueprints/FishingTest/Components/BPC_FishingAttributes.BPC_FishingAttributes_C|GetProgressPercentage _fishingattributescomp))))
  (Default|SetGaugePercent (Variables|/Game/Blueprints/FishingTest/BP_FishingMgr5.BP_FishingMgr5_C|GetCatchingUI (Variables|Default|GetFishingMgr)) _output_get)
  (if (>= _output_get 1.0) ; Are we done yet?
    (CallFunction|GameEnd false)
    (elif (<= _output_get 0.0)
      (CallFunction|GameEnd false))))

(event EventBeginPlay
  (bind _asbp_fishing_mgr_5 (Utilities|Casting|CastToBP_FishingMgr5 (Components|GetOwner)))
  (bind _output_get (Variables|Default|SetFishingMgr _asbp_fishing_mgr_5))
  (Variables|Default|SetFishingAttributesComp (Variables|/Game/Blueprints/FishingTest/BP_FishingMgr5.BP_FishingMgr5_C|GetBPC_FishingAttributes _output_get)))