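; BPC_FishingAttributes is a component holding fishing-related state: tension, progress, money and the fish inventory.
; Its setter events for tension, progress and money broadcast event dispatchers, with money changes clamped to a fixed range.
; Adding a fish appends it to the inventory data, then refreshes the player menu UI through the fisher player controller.
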(event Custom|SetTension
  (params (Tension :type Float%20%28double-precision%29))
  ;[1 1 1] Call the event dispatchers whenever their respective variables change :)
  (Default|CallETensionUpdated Tension))

(event Custom|SetProgress
  (params (Progress :type Float%20%28double-precision%29))
  ;[1 1 1] Call the event dispatchers whenever their respective variables change :)
  (Default|CallEProgressUpdated Progress))

(event Custom|AddToInventory
  (params (Fish :type S%20Fish%20Inventory%20Info%20Structure))
  ;[1 1 1] Adding Fish
  (Utilities|Array|Add (Variables|Default|GetInventoryData) Fish)
  (bind _asbp_lfisher_controller (Utilities|Casting|CastToBP_LFisherController (Game|GetPlayerController 0)))
  (Default|UpdateInventory (Variables|/Game/Blueprints/FishingTest/PD_TestMode/BP_LFisherController.BP_LFisherController_C|GetPlayerMenuUI _asbp_lfisher_controller) self))

(event Custom|UpdateMoney
  (params (DeltaMoney :type Integer))
  (Default|CallEMoneyUpdated (Math|Integer|Clamp(Integer) (+ DeltaMoney (Variables|Default|GetMoney)) 0 1000000)))