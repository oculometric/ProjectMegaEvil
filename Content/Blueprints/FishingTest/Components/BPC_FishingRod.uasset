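; Fishing rod component on BP_FishingMgr5 that runs the catch minigame, started when a fish pawn overlaps the bite collider.
; While fighting, clicks raise steadily falling line tension, which loses the fish at either limit, and steering opposite the fish drains its stamina.
; Exhausted fish can be scroll-reeled until stamina refills and fighting resumes.
; Full progress adds the catch to inventory; either outcome restores the camera and shows a popup.
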(event Custom|Change%20in%20Tension
  (params (Change :type Float%20%28double-precision%29))
  (if (Utilities|Enum|Equal(Enum) (Variables|/Game/Blueprints/FishingTest/BP_FishingMgr5.BP_FishingMgr5_C|GetFishing%20State (Variables|Default|GetFishingMgr)) "NewEnumerator2")
    (bind _output_get (Variables|Default|SetFishTension (+ (Variables|Default|GetFishTension) Change)))
    (Default|SetTension (Variables|Default|GetFishing%20Attributes) _output_get)
    (if (>= _output_get 1.0)
      (CallFunction|GameEnd false) ; Too much tension; line breaks
      (Default|FailedMinigame (Variables|Default|GetFishVictim) :!label _label)
      (elif (<= _output_get 0.0)
        (CallFunction|GameEnd false) ; Not enough tension; fish escapes
        (goto _label)))))

(event Custom|Fishing%20Result%20Popup
  (params (Result :type Boolean) (Explanation :type Text))
  (bind _returnvalue (Game|ConstructObjectfromClass "/Game/UI/Fishing/WBP_FishingResultPopup.WBP_FishingResultPopup_C" Result Explanation))
  (UserInterface|Viewport|AddtoViewport _returnvalue 0))

(event Custom|Game%20End
  (params (Success :type Boolean))
  (bind _fishvictim (Variables|Default|GetFishVictim))
  (bind _fishvictim_2 (Variables|Default|GetFishVictim))
  (bind _fishingmgr (Variables|Default|GetFishingMgr))
  (bind _fishinventorydata (Variables|/Game/Blueprints/Fish/BP_FishPawn.BP_FishPawn_C|GetFishInventoryData _fishvictim_2))
  (Default|RecallRod (Variables|Default|GetFishingMgr))
  (Default|SetCameraMode _fishingmgr false)
  (Widget|RemovefromParent (Variables|Default|GetFishingHUD))
  (if Success
    (Default|FishShowoff _fishingmgr _fishvictim)
    (Default|CatchFish _fishvictim_2)
    (Default|AddtoInventory (Variables|Default|GetFishing%20Attributes) _fishinventorydata)
    (CallFunction|FishingResultPopup true (Utilities|Text|ToText(String) (Utilities|String|Append "You caught a " (.FishName (Utilities|Struct|BreakS_FishInventoryInfo _fishinventorydata)) "!")))
    (else
      (Default|FishEscape _fishingmgr _fishvictim)
      (CallFunction|FishingResultPopup false "The fish got away..."))))

(event Custom|PotentialFishOverlap
  (params (OverlappedComponent :type Primitive%20Component%20Object%20Reference) (OtherActor :type Actor%20Object%20Reference) (OtherComp :type Primitive%20Component%20Object%20Reference) (OtherBodyIndex :type Integer) (bFromSweep :type Boolean) (SweepResult :type Hit%20Result%20Structure%20%28by%20ref%29))
  (bind _fishingmgr (Variables|Default|GetFishingMgr))
  (bind _asbp_fish_pawn (Utilities|Casting|CastToBP_FishPawn OtherActor))
  (Variables|/Script/Engine.PrimitiveComponent|SetbGenerateOverlapEvents (Variables|/Game/Blueprints/FishingTest/BP_FishingMgr5.BP_FishingMgr5_C|GetFishInterestCollider _fishingmgr) false)
  (Variables|/Script/Engine.PrimitiveComponent|SetbGenerateOverlapEvents (Variables|/Game/Blueprints/FishingTest/BP_FishingMgr5.BP_FishingMgr5_C|GetFishBiteCollider _fishingmgr) false)
  (CallFunction|FishBite _asbp_fish_pawn)
  (Default|BecomeMinigameTarget _asbp_fish_pawn (Variables|/Game/Blueprints/FishingTest/BP_FishingMgr5.BP_FishingMgr5_C|GetBoat (Variables|Default|GetFishingMgr))))

(event Custom|FishBite
  (params (Fish :type BP%20Fish%20Pawn%20Object%20Reference))
  (Variables|Default|SetFishVictim Fish)
  ;[0.6211 0.3417 1] Reset act of fishing values
  (Variables|Default|SetFishStamina 0.8)
  (Variables|Default|SetCatchProgress 0.0)
  (Variables|Default|SetFishTension 0.8)
  (Variables|Default|SetBobberOrigin (Transformation|GetWorldLocation (Variables|/Game/Blueprints/FishingTest/BP_FishingMgr5.BP_FishingMgr5_C|GetBobber (Variables|Default|GetFishingMgr))))
  (Variables|/Game/Blueprints/FishingTest/BP_FishingMgr5.BP_FishingMgr5_C|SetFishing%20State (Variables|Default|GetFishingMgr) "NewEnumerator2")
  (Utilities|FlowControl|Sequence
    (:then_0
      (bind _returnvalue (UserInterface|CreateWidget "/Game/UI/Fishing/WBP_FishingHUD.WBP_FishingHUD_C"))
      (bind _output_get (Variables|Default|SetFishingHUD _returnvalue))
      (UserInterface|Viewport|AddtoViewport _output_get 0)
      (Default|Initialise _output_get (Variables|Default|GetFishingMgr)))
    (:then_1
      (Default|SetCameraMode (Variables|Default|GetFishingMgr) true))))

(event Input|EnhancedActionEvents|EnhancedInputActionIA_FishLook
  (params (ActionValue :type Vector%202D%20Structure) (ElapsedSeconds :type Float%20%28double-precision%29) (TriggeredSeconds :type Float%20%28double-precision%29) (InputAction :type Input%20Action%20Object%20Reference :default "/Game/Input/Fishing/IA_FishLook.IA_FishLook"))
  ;[0.6419 0.1643 1] Cursor movement
  (switch Utilities|FlowControl|Switch|SwitchonE_FishingStates (Variables|/Game/Blueprints/FishingTest/BP_FishingMgr5.BP_FishingMgr5_C|GetFishing%20State (Variables|Default|GetFishingMgr))
    (:NewEnumerator2
      (Transformation|AddRelativeRotation (Variables|/Game/Blueprints/FishingTest/BP_FishingMgr5.BP_FishingMgr5_C|GetSteeringDirection (Variables|Default|GetFishingMgr)) (Math|Rotator|MakeRotator 0.0 0.0 (* (.x ActionValue) 3.0)) false false))))

(event Input|EnhancedActionEvents|EnhancedInputActionIA_FishReel
  (params (ActionValue :type Float%20%28double-precision%29) (ElapsedSeconds :type Float%20%28double-precision%29) (TriggeredSeconds :type Float%20%28double-precision%29) (InputAction :type Input%20Action%20Object%20Reference :default "/Game/Input/Fishing/IA_FishReel.IA_FishReel"))
  ;[1 0.2159 0.4694] Scroll control
  (if (Utilities|Enum|Equal(Enum) (Variables|/Game/Blueprints/FishingTest/BP_FishingMgr5.BP_FishingMgr5_C|GetFishing%20State (Variables|Default|GetFishingMgr)) "NewEnumerator3")
    (bind _output_get (Variables|Default|SetCatchProgress (+ (Variables|Default|GetCatchProgress) (* (Math|Float|Clamp(Float) ActionValue -1.0 0.0) 0.03 -1.0))))
    (Default|SetProgress (Variables|Default|GetFishing%20Attributes) _output_get)
    (if (>= (Variables|Default|GetCatchProgress) 1.0) ; We done?
      (CallFunction|GameEnd true))))

(event Input|EnhancedActionEvents|EnhancedInputActionIA_FishCast
  (params (ActionValue :type Boolean) (ElapsedSeconds :type Float%20%28double-precision%29) (TriggeredSeconds :type Float%20%28double-precision%29) (InputAction :type Input%20Action%20Object%20Reference :default "/Game/Input/Fishing/IA_FishCast.IA_FishCast"))
  ;[0.3277 0.2491 1] Click control
  (:Started
    (if (Utilities|Enum|Equal(Enum) (Variables|/Game/Blueprints/FishingTest/BP_FishingMgr5.BP_FishingMgr5_C|GetFishing%20State (Variables|Default|GetFishingMgr)) "NewEnumerator2")
      (CallFunction|ChangeinTension 0.15) ; Manual tension control
    )))

(event EventBeginPlay
  (bind _asbp_fishing_mgr_5 (Utilities|Casting|CastToBP_FishingMgr5 (Components|GetOwner)))
  (bind _output_get (Variables|Default|SetFishingMgr _asbp_fishing_mgr_5))
  (Collision|BindEventtoOnComponentBeginOverlap (Variables|/Game/Blueprints/FishingTest/BP_FishingMgr5.BP_FishingMgr5_C|GetFishBiteCollider _output_get) (delegate Custom|PotentialFishOverlap))
  (Variables|Default|SetFishing%20Attributes (Variables|/Game/Blueprints/FishingTest/BP_FishingMgr5.BP_FishingMgr5_C|GetFishingAttributes (Variables|Default|GetFishingMgr))))

(event EventTick
  (params (DeltaSeconds :type Float%20%28single-precision%29))
  (bind _fishingmgr (Variables|Default|GetFishingMgr))
  (bind _defaultsceneroot (Variables|/Game/Blueprints/FishingTest/BP_FishingMgr5.BP_FishingMgr5_C|GetDefaultSceneRoot _fishingmgr))
  (bind _returnvalue (Transformation|GetWorldLocation _defaultsceneroot))
  (switch Utilities|FlowControl|Switch|SwitchonE_FishingStates (Variables|/Game/Blueprints/FishingTest/BP_FishingMgr5.BP_FishingMgr5_C|GetFishing%20State (Variables|Default|GetFishingMgr))
    (:NewEnumerator2
      (Development|PrintString "Battling the fish!" true true "(R=0.595891,G=0.092255,B=1.000000,A=1.000000)" 2.0 "fishstate")
      (Collision|LineTraceByChannel (Transformation|GetWorldLocation (Variables|/Game/Blueprints/FishingTest/BP_FishingMgr5.BP_FishingMgr5_C|GetPointer (Variables|Default|GetFishingMgr))) (Transformation|GetWorldLocation (Variables|/Game/Blueprints/Fish/BP_FishPawn.BP_FishPawn_C|GetDefaultSceneRoot (Variables|Default|GetFishVictim))) "TraceTypeQuery1" false 0 "ForOneFrame")
      (bind _output_get (Variables|/Game/Blueprints/FishingTest/BP_FishingMgr5.BP_FishingMgr5_C|SetRodSteerAngle (Variables|Default|GetFishingMgr) (Class|KismetMathLibrary|DegAcos (Math|Vector|DotProduct (Math|Vector|Normalize (- (Transformation|GetWorldLocation (Variables|/Game/Blueprints/FishingTest/BP_FishingMgr5.BP_FishingMgr5_C|GetPointer _fishingmgr)) _returnvalue)) (Math|Vector|Normalize (- (Transformation|GetWorldLocation (Variables|/Script/Engine.Actor|GetRootComponent (Variables|Default|GetFishVictim))) _returnvalue))))))
      (Development|PrintString (Utilities|String|ToString(Float) _output_get) true true "(R=1.000000,G=0.630471,B=0.000000,A=1.000000)" 2.0 "divide")
      (Utilities|FlowControl|Sequence
        (:then_0
          (bind _output_get_2 (Variables|Default|SetFishStamina (Math|Float|Clamp(Float) (+ (Variables|Default|GetFishStamina) (* (Utilities|Time|GetWorldDeltaSeconds) (Math|Float|SelectFloat -0.4 0.1 (>= _output_get 1.4e+02)))))))
          (Utilities|FlowControl|Sequence
            (:then_0
              (if (<= _output_get_2 0.0)
                (Variables|/Game/Blueprints/FishingTest/BP_FishingMgr5.BP_FishingMgr5_C|SetFishing%20State (Variables|Default|GetFishingMgr) "NewEnumerator3")
                (Default|UpdateInstructions (Variables|Default|GetFishingHUD) false)
                (Default|ToggleReel (Variables|Default|GetFishVictim))))
            (:then_1
              (Development|PrintString (Utilities|String|ToString(Float) _output_get_2) true true (Math|Color|SelectColor "(R=0.000000,G=1.000000,B=0.745748,A=1.000000)" "(R=1.000000,G=0.085407,B=0.306603,A=1.000000)" (>= _output_get 1.4e+02)) 2.0 "fishtired") ; debug for displaying fish tiredness
            )))
        (:then_1
          (CallFunction|ChangeinTension (* 0.3 (Utilities|Time|GetWorldDeltaSeconds) -1.0)) ; Gradual fall in tension
          (Transformation|SetWorldLocation (Variables|/Game/Blueprints/FishingTest/BP_FishingMgr5.BP_FishingMgr5_C|GetBobber (Variables|Default|GetFishingMgr)) (Transformation|GetWorldLocation (Variables|/Game/Blueprints/Fish/BP_FishPawn.BP_FishPawn_C|GetDefaultSceneRoot (Variables|Default|GetFishVictim))) false false))))
    (:NewEnumerator3
      (Development|PrintString "Reeling in the fish!" true true "(R=1.000000,G=0.240874,B=0.000000,A=1.000000)" 2.0 "fishstate")
      (bind _output_get_3 (Variables|Default|SetFishStamina (Math|Float|Clamp(Float) (+ (Variables|Default|GetFishStamina) (* (Utilities|Time|GetWorldDeltaSeconds) 0.5))))) ; Replenish stamina when reeling
      (Utilities|FlowControl|Sequence
        (:then_0
          (if (>= _output_get_3 1.0)
            (Variables|/Game/Blueprints/FishingTest/BP_FishingMgr5.BP_FishingMgr5_C|SetFishing%20State (Variables|Default|GetFishingMgr) "NewEnumerator2")
            (Default|UpdateInstructions (Variables|Default|GetFishingHUD) true)
            (Default|ToggleReel (Variables|Default|GetFishVictim))))
        (:then_1
          (Development|PrintString (Utilities|String|ToString(Float) _output_get_3) true true "(R=0.000000,G=0.660000,B=1.000000,A=1.000000)" 2.0 "fishtired") ; debug for displaying fish tiredness
        )))))