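; Fishing rod component on BP_FishingPawn that runs the fish-catching minigame from bite to catch or escape.
; While fighting, clamped steering against the fish's pull, judged by dot product, drains its stamina, and clicks offset falling line tension.
; An exhausted fish can be scroll-reeled to build catch progress until its stamina refills and fighting resumes.
; Full progress adds it to inventory, tension extremes lose it, and a popup reports either result.
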(event Custom|Change%20in%20Tension
  (params (Change :type Float%20%28double-precision%29))
  ;[0.1303 0.5034 1] When modifying tension
  (if (Utilities|Enum|Equal(Enum) (Variables|/Game/Blueprints/Fishing/BP_FishingPawn.BP_FishingPawn_C|GetFishing%20State (Variables|Default|GetFishingMgr)) "NewEnumerator2")
    (bind _output_get (Variables|Default|SetFishTension (+ (Variables|Default|GetFishTension) Change)))
    (Default|SetTension (Variables|Default|GetFishing%20Attributes) _output_get)
    (if (>= _output_get 1.0)
      (CallFunction|GameEnd false 1) ; Too much tension; line breaks
      (Default|FailedMinigame (Variables|Default|GetFishVictim) :!label _label)
      (elif (<= _output_get 0.0)
        (CallFunction|GameEnd false) ; Not enough tension; fish escapes
        (goto _label)))))

(event Custom|Fishing%20Result%20Popup
  (params (Result :type Boolean) (Explanation :type Text))
  ;[0 1 0.01766] End of act of fishing - fish catch or fail
  (bind _returnvalue (Game|ConstructObjectfromClass "/Game/UI/Fishing/WBP_FishingResultPopup.WBP_FishingResultPopup_C" Result Explanation))
  (UserInterface|Viewport|AddtoViewport _returnvalue 0))

(event Custom|Game%20End
  (params (Success :type Boolean) (Reason%20for%20Failure :type Byte))
  (bind _fishvictim (Variables|Default|GetFishVictim))
  (bind _fishvictim_2 (Variables|Default|GetFishVictim))
  (bind _fishingmgr (Variables|Default|GetFishingMgr))
  (bind _fishinventorydata (Variables|/Game/Blueprints/Fish/BP_FishPawn.BP_FishPawn_C|GetFishInventoryData _fishvictim_2))
  ;[0 1 0.01766] End of act of fishing - fish catch or fail
  (Rendering|SetVisibility (Variables|/Game/Blueprints/Fishing/BP_FishingPawn.BP_FishingPawn_C|GetPlayerSteerIndicator _fishingmgr) false false) ; Show steer UI thing
  (Default|RecallRod (Variables|Default|GetFishingMgr))
  (Default|SetCameraMode _fishingmgr false)
  (Widget|RemovefromParent (Variables|Default|GetFishingHUD))
  (if Success
    (Default|FishShowoff _fishingmgr _fishvictim)
    (Default|CatchFish _fishvictim_2)
    (Default|AddtoInventory (Variables|Default|GetFishing%20Attributes) _fishinventorydata)
    (CallFunction|FishingResultPopup true (Utilities|Text|ToText(String) (Utilities|String|Append "You caught a " (.FishName (Utilities|Struct|BreakF_FishInventoryInfo _fishinventorydata)) "!")))
    (else
      (Default|FishEscape _fishingmgr _fishvictim)
      (CallFunction|FishingResultPopup false (Utilities|Select :Index Reason%20for%20Failure :Option%200 "The rod's tension was too low..." :Option%201 "The rod's tension was too high...")))))

(event Custom|PotentialFishOverlap
  (params (OverlappedComponent :type Primitive%20Component%20Object%20Reference) (OtherActor :type Actor%20Object%20Reference) (OtherComp :type Primitive%20Component%20Object%20Reference) (OtherBodyIndex :type Integer) (bFromSweep :type Boolean) (SweepResult :type Hit%20Result%20Structure%20%28by%20ref%29))
  (bind _fishingmgr (Variables|Default|GetFishingMgr))
  (bind _asbp_fish_pawn (Utilities|Casting|CastToBP_FishPawn OtherActor))
  (Variables|/Script/Engine.PrimitiveComponent|SetbGenerateOverlapEvents (Variables|/Game/Blueprints/Fishing/BP_FishingPawn.BP_FishingPawn_C|GetFishInterestCollider _fishingmgr) false)
  (Variables|/Script/Engine.PrimitiveComponent|SetbGenerateOverlapEvents (Variables|/Game/Blueprints/Fishing/BP_FishingPawn.BP_FishingPawn_C|GetFishBiteCollider _fishingmgr) false)
  (CallFunction|FishBite _asbp_fish_pawn)
  (Default|BecomeMinigameTarget _asbp_fish_pawn (Variables|/Game/Blueprints/Fishing/BP_FishingPawn.BP_FishingPawn_C|GetBoat (Variables|Default|GetFishingMgr))))

(event Custom|FishBite
  (params (Fish :type BP%20Fish%20Pawn%20Object%20Reference))
  (Variables|Default|SetFishVictim Fish)
  (Rendering|SetVisibility (Variables|/Game/Blueprints/Fishing/BP_FishingPawn.BP_FishingPawn_C|GetPlayerSteerIndicator (Variables|Default|GetFishingMgr)) true false) ; Show steer UI thing
  ;[0.6211 0.3417 1] Reset act of fishing values
  (Variables|Default|SetFishStamina 0.8)
  (Variables|Default|SetCatchProgress 0.0)
  (Variables|Default|SetFishTension 0.8)
  (Variables|Default|SetBobberOrigin (Transformation|GetWorldLocation (Variables|/Game/Blueprints/Fishing/BP_FishingPawn.BP_FishingPawn_C|GetBobber (Variables|Default|GetFishingMgr))))
  (Variables|/Game/Blueprints/Fishing/BP_FishingPawn.BP_FishingPawn_C|SetFishing%20State (Variables|Default|GetFishingMgr) "NewEnumerator2")
  (Utilities|FlowControl|Sequence
    (:then_0
      (bind _returnvalue (UserInterface|CreateWidget "/Game/UI/Fishing/WBP_FishingHUD.WBP_FishingHUD_C"))
      (bind _output_get (Variables|Default|SetFishingHUD _returnvalue))
      (UserInterface|Viewport|AddtoViewport _output_get 0)
      (Default|Initialise _output_get (Variables|Default|GetFishingMgr)))
    (:then_1
      (Default|SetCameraMode (Variables|Default|GetFishingMgr) true))))

(event Input|EnhancedActionEvents|EnhancedInputActionIA_FishLook
  (params (ActionValue :type Vector%202D%20Structure) (ElapsedSeconds :type Float%20%28double-precision%29) (TriggeredSeconds :type Float%20%28double-precision%29) (InputAction :type Input%20Action%20Object%20Reference :default "/Game/Input/Fishing/IA_FishLook.IA_FishLook"))
  (bind _fishingmgr (Variables|Default|GetFishingMgr))
  (bind _fishvictim (Variables|Default|GetFishVictim))
  (bind _fishingmgr_2 (Variables|Default|GetFishingMgr))
  (bind _returnvalue (Transformation|GetActorLocation _fishvictim))
  (bind _boat (Variables|/Game/Blueprints/Fishing/BP_FishingPawn.BP_FishingPawn_C|GetBoat _fishingmgr_2))
  (bind _steeringdirection (Variables|/Game/Blueprints/Fishing/BP_FishingPawn.BP_FishingPawn_C|GetSteeringDirection _fishingmgr))
  (bind _returnvalue_2 (Transformation|GetWorldRotation _steeringdirection))
  (bind _returnvalue_3 (Transformation|GetActorLocation _boat))
  (bind _returnvalue_4 (- _returnvalue _returnvalue_3))
  (bind _returnvalue_5 (Math|Vector|Normalize _returnvalue_4))
  (bind _returnvalue_6 (Math|Rotator|MakeRotfromX _returnvalue_5))
  ;[0.6419 0.1643 1] Cursor movement
  (switch Utilities|FlowControl|Switch|SwitchonE_FishingStates (Variables|/Game/Blueprints/Fishing/BP_FishingPawn.BP_FishingPawn_C|GetFishing%20State (Variables|Default|GetFishingMgr))
    (:NewEnumerator2
      (Transformation|AddRelativeRotation _steeringdirection (Math|Rotator|MakeRotator 0.0 0.0 (* (.x ActionValue) 3.0)) false false)
      (Transformation|SetWorldRotation _steeringdirection (Math|Rotator|MakeRotator (.roll _returnvalue_2) (.pitch _returnvalue_2) (+ (Math|Float|Clamp(Float) (- (.yaw _returnvalue_2) (.yaw _returnvalue_6)) -2e+01 2e+01) (.yaw _returnvalue_6))) false false))))

(event Input|EnhancedActionEvents|EnhancedInputActionIA_FishReel
  (params (ActionValue :type Float%20%28double-precision%29) (ElapsedSeconds :type Float%20%28double-precision%29) (TriggeredSeconds :type Float%20%28double-precision%29) (InputAction :type Input%20Action%20Object%20Reference :default "/Game/Input/Fishing/IA_FishReel.IA_FishReel"))
  ;[1 0.2159 0.4694] Scroll control
  (if (Utilities|Enum|Equal(Enum) (Variables|/Game/Blueprints/Fishing/BP_FishingPawn.BP_FishingPawn_C|GetFishing%20State (Variables|Default|GetFishingMgr)) "NewEnumerator3")
    (bind _output_get (Variables|Default|SetCatchProgress (+ (Variables|Default|GetCatchProgress) (* (Math|Float|Clamp(Float) ActionValue -1.0 0.0) (Variables|FishFightParams|GetFScrollRate) -1.0))))
    (Default|SetProgress (Variables|Default|GetFishing%20Attributes) _output_get)
    (if (>= (Variables|Default|GetCatchProgress) 1.0) ; We done?
      (CallFunction|GameEnd true))))

(event Input|EnhancedActionEvents|EnhancedInputActionIA_FishCast
  (params (ActionValue :type Boolean) (ElapsedSeconds :type Float%20%28double-precision%29) (TriggeredSeconds :type Float%20%28double-precision%29) (InputAction :type Input%20Action%20Object%20Reference :default "/Game/Input/Fishing/IA_FishCast.IA_FishCast"))
  ;[0.3277 0.2491 1] Click control
  (:Started
    (if (Utilities|Enum|Equal(Enum) (Variables|/Game/Blueprints/Fishing/BP_FishingPawn.BP_FishingPawn_C|GetFishing%20State (Variables|Default|GetFishingMgr)) "NewEnumerator2")
      (CallFunction|ChangeinTension (Variables|FishFightParams|GetFTensionRiseRate)) ; Manual tension control
    )))

(event EventBeginPlay
  (bind _asbp_fishing_pawn (Utilities|Casting|CastToBP_FishingPawn (Components|GetOwner)))
  (bind _output_get (Variables|Default|SetFishingMgr _asbp_fishing_pawn))
  (Collision|BindEventtoOnComponentBeginOverlap (Variables|/Game/Blueprints/Fishing/BP_FishingPawn.BP_FishingPawn_C|GetFishBiteCollider _output_get) (delegate Custom|PotentialFishOverlap))
  (Variables|Default|SetFishing%20Attributes (Variables|/Game/Blueprints/Fishing/BP_FishingPawn.BP_FishingPawn_C|GetFishingAttributes (Variables|Default|GetFishingMgr))))

(event EventTick
  (params (DeltaSeconds :type Float%20%28single-precision%29))
  (bind _fishingmgr (Variables|Default|GetFishingMgr))
  (bind _fishingmgr_2 (Variables|Default|GetFishingMgr))
  (bind _fishingmgr_3 (Variables|Default|GetFishingMgr))
  (bind _fishvictim (Variables|Default|GetFishVictim))
  (bind _fishingmgr_4 (Variables|Default|GetFishingMgr))
  (bind _fishingmgr_5 (Variables|Default|GetFishingMgr))
  (bind _fishvictim_2 (Variables|Default|GetFishVictim))
  (bind _fishingmgr_6 (Variables|Default|GetFishingMgr))
  (bind _returnvalue (Transformation|GetActorLocation _fishingmgr_6))
  (bind _returnvalue_2 (Transformation|GetActorLocation _fishvictim_2))
  (bind _defaultsceneroot (Variables|/Game/Blueprints/Fishing/BP_FishingPawn.BP_FishingPawn_C|GetDefaultSceneRoot _fishingmgr))
  (bind _steeringdirection (Variables|/Game/Blueprints/Fishing/BP_FishingPawn.BP_FishingPawn_C|GetSteeringDirection _fishingmgr_2))
  (bind _bp_fishpawnfsmcomponent (Variables|/Game/Blueprints/Fish/BP_FishPawn.BP_FishPawn_C|GetBP_FishPawnFSMComponent _fishvictim))
  (bind _bobber (Variables|/Game/Blueprints/Fishing/BP_FishingPawn.BP_FishingPawn_C|GetBobber _fishingmgr_4))
  (bind _boat (Variables|/Game/Blueprints/Fishing/BP_FishingPawn.BP_FishingPawn_C|GetBoat _fishingmgr_2))
  (bind _playersteerindicator (Variables|/Game/Blueprints/Fishing/BP_FishingPawn.BP_FishingPawn_C|GetPlayerSteerIndicator _fishingmgr_5))
  (bind _returnvalue_3 (Transformation|GetWorldLocation _defaultsceneroot))
  (bind _returnvalue_4 (Transformation|GetWorldLocation _bobber))
  (bind _returnvalue_5 (Math|Vector|GetForwardVector _steeringdirection))
  (bind _returnvalue_6 (Transformation|GetActorLocation _boat))
  (bind _returnvalue_7 (- _returnvalue _returnvalue_2))
  (bind _aofdirection (Variables|/Game/Blueprints/Fish/BPC_FishPawnFSMComponent.BPC_FishPawnFSMComponent_C|GetAOFDirection _bp_fishpawnfsmcomponent))
  (bind _returnvalue_8 (Math|Vector|Normalize _aofdirection))
  (bind _returnvalue_9 (Math|Vector|VectorLength _returnvalue_7))
  (bind _returnvalue_10 (* _returnvalue_5 _returnvalue_9))
  (bind _returnvalue_11 (+ _returnvalue_10 _returnvalue_6))
  (bind _returnvalue_12 (- _returnvalue_11 _returnvalue_4))
  (bind _returnvalue_13 (Math|Vector|Normalize _returnvalue_12))
  (bind _returnvalue_14 (Math|Vector|DotProduct _returnvalue_13 _returnvalue_8))
  (bind _returnvalue_15 (< _returnvalue_14 -0.5))
  ;[1 0.1765 0.2063 1 41] Tick (act of fishing update)
  (switch Utilities|FlowControl|Switch|SwitchonE_FishingStates (Variables|/Game/Blueprints/Fishing/BP_FishingPawn.BP_FishingPawn_C|GetFishing%20State (Variables|Default|GetFishingMgr))
    (:NewEnumerator2
      (Variables|/Game/Blueprints/Fishing/BP_FishingPawn.BP_FishingPawn_C|SetRodSteerAngle _fishingmgr_3 (Class|KismetMathLibrary|DegAcos (Math|Vector|DotProduct (Math|Vector|Normalize (- (Transformation|GetWorldLocation (Variables|/Game/Blueprints/Fishing/BP_FishingPawn.BP_FishingPawn_C|GetPointer _fishingmgr)) _returnvalue_3)) (Math|Vector|Normalize (- (Transformation|GetWorldLocation (Variables|/Script/Engine.Actor|GetRootComponent (Variables|Default|GetFishVictim))) _returnvalue_3)))))
      (Transformation|SetWorldRotation (Variables|/Game/Blueprints/Fishing/BP_FishingPawn.BP_FishingPawn_C|GetPlayerSteerIndicator _fishingmgr_3) (Math|Rotator|FindLookatRotation (Transformation|GetWorldLocation (Variables|/Game/Blueprints/Fish/BP_FishPawn.BP_FishPawn_C|GetDefaultSceneRoot (Variables|Default|GetFishVictim))) (Transformation|GetWorldLocation (Variables|/Game/Blueprints/Fishing/BP_FishingPawn.BP_FishingPawn_C|GetPointer (Variables|Default|GetFishingMgr)))) false false) ; Sets rotation of UI helper...
      (Variables|/Script/Engine.ArrowComponent|SetArrowLength _playersteerindicator (Utilities|Operators|Divide (Math|Vector|VectorLength (- (Transformation|GetWorldLocation (Variables|/Game/Blueprints/Fishing/BP_FishingPawn.BP_FishingPawn_C|GetPointer _fishingmgr_5)) (Transformation|GetActorLocation (Variables|Default|GetFishVictim)))) (Variables|/Script/Engine.ArrowComponent|GetArrowSize _playersteerindicator) 0.35)) ; ...and length of it too\nThis is kind of unnecessary as\nthe direction is more important;\nUI concept designs should fix this
      (Transformation|SetWorldLocation (Variables|/Game/Blueprints/Fishing/BP_FishingPawn.BP_FishingPawn_C|GetBobber (Variables|Default|GetFishingMgr)) (Transformation|GetWorldLocation (Variables|/Game/Blueprints/Fish/BP_FishPawn.BP_FishPawn_C|GetDefaultSceneRoot (Variables|Default|GetFishVictim))) false false) ; Move bobber over fish
      (Utilities|FlowControl|Sequence
        (:then_0
          ;[0.5871 1 0.5667] Cosmetic changes
          (Components|Arrow|SetArrowColor(LinearColor) (Variables|/Game/Blueprints/Fishing/BP_FishingPawn.BP_FishingPawn_C|GetPlayerSteerIndicator _fishingmgr_6) (Math|Color|SelectColor "(R=0.000000,G=1.000000,B=0.000000,A=1.000000)" "(R=1.000000,G=0.000000,B=0.000000,A=1.000000)" _returnvalue_15)) ; Change colour of arrow based on \nwhether or not you're succeeding the pull
          (Transformation|SetRelativeLocation (Variables|/Game/Blueprints/Fishing/BP_FishingPawn.BP_FishingPawn_C|GetPointer _fishingmgr_6) (Math|Vector|MakeVector _returnvalue_9 0.0 0.0) false false))
        (:then_1
          ;[1 0.4782 0.5081] Value changes
          (CallFunction|ChangeinTension (* (Variables|FishFightParams|GetFTensionFallRate) (Utilities|Time|GetWorldDeltaSeconds) -1.0)) ; Gradual fall in tension
          (bind _output_get (Variables|Default|SetFishStamina (Math|Float|Clamp(Float) (+ (Variables|Default|GetFishStamina) (* (Utilities|Time|GetWorldDeltaSeconds) (Math|Float|SelectFloat (Variables|FishFightParams|GetFStaminaDrainRate) (Variables|FishFightParams|GetFStaminaRecoverRate) _returnvalue_15)))))) ; Change in stamina
          ;[0.165 0.4372 1] Switch state when fish is tired out
          (if (<= _output_get 0.0)
            (Variables|/Game/Blueprints/Fishing/BP_FishingPawn.BP_FishingPawn_C|SetFishing%20State (Variables|Default|GetFishingMgr) "NewEnumerator3")
            (Default|UpdateInstructions (Variables|Default|GetFishingHUD) false)
            (Default|ToggleReel (Variables|Default|GetFishVictim))
            (Rendering|SetVisibility (Variables|/Game/Blueprints/Fishing/BP_FishingPawn.BP_FishingPawn_C|GetPlayerSteerIndicator (Variables|Default|GetFishingMgr)) false false)))))
    (:NewEnumerator3
      ;[0.4423 1 0.399] When reeling in fish
      (bind _output_get_2 (Variables|Default|SetFishStamina (Math|Float|Clamp(Float) (+ (Variables|Default|GetFishStamina) (* (Utilities|Time|GetWorldDeltaSeconds) (/ 1.0 (Variables|FishFightParams|GetFTiredRevivalTime))))))) ; Replenish stamina when reeling
      (if (>= _output_get_2 1.0)
        (Variables|/Game/Blueprints/Fishing/BP_FishingPawn.BP_FishingPawn_C|SetFishing%20State (Variables|Default|GetFishingMgr) "NewEnumerator2")
        (Default|UpdateInstructions (Variables|Default|GetFishingHUD) true)
        (Default|ToggleReel (Variables|Default|GetFishVictim))
        (Rendering|SetVisibility (Variables|/Game/Blueprints/Fishing/BP_FishingPawn.BP_FishingPawn_C|GetPlayerSteerIndicator (Variables|Default|GetFishingMgr)) true false)))))