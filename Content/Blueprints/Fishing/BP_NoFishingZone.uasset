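; BP_NoFishingZone is a volume that tells actors when they are inside an area where fishing is not allowed.
; When Enabled, its Zone component sends NoFishingZoneMessage(true) through BPI_FishingZoneReactor to implementing actors on overlap begin, and false on overlap end.
; BeginPlay also scans actors already overlapping the zone, so those starting inside receive the message.
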(event OnComponentBeginOverlap(Zone)
  (params (OverlappedComponent :type Primitive%20Component%20Object%20Reference) (OtherActor :type Actor%20Object%20Reference) (OtherComp :type Primitive%20Component%20Object%20Reference) (OtherBodyIndex :type Integer) (bFromSweep :type Boolean) (SweepResult :type Hit%20Result%20Structure%20%28by%20ref%29))
  (if (Variables|Default|GetEnabled)
    (if (Utilities|DoesObjectImplementInterface OtherActor "/Game/Blueprints/Fishing/BPI_FishingZoneReactor.BPI_FishingZoneReactor_C")
      (Class|BPIFishingZoneReactor|NoFishingZone(Message) OtherActor true))))

(event OnComponentEndOverlap(Zone)
  (params (OverlappedComponent :type Primitive%20Component%20Object%20Reference) (OtherActor :type Actor%20Object%20Reference) (OtherComp :type Primitive%20Component%20Object%20Reference) (OtherBodyIndex :type Integer))
  (if (Variables|Default|GetEnabled)
    (if (Utilities|DoesObjectImplementInterface OtherActor "/Game/Blueprints/Fishing/BPI_FishingZoneReactor.BPI_FishingZoneReactor_C")
      (Class|BPIFishingZoneReactor|NoFishingZone(Message) OtherActor false))))

(event EventBeginPlay
  (if (Variables|Default|GetEnabled)
    (for _array_element (Collision|GetOverlappingActors (Variables|Default|GetZone) 0 :!class /Script/Engine.PrimitiveComponent)
      (if (Utilities|DoesObjectImplementInterface _array_element "/Game/Blueprints/Fishing/BPI_FishingZoneReactor.BPI_FishingZoneReactor_C")
        (Class|BPIFishingZoneReactor|NoFishingZone(Message) _array_element true)))))

(fn ConstructionScript)