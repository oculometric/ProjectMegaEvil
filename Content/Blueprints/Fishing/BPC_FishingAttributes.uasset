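; Fishing attributes component that handles tension, progress, money and the fish inventory.
; Setter events broadcast tension, progress and money through event dispatchers, with the money delta added to Money and clamped between zero and MaxMoney.
; Added fish go into InventoryData, then the inventory in the fishing player controller's menu UI is refreshed directly rather than through a dispatcher.
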(event Custom|SetTension
  (params (Tension :type Float%20%28double-precision%29))
  ;[1 1 1] Call the event dispatchers whenever their respective variables change :)
  (Default|CallETensionUpdated Tension))

(event Custom|SetProgress
  (params (Progress :type Float%20%28double-precision%29))
  ;[1 1 1] Call the event dispatchers whenever their respective variables change :)
  (Default|CallEProgressUpdated Progress))

(event Custom|AddToInventory
  (params (Fish :type F%20Fish%20Inventory%20Info%20Structure))
  ;[1 1 1] Adding Fish
  (Utilities|Array|Add (Variables|Default|GetInventoryData) Fish)
  (bind _asbp_fishing_player_controller (Utilities|Casting|CastToBP_FishingPlayerController (Game|GetPlayerController 0)))
  (Default|UpdateInventory (Variables|/Game/Blueprints/BP_FishingPlayerController.BP_FishingPlayerController_C|GetPlayerMenuUI _asbp_fishing_player_controller)))

(event Custom|UpdateMoney
  (params (DeltaMoney :type Integer))
  (Default|CallEMoneyUpdated (Math|Integer|Clamp(Integer) (+ DeltaMoney (Variables|Default|GetMoney)) 0 (Variables|Default|GetMaxMoney))))