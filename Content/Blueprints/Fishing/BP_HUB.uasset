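; BP_HUB is a hub actor in the fishing game with a no-fishing zone and an interaction area.
; When enabled, the NoFishZone volume sets and clears the no-fishing flag on any BP_BoatPawn entering or leaving it.
; InteractBox overlaps, unfiltered by actor, toggle the interact prompt on the boat HUD and CanInteract on the first player's controller.
; The BeginPlay scan for already-overlapping boats only casts them, without setting the flag.
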(event OnComponentBeginOverlap(NoFishZone)
  (params (OverlappedComponent :type Primitive%20Component%20Object%20Reference) (OtherActor :type Actor%20Object%20Reference) (OtherComp :type Primitive%20Component%20Object%20Reference) (OtherBodyIndex :type Integer) (bFromSweep :type Boolean) (SweepResult :type Hit%20Result%20Structure%20%28by%20ref%29))
  ;[1 1 1] NoFishingZone
  (if (Variables|Default|GetEnabled)
    (bind _asbp_boat_pawn (Utilities|Casting|CastToBP_BoatPawn OtherActor))
    (Default|SetNoFishingZone _asbp_boat_pawn true)))

(event OnComponentEndOverlap(NoFishZone)
  (params (OverlappedComponent :type Primitive%20Component%20Object%20Reference) (OtherActor :type Actor%20Object%20Reference) (OtherComp :type Primitive%20Component%20Object%20Reference) (OtherBodyIndex :type Integer))
  ;[1 1 1] NoFishingZone
  (if (Variables|Default|GetEnabled)
    (bind _asbp_boat_pawn (Utilities|Casting|CastToBP_BoatPawn OtherActor))
    (Default|SetNoFishingZone _asbp_boat_pawn false)))

(event OnComponentBeginOverlap(InteractBox)
  (params (OverlappedComponent :type Primitive%20Component%20Object%20Reference) (OtherActor :type Actor%20Object%20Reference) (OtherComp :type Primitive%20Component%20Object%20Reference) (OtherBodyIndex :type Integer) (bFromSweep :type Boolean) (SweepResult :type Hit%20Result%20Structure%20%28by%20ref%29))
  (bind _asbp_fishing_player_controller (Utilities|Casting|CastToBP_FishingPlayerController (Game|GetPlayerController 0)))
  (Widget|SetVisibility (Variables|/Game/UI/BoatHUD/WBP_BoatHUD.WBP_BoatHUD_C|GetWBP_InteractPrompt (Variables|/Game/Blueprints/BP_FishingPlayerController.BP_FishingPlayerController_C|GetBoatHUD _asbp_fishing_player_controller)) "Visible")
  (Variables|/Game/Blueprints/BP_FishingPlayerController.BP_FishingPlayerController_C|SetbCanInteract _asbp_fishing_player_controller true))

(event OnComponentEndOverlap(InteractBox)
  (params (OverlappedComponent :type Primitive%20Component%20Object%20Reference) (OtherActor :type Actor%20Object%20Reference) (OtherComp :type Primitive%20Component%20Object%20Reference) (OtherBodyIndex :type Integer))
  (bind _asbp_fishing_player_controller (Utilities|Casting|CastToBP_FishingPlayerController (Game|GetPlayerController 0)))
  (Widget|SetVisibility (Variables|/Game/UI/BoatHUD/WBP_BoatHUD.WBP_BoatHUD_C|GetWBP_InteractPrompt (Variables|/Game/Blueprints/BP_FishingPlayerController.BP_FishingPlayerController_C|GetBoatHUD _asbp_fishing_player_controller)) "Hidden")
  (Variables|/Game/Blueprints/BP_FishingPlayerController.BP_FishingPlayerController_C|SetbCanInteract _asbp_fishing_player_controller false))

(event EventBeginPlay
  ;[1 1 1] NoFishingZone
  (if (Variables|Default|GetEnabled)
    (for _array_element (Collision|GetOverlappingActors (Variables|Default|GetNoFishZone) 0 :!class /Script/Engine.PrimitiveComponent)
      (Utilities|Casting|CastToBP_BoatPawn _array_element))))

(fn ConstructionScript)