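; BP_FishSpawner spawns a randomly chosen fish suited to a given area, depth and time.
; SpawnFish filters DT_FishParameters rows by those three conditions and maps each match's rarity to a spawn weight.
; A cumulative weighted roll picks one row, whose data goes to a new BP_FishPawn at the given position with random yaw.
; The event graph is inactive, and GetNearbyDepthClasses is an empty stub.
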(event EventBeginPlay)

(event Collision|EventActorBeginOverlap
  (params (OtherActor :type Actor%20Object%20Reference)))

(event EventTick
  (params (DeltaSeconds :type Float%20%28single-precision%29)))

(fn ConstructionScript)

(fn SpawnFish
  (params (Area :type E_FishArea%20Enum :default "NewEnumerator0") (Depth :type E_FishDepth%20Enum :default "NewEnumerator0") (Time :type E_FishTime%20Enum :default "NewEnumerator0") (Position :type Vector))
  (bind _fishspawnchances (LocalVariables|GetFishSpawnChances))
  (bind _spawnablefishnames (LocalVariables|GetSpawnableFishNames))
  (bind _outrownames (DataTable|GetDataTableRowNames "/Game/DataAssets/DT_FishParameters.DT_FishParameters"))
  (Utilities|Map|Clear (LocalVariables|GetSpawnableFishNames))
  (for _array_element _outrownames
    (bind _returnvalue (Utilities|GetDataTableRow "/Game/DataAssets/DT_FishParameters.DT_FishParameters" _array_element)
      (:then
        (if (Math|Boolean|ANDBoolean (Utilities|Array|ContainsItem (.SpawnableAreas (Utilities|Struct|BreakS_Fish _returnvalue)) Area) (Utilities|Array|ContainsItem (.SpawnableDepths (Utilities|Struct|BreakS_Fish _returnvalue)) Depth) (Utilities|Array|ContainsItem (.SpawnableTimes (Utilities|Struct|BreakS_Fish _returnvalue)) Time))
          (Utilities|Map|Add (LocalVariables|GetSpawnableFishNames) _array_element _returnvalue)))))
  (LocalVariables|SetTotalFishSpawnChance 0.0)
  (Utilities|Map|Clear _fishspawnchances)
  (bind _keys (Utilities|Map|Keys _spawnablefishnames))
  (for _array_element_2 _keys
    (Utilities|Map|Add (LocalVariables|GetFishSpawnChances) _array_element_2 (Utilities|Select :Index (.Rarity (Utilities|Struct|BreakS_Fish (.Value (Utilities|Map|Find _spawnablefishnames _array_element_2)))) :NewEnumerator0 0.55 :NewEnumerator1 0.3 :NewEnumerator2 0.148 :NewEnumerator3 0.02))
    (LocalVariables|SetTotalFishSpawnChance (+ (LocalVariables|GetTotalFishSpawnChance) (Utilities|Select :Index (.Rarity (Utilities|Struct|BreakS_Fish (.Value (Utilities|Map|Find _spawnablefishnames _array_element_2)))) :NewEnumerator0 0.55 :NewEnumerator1 0.3 :NewEnumerator2 0.148 :NewEnumerator3 0.02))))
  (bind _keys_2 (Utilities|Map|Keys _fishspawnchances))
  (LocalVariables|SetTrackedFishSpawnChance (* (Math|Random|RandomFloat) (LocalVariables|GetTotalFishSpawnChance)))
  (bind _array_element_3 (Utilities|Array|ForEachLoopwithBreak _keys_2 :!label _label)
    (:LoopBody
      (bind _output_get (LocalVariables|SetTrackedFishSpawnChance (- (LocalVariables|GetTrackedFishSpawnChance) (.Value (Utilities|Map|Find (LocalVariables|GetFishSpawnChances) _array_element_3)))))
      (if (<= _output_get 0.0)
        (LocalVariables|SetFishToSpawn _array_element_3)
        (goto _label Break)))
    (:Completed
      (Game|SpawnActorfromClass "/Game/Blueprints/Fish/BP_FishPawn.BP_FishPawn_C" (Math|Transform|MakeTransform Position (Math|Rotator|MakeRotator 0.0 0.0 (* (Math|Random|RandomFloat) 3.6e+02)) "1.000000,1.000000,1.000000") "Undefined" "MultiplyWithRoot" 0 (.Value (Utilities|Map|Find (LocalVariables|GetSpawnableFishNames) (LocalVariables|GetFishToSpawn))) 0))))