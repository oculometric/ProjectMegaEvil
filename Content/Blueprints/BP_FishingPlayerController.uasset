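; Player controller for the boat fishing game that owns the UI and routes menu, pause and day-end input.
; BeginPlay waits briefly, caches the boat and fisher, adds the boat input context, then creates the tabbed player menu, pause menu, HUD and day-end screen, and initialises the weekly quota manager.
; MenuSwitching toggles menu tabs, cursor, input mode and HUD.
; Interact ends the day; debug keys damage or heal the boat.
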(event Input|EnhancedActionEvents|EnhancedInputActionIA_Pause
  (params (ActionValue :type Boolean) (ElapsedSeconds :type Float%20%28double-precision%29) (TriggeredSeconds :type Float%20%28double-precision%29) (InputAction :type Input%20Action%20Object%20Reference :default "/Game/Input/IA_Pause.IA_Pause"))
  ;[1 1 1] Inventory Widget
  (:Started
    (if (not (Widget|IsVisible (Variables|Default|GetDayEndUI)))
      (CallFunction|MenuClose)
      (UserInterface|Viewport|AddtoViewport (Variables|Default|GetPauseMenuUI) 0))))

(event Input|EnhancedActionEvents|EnhancedInputActionIA_Interact
  (params (ActionValue :type Boolean) (ElapsedSeconds :type Float%20%28double-precision%29) (TriggeredSeconds :type Float%20%28double-precision%29) (InputAction :type Input%20Action%20Object%20Reference :default "/Game/Input/Boat/IA_Interact.IA_Interact"))
  ;[1 1 0] Interaction
  (:Started
    (if (Math|Boolean|ANDBoolean (Variables|Default|GetbCanInteract) (not (Widget|IsVisible (Variables|Default|GetPlayerMenuUI))) (not (Widget|IsVisible (Variables|Default|GetPauseMenuUI))))
      (Input|RemoveMappingContext (PlayerController|LocalPlayerSubsystems|GetEnhancedInputLocalPlayerSubsystem) "/Game/Input/Boat/IMC_Boat.IMC_Boat" "(bIgnoreAllPressedKeysUntilRelease=True,bForceImmediately=False,bNotifyUserSettings=False)")
      (Default|EndDay (Variables|Default|GetDayEndUI)))))

(event Input|EnhancedActionEvents|EnhancedInputActionIA_Inventory
  (params (ActionValue :type Boolean) (ElapsedSeconds :type Float%20%28double-precision%29) (TriggeredSeconds :type Float%20%28double-precision%29) (InputAction :type Input%20Action%20Object%20Reference :default "/Game/Input/Boat/IA_Inventory.IA_Inventory"))
  ;[1 1 1] Inventory Widget
  (:Started
    (if (Utilities|Enum|Equal(Enum) (Variables|/Game/Blueprints/Fishing/BP_FishingPawn.BP_FishingPawn_C|GetFishing%20State (Variables|Default|GetFisher)) "NewEnumerator0")
      (CallFunction|MenuSwitching))))

(event Input|EnhancedActionEvents|EnhancedInputActionIA_Map
  (params (ActionValue :type Boolean) (ElapsedSeconds :type Float%20%28double-precision%29) (TriggeredSeconds :type Float%20%28double-precision%29) (InputAction :type Input%20Action%20Object%20Reference :default "/Game/Input/Boat/IA_Map.IA_Map"))
  ;[1 1 1] Inventory Widget
  (:Started
    (CallFunction|MenuSwitching 1)))

(event Input|EnhancedActionEvents|EnhancedInputActionIA_Fishopedia
  (params (ActionValue :type Boolean) (ElapsedSeconds :type Float%20%28double-precision%29) (TriggeredSeconds :type Float%20%28double-precision%29) (InputAction :type Input%20Action%20Object%20Reference :default "/Game/Input/Boat/IA_Fishopedia.IA_Fishopedia"))
  ;[1 1 1] Inventory Widget
  (:Started
    (CallFunction|MenuSwitching 2)))

(event Input|EnhancedActionEvents|EnhancedInputActionIA_Options
  (params (ActionValue :type Boolean) (ElapsedSeconds :type Float%20%28double-precision%29) (TriggeredSeconds :type Float%20%28double-precision%29) (InputAction :type Input%20Action%20Object%20Reference :default "/Game/Input/Boat/IA_Options.IA_Options"))
  ;[1 1 1] Inventory Widget
  (:Started
    (CallFunction|MenuSwitching 3)))

(event EventBeginPlay
  (bind _returnvalue (PlayerController|LocalPlayerSubsystems|GetEnhancedInputLocalPlayerSubsystem))
  (bind _self self)
  ;[1 1 1] Setup
  (Utilities|FlowControl|Delay 0.2)
  (bind _asbp_boat_pawn (Utilities|Casting|CastToBP_BoatPawn (Pawn|GetControlledPawn)))
  (bind _output_get (Variables|Default|SetBoat _asbp_boat_pawn))
  (Variables|Default|SetFisher (Variables|/Game/Blueprints/BP_BoatPawn.BP_BoatPawn_C|GetFisher _output_get))
  (Utilities|IsValid _returnvalue
    (:Is%20Valid
      (Input|AddMappingContext _returnvalue "/Game/Input/Boat/IMC_Boat.IMC_Boat" 0 "(bIgnoreAllPressedKeysUntilRelease=True,bForceImmediately=False,bNotifyUserSettings=False)")
      (Utilities|FlowControl|Sequence
        (:then_0
          (bind _returnvalue_2 (UserInterface|CreateWidget "/Game/UI/MenuPrototypes/WBP_PlayerMenu.WBP_PlayerMenu_C" _self))
          (bind _output_get_2 (Variables|Default|SetPlayerMenuUI _returnvalue_2))
          (UserInterface|Viewport|AddtoViewport _output_get_2 0)
          (Widget|SetVisibility _output_get_2 "Hidden")
          (Default|Initialize _output_get_2 (Variables|Default|GetFisher)))
        (:then_1
          (bind _returnvalue_3 (UserInterface|CreateWidget "/Game/UI/MenuPrototypes/WBP_PauseMenu.WBP_PauseMenu_C" _self))
          (Variables|Default|SetPauseMenuUI _returnvalue_3))
        (:then_2
          (bind _returnvalue_4 (UserInterface|CreateWidget "/Game/UI/BoatHUD/WBP_BoatHUD.WBP_BoatHUD_C" _self))
          (bind _output_get_3 (Variables|Default|SetBoatHUD _returnvalue_4))
          (UserInterface|Viewport|AddtoViewport _output_get_3 0)
          (Default|Initialise _output_get_3 (Variables|Default|GetBoat))
          (bind _returnvalue_5 (Actor|GetActorOfClass "/Game/Blueprints/BP_WeeklyQuotaManager.BP_WeeklyQuotaManager_C"))
          (Default|Initialise _returnvalue_5 _output_get_3))
        (:then_3
          (bind _returnvalue_6 (UserInterface|CreateWidget "/Game/UI/Shop/WBP_DayEndUI.WBP_DayEndUI_C" _self))
          (bind _output_get_4 (Variables|Default|SetDayEndUI _returnvalue_6))
          (UserInterface|Viewport|AddtoViewport _output_get_4 0)
          (Widget|SetVisibility _output_get_4 "Hidden")
          (Default|Initialise _output_get_4 (Variables|Default|GetBoat) (Variables|Default|GetFisher) _self))))
    (:Is%20Not%20Valid
      (Development|PrintString "EILPS Not Valid"))))

(event Input|KeyboardEvents|DebugKey7
  (params (Key :type Key%20Structure :default "None") (ActionValue :type Input%20Action%20Value%20Structure))
  ;[1 0 0] Damage Debug
  (:Pressed
    (Game|Damage|ApplyDamage (Variables|Default|GetBoat) 2e+01 0 0)))

(event Input|KeyboardEvents|DebugKey8
  (params (Key :type Key%20Structure :default "None") (ActionValue :type Input%20Action%20Value%20Structure))
  ;[1 0 0] Damage Debug
  (:Pressed
    (Game|Damage|ApplyDamage (Variables|Default|GetBoat) -2e+01 0 0)))

(fn ConstructionScript)

(fn MenuSwitching
  (params (TabIndex :type Integer))
  (bind _self self)
  (bind _boathud (Variables|Default|GetBoatHUD))
  (bind _playermenuui (Variables|Default|GetPlayerMenuUI))
  (Utilities|IsValid _playermenuui
    (:Is%20Valid
      (if (and (Widget|IsVisible _playermenuui) (== TabIndex (Variables|/Game/UI/MenuPrototypes/WBP_PlayerMenu.WBP_PlayerMenu_C|GetActiveMenu _playermenuui)))
        (Widget|SetVisibility _playermenuui "Hidden")
        (Input|SetInputModeGameOnly _self false)
        (Variables|Default|SetbShowMouseCursor false)
        (Default|SetHUDVisibility _boathud true)
        (else
          (Widget|SetVisibility _playermenuui "Visible")
          (Input|SetInputModeGameandUI _self _playermenuui "DoNotLock" false false)
          (Variables|Default|SetbShowMouseCursor true)
          (Default|SwitchTab _playermenuui TabIndex)
          (Default|SetHUDVisibility _boathud false))))))

(fn MenuClose
  (Widget|SetVisibility (Variables|Default|GetPlayerMenuUI) "Hidden")
  (Input|SetInputModeGameOnly self false)
  (Variables|Default|SetbShowMouseCursor false)
  (Default|SetHUDVisibility (Variables|Default|GetBoatHUD) true))