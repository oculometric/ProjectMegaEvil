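; BP_GameStateSaver is the fishing game's save object, persisting the player's current bait and money in a single fixed slot.
; UpdateSaveGame copies both values from the passed FishingAttributes, then the object saves itself to that slot.
; LoadSaveGame, if a save exists, writes the stored values back into FishingAttributes and calls its bait and money update functions with zero, apparently to refresh dependent state.
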(event Custom|UpdateSaveGame
  (params (FishingAttributes :type BPC%20Fishing%20Attributes%20Object%20Reference))
  (Variables|Default|SetCurrentBait (Variables|/Game/Blueprints/Fishing/BPC_FishingAttributes.BPC_FishingAttributes_C|GetCurrentBait FishingAttributes))
  (Variables|Default|SetCurrentMoney (Variables|/Game/Blueprints/Fishing/BPC_FishingAttributes.BPC_FishingAttributes_C|GetCurrentMoney FishingAttributes))
  (SaveGame|SaveGametoSlot self "fish"))

(event Custom|LoadSaveGame
  (params (FishingAttributes :type BPC%20Fishing%20Attributes%20Object%20Reference))
  (bind _returnvalue (SaveGame|DoesSaveGameExist "fish"))
  (if _returnvalue
    (bind _returnvalue_2 (SaveGame|LoadGamefromSlot "fish"))
    (Variables|/Game/Blueprints/Fishing/BPC_FishingAttributes.BPC_FishingAttributes_C|SetCurrentBait FishingAttributes (Variables|BP_GameStateSaver_C|GetCurrentBait (.AsBP%20Game%20State%20Saver (Utilities|Casting|CastToBP_GameStateSaver _returnvalue_2))))
    (Variables|/Game/Blueprints/Fishing/BPC_FishingAttributes.BPC_FishingAttributes_C|SetCurrentMoney FishingAttributes (Variables|BP_GameStateSaver_C|GetCurrentMoney (.AsBP%20Game%20State%20Saver (Utilities|Casting|CastToBP_GameStateSaver _returnvalue_2))))
    (Default|UpdateBait FishingAttributes)
    (Default|UpdateMoney FishingAttributes)))