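; BP_FishPawn is a spawner-managed fish for the fishing minigame.
; On BeginPlay it applies FishData, rolls length and weight, derives sell value and inventory data, then scales in by timeline.
; Overlaps with the fishing pawn, targeting, fleeing and reel state feed its FSM component, while leaving the spawner's area triggers a despawn.
; DT_FishMath drives price and difficulty formulas, and a Perlin-noise random roll computes quality from fishing power.
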(event OnComponentEndOverlap(FishCollider)
  (params (OverlappedComponent :type Primitive%20Component%20Object%20Reference) (OtherActor :type Actor%20Object%20Reference) (OtherComp :type Primitive%20Component%20Object%20Reference) (OtherBodyIndex :type Integer))
  ;[1 1 0] Overlapping
  (if (== OtherActor (Variables|Default|GetSpawner))
    (CallFunction|Kill)
    (elif (not (Utilities|Enum|Equal(Enum) (Variables|/Game/Blueprints/Fish/BPC_FishPawnFSMComponent.BPC_FishPawnFSMComponent_C|GetFishFSM (Variables|Default|GetBP_FishPawnFSMComponent)) "NewEnumerator2"))
      (if (.bSuccess (Utilities|Casting|CastToBP_FishingPawn OtherActor))
        (Variables|/Game/Blueprints/Fish/BPC_FishPawnFSMComponent.BPC_FishPawnFSMComponent_C|SetFishing (Variables|Default|GetBP_FishPawnFSMComponent) false)))))

(event OnComponentBeginOverlap(FishCollider)
  (params (OverlappedComponent :type Primitive%20Component%20Object%20Reference) (OtherActor :type Actor%20Object%20Reference) (OtherComp :type Primitive%20Component%20Object%20Reference) (OtherBodyIndex :type Integer) (bFromSweep :type Boolean) (SweepResult :type Hit%20Result%20Structure%20%28by%20ref%29))
  (bind (_asbp_fishing_pawn _bsuccess) (Utilities|Casting|CastToBP_FishingPawn OtherActor))
  (bind _bp_fishpawnfsmcomponent (Variables|Default|GetBP_FishPawnFSMComponent))
  ;[1 1 0] Overlapping
  (if (not (Utilities|Enum|Equal(Enum) (Variables|/Game/Blueprints/Fish/BPC_FishPawnFSMComponent.BPC_FishPawnFSMComponent_C|GetFishFSM (Variables|Default|GetBP_FishPawnFSMComponent)) "NewEnumerator2"))
    (if _bsuccess
      (Variables|/Game/Blueprints/Fish/BPC_FishPawnFSMComponent.BPC_FishPawnFSMComponent_C|SetFishingMngr _bp_fishpawnfsmcomponent _asbp_fishing_pawn)
      (Variables|/Game/Blueprints/Fish/BPC_FishPawnFSMComponent.BPC_FishPawnFSMComponent_C|SetFishing _bp_fishpawnfsmcomponent true))))

(event Custom|Kill
  (bind _spawner (Variables|Default|GetSpawner))
  ;[1 1 1] Kill
  (bind _fishscale (Timeline|FishDespawn PlayFromStart)
    (:Update
      (Transformation|SetRelativeScale3D (Variables|Default|GetFishMesh) (Math|Conversions|ToVector(Float) _fishscale)))
    (:Finished
      (Actor|DestroyActor)
      (Variables|/Game/Blueprints/BP_FishSpawner.BP_FishSpawner_C|SetTotalFish _spawner (- (Variables|/Game/Blueprints/BP_FishSpawner.BP_FishSpawner_C|GetTotalFish _spawner) 1)))))

(event Custom|Catch%20Fish
  (bind _spawner (Variables|Default|GetSpawner))
  ;[1 1 1] Catch
  (Variables|/Game/Blueprints/BP_FishSpawner.BP_FishSpawner_C|SetTotalFish _spawner (- (Variables|/Game/Blueprints/BP_FishSpawner.BP_FishSpawner_C|GetTotalFish _spawner) 1)))

(event Custom|BecomeMinigameTarget
  (params (Boat :type BP%20Boat%20Pawn%20Object%20Reference))
  ;[1 1 1] Become Target
  (Default|SwitchState (Variables|Default|GetBP_FishPawnFSMComponent) "NewEnumerator2"))

(event Custom|Generate%20Weight%20and%20Length
  (params (MinLength :type Float%20%28double-precision%29) (MaxLength :type Float%20%28double-precision%29) (MinWeight :type Float%20%28double-precision%29) (MaxWeight :type Float%20%28double-precision%29))
  ;[1 1 1] Data generation
  (bind _rounded_value (CallFunction|RoundValue (Math|Random|RandomFloatinRange MinLength MaxLength) 0.0))
  (bind _output_get (Variables|Default|SetLength _rounded_value))
  (bind _rounded_value_2 (CallFunction|RoundValue (Math|Random|RandomFloatinRange MinWeight MaxWeight) 0.0))
  (Variables|Default|SetWeight _rounded_value_2)
  (Transformation|SetRelativeScale3D (Variables|Default|GetFishMesh) (Math|Conversions|ToVector(Float) _output_get)))

(event Custom|FleeFromTarget
  (params (FleeTarget :type Actor%20Object%20Reference))
  ;[1 1 1] Runs Flee From a Set Actor e.g shark, boat
  (Default|FleefromLocation (Variables|Default|GetBP_FishPawnFSMComponent) FleeTarget))

(event Custom|ConfigureFromData
  (bind _fishdata (Variables|Default|GetFishData))
  (bind _fishdata_2 (Variables|Default|GetFishData))
  (bind (_id _fishmesh _fishicon _name _pokedexdescription _caught _rarity _fishinglevel _difficulty _minlength _maxlength _minweight _maxweight) (Utilities|Struct|BreakF_Fish _fishdata_2))
  (bind (_id_2 _fishmesh_2 _fishicon_2 _name_2 _pokedexdescription_2 _caught_2 _rarity_2 _fishinglevel_2 _difficulty_2) (Utilities|Struct|BreakF_Fish _fishdata))
  ;[1 1 1] Config
  (Components|StaticMesh|SetStaticMesh (Variables|Default|GetFishMesh) _fishmesh)
  (CallFunction|GenerateWeightandLength _minlength _maxlength _minweight _maxweight)
  (Variables|Default|SetFishRarity _rarity_2)
  (Variables|Default|SetFishDifficulty _difficulty_2)
  (Variables|Default|SetFIshingLevel _fishinglevel_2)
  (bind _sell_price (CallFunction|CalculateSellPrice))
  (Variables|Default|SetSellValue _sell_price)
  (bind _fishinventorydata (CallFunction|CreateFishInventoryDesc))
  (Variables|Default|SetFishInventoryData _fishinventorydata)
  (CallFunction|CalculateDifficulty 1))

(event Custom|FailedMinigame
  ;[1 1 1] Failed
  (Default|FailedMinigame (Variables|Default|GetBP_FishPawnFSMComponent)))

(event Custom|ToggleReel
  (bind _bp_fishpawnfsmcomponent (Variables|Default|GetBP_FishPawnFSMComponent))
  ;[1 1 1] Toggles Fish to be in the reel state
  (Variables|/Game/Blueprints/Fish/BPC_FishPawnFSMComponent.BPC_FishPawnFSMComponent_C|SetIsTired _bp_fishpawnfsmcomponent (not (Variables|/Game/Blueprints/Fish/BPC_FishPawnFSMComponent.BPC_FishPawnFSMComponent_C|GetIsTired _bp_fishpawnfsmcomponent))))

(event EventBeginPlay
  (bind _spawner (Variables|Default|GetSpawner))
  ;[0 1 0] Begin Play
  (Variables|/Game/Blueprints/Fish/BPC_FishPawnFSMComponent.BPC_FishPawnFSMComponent_C|SetFishPawn (Variables|Default|GetBP_FishPawnFSMComponent) self)
  (CallFunction|ConfigurefromData)
  (bind _fishscale (Timeline|FishSpawn PlayFromStart)
    (:Update
      (Transformation|SetRelativeScale3D (Variables|Default|GetFishMesh) (Math|Conversions|ToVector(Float) _fishscale)))
    (:Finished
      (Utilities|IsValid _spawner
        (:Is%20Valid
          (EventDispatchers|BindEventtoKillFish _spawner (EventDispatchers|CreateEvent :!event Custom|Kill)))))))

(fn ConstructionScript)

(fn CreateFishInventoryDesc
  (bind _fishdata (Variables|Default|GetFishData))
  (bind (_id _fishmesh _fishicon _name) (Utilities|Struct|BreakF_Fish _fishdata))
  (bind _outrownames (DataTable|GetDataTableRowNames "/Game/DataAssets/DT_FishParameters.DT_FishParameters"))
  (for _array_element _outrownames
    (bind _returnvalue (Utilities|GetDataTableRow "/Game/DataAssets/DT_FishParameters.DT_FishParameters" _array_element)
      (:then
        (if (== (.ID (Utilities|Struct|BreakF_Fish _returnvalue)) (.ID (Utilities|Struct|BreakF_Fish (Variables|Default|GetFishData))))
          (Variables|Default|SetFishRowName _array_element)
          (return (Utilities|Struct|MakeF_FishInventoryInfo _id _name _fishicon 0.0 (Variables|Default|GetLength) (Variables|Default|GetWeight) (Variables|Default|GetFishRowName) (Variables|Default|GetDepth) (Variables|Default|GetTime) (Variables|Default|GetMapArea) (Variables|Default|GetFishRarity) (Variables|Default|GetFishQuality) (Variables|Default|GetFishData))))))))

(fn CalculateSellPrice
  (bind _returnvalue (Utilities|GetDataTableRow "/Game/DataAssets/DT_FishMath.DT_FishMath" "SellPrice")
    (:then
      (bind _rounded_value (CallFunction|RoundValue (* (+ (Variables|Default|GetLength) (/ (Variables|Default|GetWeight) (.Divisor (Utilities|Struct|BreakF_FishMathValues _returnvalue)))) (.Value (Utilities|Map|Find (.Rarities (Utilities|Struct|BreakF_FishMathValues _returnvalue)) (Variables|Default|GetFishRarity))) (.Value (Utilities|Map|Find (.Times (Utilities|Struct|BreakF_FishMathValues _returnvalue)) (Variables|Default|GetTime))) (.Multiplier (Utilities|Struct|BreakF_FishMathValues _returnvalue)) (.Value (Utilities|Map|Find (.Qualities (Utilities|Struct|BreakF_FishMathValues _returnvalue)) (Variables|Default|GetFishQuality))) (+ (.Value (Utilities|Map|Find (.Depths (Utilities|Struct|BreakF_FishMathValues _returnvalue)) (Variables|Default|GetDepth))) (.Value (Utilities|Map|Find (.Difficulties (Utilities|Struct|BreakF_FishMathValues _returnvalue)) (Variables|Default|GetFishDifficulty))) (/ (Variables|Default|GetFIshingLevel) (.Divisor (Utilities|Struct|BreakF_FishMathValues _returnvalue))))) (Math|Conversions|ToFloat(Integer) (.Round (Utilities|Struct|BreakF_FishMathValues _returnvalue)))))
      (return _rounded_value))))

(fn CalculateDifficulty
  (params (FishingPower :type Integer))
  (bind _quality (CallFunction|AssignQuality FishingPower))
  (bind _returnvalue (Utilities|GetDataTableRow "/Game/DataAssets/DT_FishMath.DT_FishMath" "DifficultyScaling")
    (:then
      (bind _rounded_value (CallFunction|RoundValue (* (/ (* (.Value (Utilities|Map|Find (.Rarities (Utilities|Struct|BreakF_FishMathValues _returnvalue)) (Variables|Default|GetFishRarity))) (.Value (Utilities|Map|Find (.Depths (Utilities|Struct|BreakF_FishMathValues _returnvalue)) (Variables|Default|GetDepth))) (.Value (Utilities|Map|Find (.Times (Utilities|Struct|BreakF_FishMathValues _returnvalue)) (Variables|Default|GetTime))) (.Value (Utilities|Map|Find (.Difficulties (Utilities|Struct|BreakF_FishMathValues _returnvalue)) (Variables|Default|GetFishDifficulty))) (/ (Variables|Default|GetFIshingLevel) FishingPower)) (.Divisor (Utilities|Struct|BreakF_FishMathValues _returnvalue))) (.Multiplier (Utilities|Struct|BreakF_FishMathValues _returnvalue))) (Math|Conversions|ToFloat(Integer) (.Round (Utilities|Struct|BreakF_FishMathValues _returnvalue)))))
      (bind _fishinventorydata (CallFunction|CreateFishInventoryDesc))
      (Variables|Default|SetFishInventoryData _fishinventorydata)
      (return (Math|Float|Max(Float) (Math|Float|Min(Float) _rounded_value (.MaxClamp (Utilities|Struct|BreakF_FishMathValues _returnvalue))) (.MinClamp (Utilities|Struct|BreakF_FishMathValues _returnvalue)))))))

(fn AssignQuality
  (params (FishingPower :type Integer))
  (bind _returnvalue (Math|Float|Absolute(Float) 14.0))
  (bind _returnvalue_2 (/ FishingPower _returnvalue))
  (bind _returnvalue_3 (Math|Random|RandomFloatinRange _returnvalue_2 1.0))
  (bind _returnvalue_4 (Class|KismetMathLibrary|PerlinNoise1D _returnvalue_3))
  (return (Utilities|Select :Index (Math|Integer|Min(Integer) (Math|Float|Round (* (Math|Random|RandomFloatinRange _returnvalue_3 (Math|Float|Min(Float) (Math|Float|Max(Float) (/ FishingPower (Math|Float|Absolute(Float) 28.0)) (* _returnvalue_4 (Math|Float|SelectFloat -1.0 1.0 (< _returnvalue_4 0.0)))) 1.0)) (* (Math|Float|Min(Float) (/ FishingPower (Math|Float|Absolute(Float) (Math|Random|RandomFloatinRange 1.0 4.0))) (Math|Random|RandomFloatinRange 0.425 1.5)) 2.25))) 2) :Option%200 "NewEnumerator0" :Option%201 "NewEnumerator1" :Option%202 "NewEnumerator2")))