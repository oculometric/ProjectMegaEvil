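; Fish AI component that drives a fish pawn through Wander, Bait Interested, Return, fishing minigame and Flee states.
; On BeginPlay it loads tuning from DT_FishAIParameters, randomises speed and runs the state machine on a looping timer instead of Tick.
; Fish wander around spawn, may chase the bobber while fishing is active, and flee after a failed minigame.
; Movement sets transforms directly; hooked fish pull sideways from the fishing manager, with Perlin noise picking the side.
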(event Custom|FleeFromLocation
  (params (Flee%20Target :type Actor%20Object%20Reference))
  ;[1 1 1] Set Flee Target and Run Flee
  (Variables|Default|SetFleeTarget Flee%20Target)
  (CallFunction|SwitchState "NewEnumerator3"))

(event Custom|Failed%20Minigame
  ;[1 1 1] Runs Flee Behaviour from the fisher
  (Variables|Default|SetFleeTarget (Variables|Default|GetFishingMngr))
  (CallFunction|SwitchState "NewEnumerator3"))

(event Custom|RunFSM
  ;[1 1 1] Intitialise FSM
  (CallFunction|FSMLogic))

(event Custom|Initialise
  ;[1 1 1] Parses Data table values into the matching Fish values
  (bind _returnvalue (Utilities|GetDataTableRow "/Game/DataAssets/DT_FishAIParameters.DT_FishAIParameters" "Default")
    (:then
      (Variables|Default|SetWanderRadius (.WanderDistance (Utilities|Struct|BreakF_FishAIParameters _returnvalue)))
      (Variables|Default|SetSpeed (.Speed (Utilities|Struct|BreakF_FishAIParameters _returnvalue)))
      (Variables|Default|SetRotationSpeed (.RotationSpeed (Utilities|Struct|BreakF_FishAIParameters _returnvalue)))
      (Variables|Default|SetAcceptanceRadius (.AcceptanceRadius (Utilities|Struct|BreakF_FishAIParameters _returnvalue)))
      (Variables|Default|SetLureChance (.LureChance (Utilities|Struct|BreakF_FishAIParameters _returnvalue)))
      (Variables|Default|Settimer (.Timer (Utilities|Struct|BreakF_FishAIParameters _returnvalue))))))

(event EventBeginPlay
  ;[1 1 1] Intitialise FSM
  (Utilities|FlowControl|DelayUntilNextTick)
  (Variables|Default|SetSpawnLocation (Transformation|GetActorLocation (Variables|Default|GetFishPawn)))
  (CallFunction|Initialise)
  (Variables|Default|SetSpeed (* (Variables|Default|GetSpeed) (Math|Random|RandomFloatinRange 0.75 1.5)))
  (CallFunction|SwitchState "NewEnumerator0")
  (Utilities|Time|SetTimerbyEvent (delegate Custom|RunFSM) (Variables|Default|Gettimer) true))

(event EventTick
  (params (DeltaSeconds :type Float%20%28single-precision%29))
  ;[1 1 1] Run FSM
)

(fn SwitchState
  (params (New%20State :type E_FishFSM%20Enum :default "NewEnumerator0"))
  (bind _fleetarget (Variables|Default|GetFleeTarget))
  (bind _returnvalue (Transformation|GetActorForwardVector _fleetarget))
  (bind _output_get (Variables|Default|SetFishFSM New%20State))
  (switch Utilities|FlowControl|Switch|SwitchonE_FishFSM _output_get
    (:NewEnumerator0
      (CallFunction|FindWanderLocation))
    (:NewEnumerator1
      (Variables|Default|SetTargetLocation (Transformation|GetWorldLocation (Variables|/Game/Blueprints/Fishing/BP_FishingPawn.BP_FishingPawn_C|GetBobber (Variables|Default|GetFishingMngr)))))
    (:NewEnumerator4
      (Variables|Default|SetTargetLocation (Variables|Default|GetSpawnLocation)))
    (:NewEnumerator2
      (Transformation|SetActorLocation (Variables|Default|GetFishPawn) (Transformation|GetWorldLocation (Variables|/Game/Blueprints/Fishing/BP_FishingPawn.BP_FishingPawn_C|GetFishBiteCollider (Variables|Default|GetFishingMngr))) false false))
    (:NewEnumerator3
      (Variables|Default|SetSpeed (* (Variables|Default|GetSpeed) 4e+01))
      (Variables|Default|SetTargetLocation (+ (Transformation|GetActorLocation _fleetarget) (* (Math|Vector|MakeVector (.x _returnvalue) (.y _returnvalue) (- (.z _returnvalue) 5e+01)) 2e+02)))))
  (return))

(fn FSMLogic
  ;[1 1 1] Runs different Fish states/behaviour
  (switch Utilities|FlowControl|Switch|SwitchonE_FishFSM (Variables|Default|GetFishFSM)
    (:NewEnumerator0
      ;[1 1 1] If the Player is not Fishing calls wander behaviour on fish
      (if (not (Variables|Default|GetFishing))
        (CallFunction|WandertoLocation :!label _label)
        (else
          ;[1 1 1] If the Player is Fishing there is a chance the fish gets interested in the rod, or continues to wander
          (if (>= (Math|Random|RandomFloat) (Variables|Default|GetLureChance))
            (goto _label)
            (else
              (CallFunction|SwitchState "NewEnumerator1")))))
      (return))
    (:NewEnumerator1
      ;[1 1 1] Runs the Bobber pathing behaviour, until the fish bites the bobber to start the fishing game
      (CallFunction|InterestedinBait)
      (return))
    (:NewEnumerator4
      ;[1 1 1] Return runs, if the fish loses interest in the bobber or the player stops fishing to path the fish to their spawn point
      (if (not (Variables|Default|GetFishing))
        (CallFunction|Return)
        (return)
        (elif (not (>= (Math|Random|RandomFloat) (Variables|Default|GetLureChance)))
          (CallFunction|SwitchState "NewEnumerator1")
          (return))))
    (:NewEnumerator2
      ;[1 1 1] State called to begin the fishing game
      (CallFunction|TheActOfFishing)
      (return))
    (:NewEnumerator3
      ;[1 1 1] State called if player fails the fishing game, to make the fish run away
      (CallFunction|Flee)
      (return))))

(fn WandertoLocation
  (if (<= (Math|Vector|Distance(Vector) (Transformation|GetActorLocation (Variables|Default|GetFishPawn)) (Variables|Default|GetTargetLocation)) (Variables|Default|GetAcceptanceRadius))
    (CallFunction|FindWanderLocation))
  (CallFunction|MovetoTargetLocation)
  (return))

(fn InterestedinBait
  ;[1 1 1] If Player No Longer Fishing Exit State
  (if (not (Variables|Default|GetFishing))
    (CallFunction|SwitchState "NewEnumerator4")
    (return)
    (else
      ;[1 1 1] If Player Has not reached the bobber move towards the bobber
      (if (Variables|Default|GetFishing)
        (CallFunction|MovetoTargetLocation)
        (else
          ;[1 1 1] Small chance for the fish to lose interest in the Bobber
          (CallFunction|SwitchState "NewEnumerator4")))
      (return))))

(fn Return
  (if (<= (Math|Vector|Distance(Vector) (Transformation|GetActorLocation (Variables|Default|GetFishPawn)) (Variables|Default|GetTargetLocation)) (Variables|Default|GetAcceptanceRadius))
    (CallFunction|SwitchState "NewEnumerator0")
    (else
      (CallFunction|MovetoTargetLocation)))
  (return))

(fn TheActOfFishing
  (bind _fishingmngr (Variables|Default|GetFishingMngr))
  (bind _fishpawn (Variables|Default|GetFishPawn))
  (bind _timer (Variables|Default|Gettimer))
  (bind _returnvalue (Transformation|GetActorLocation _fishpawn))
  (bind _returnvalue_2 (Transformation|GetActorLocation _fishingmngr))
  (bind _returnvalue_3 (* _timer 0.2))
  (bind _returnvalue_4 (Class|KismetMathLibrary|PerlinNoise1D _returnvalue_3))
  (bind _returnvalue_5 (- _returnvalue_2 _returnvalue))
  (bind _returnvalue_6 (* _returnvalue_5 "1.000000,1.000000,0.000000"))
  (bind _returnvalue_7 (> _returnvalue_4 0.0))
  (bind _returnvalue_8 (Math|Vector|Normalize _returnvalue_6))
  (bind _returnvalue_9 (Math|Vector|CrossProduct _returnvalue_8 "0.000000,0.000000,1.000000"))
  (bind _returnvalue_10 (Math|Vector|NegateVector _returnvalue_9))
  (bind _returnvalue_11 (Math|Vector|SelectVector _returnvalue_10 _returnvalue_9 _returnvalue_7))
  (if (Variables|Default|GetIsTired)
    (Transformation|SetActorLocation (Variables|Default|GetFishPawn) (Transformation|GetWorldLocation (Variables|/Game/Blueprints/Fishing/BP_FishingPawn.BP_FishingPawn_C|GetFishBiteCollider (Variables|Default|GetFishingMngr))) false false)
    (else
      (CallFunction|HandleMovetoVector _returnvalue_11)
      (Variables|Default|SetAOFDirection _returnvalue_11))))

(fn Flee
  (if (<= (Math|Vector|Distance(Vector) (Transformation|GetActorLocation (Variables|Default|GetFishPawn)) (Variables|Default|GetTargetLocation)) (Variables|Default|GetAcceptanceRadius))
    (CallFunction|SwitchState "NewEnumerator4")
    (else
      (CallFunction|MovetoTargetLocation)))
  (return))

(fn MovetoTargetLocation
  (if (Utilities|Operators|EqualEqual (Transformation|GetActorRotation (Variables|Default|GetFishPawn)) (Math|Rotator|FindLookatRotation (Transformation|GetActorLocation (Variables|Default|GetFishPawn)) (Variables|Default|GetTargetLocation)) 0.1)
    _
    (else
      (CallFunction|HandleRotation)))
  (CallFunction|HandleMovement)
  (return))

(fn FindWanderLocation
  (Variables|Default|SetTargetLocation (+ (Variables|Default|GetSpawnLocation) (* (Math|Random|RandomUnitVector) "1.000000,1.000000,0.000000" (Variables|Default|GetWanderRadius))))
  (return))

(fn HandleMovement
  (Transformation|SetActorLocation (Variables|Default|GetFishPawn) (+ (* (Transformation|GetActorForwardVector (Variables|Default|GetFishPawn)) (* (Variables|Default|Gettimer) (Variables|Default|GetSpeed))) (Transformation|GetActorLocation (Variables|Default|GetFishPawn))) false false)
  (return))

(fn HandleRotation
  (Transformation|SetActorRotation (Variables|Default|GetFishPawn) (Math|Rotator|Lerp(Rotator) (Transformation|GetActorRotation (Variables|Default|GetFishPawn)) (Math|Rotator|FindLookatRotation (Transformation|GetActorLocation (Variables|Default|GetFishPawn)) (Variables|Default|GetTargetLocation)) (* (Variables|Default|Gettimer) (Variables|Default|GetRotationSpeed)) true))
  (return))

(fn HandleMovetoVector
  (params (InputVector :type Vector))
  (bind _speed (Variables|Default|GetSpeed))
  (bind _timer (Variables|Default|Gettimer))
  (bind _fishpawn (Variables|Default|GetFishPawn))
  (bind _returnvalue (Transformation|GetActorLocation _fishpawn))
  (bind _returnvalue_2 (* _timer _speed 9.0))
  (bind _returnvalue_3 (* InputVector _returnvalue_2))
  (bind _returnvalue_4 (+ _returnvalue_3 _returnvalue))
  (Transformation|SetActorLocation (Variables|Default|GetFishPawn) _returnvalue_4 false false)
  (Transformation|SetActorRotation (Variables|Default|GetFishPawn) (Math|Rotator|FindLookatRotation (Transformation|GetActorLocation (Variables|Default|GetFishPawn)) _returnvalue_4)))