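; Blueprint function library of fish economy math, covering sell prices and average price per rarity.
; CalculateFishSellPrice combines size, level and trait factors from the DT_FishMath SellPrice row, then rounds through RoundValue.
; FishRarityAveragePrice prices each DT_FishParameters fish at midpoint weight and length, last-listed spawn depth and time, and fixed quality.
; It groups those prices by rarity and returns a map of their ArrayAverage results.
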(fn RoundValue
  (params (Value%20To%20round :type Float%20%28double-precision%29) (Round%20Points :type Float%20%28double-precision%29))
  (bind _returnvalue (Math|Float|Power 1e+01 Round%20Points))
  (return (* (Math|Float|Round (* Value%20To%20round _returnvalue)) (/ 1.0 (* 1.0 _returnvalue)))))

(fn FishRarityAveragePrice
  (bind _outrownames (DataTable|GetDataTableRowNames "/Game/DataAssets/DT_FishParameters.DT_FishParameters"))
  (for _array_element _outrownames
    (bind _returnvalue (Utilities|GetDataTableRow "/Game/DataAssets/DT_FishParameters.DT_FishParameters" _array_element)
      (:then
        (bind _sellvalue (CallFunction|CalculateFishSellPrice (/ (+ (.MinWeight (Utilities|Struct|BreakF_Fish _returnvalue)) (.MaxWeight (Utilities|Struct|BreakF_Fish _returnvalue))) 2.0) (/ (+ (.MinLength (Utilities|Struct|BreakF_Fish _returnvalue)) (.MaxLength (Utilities|Struct|BreakF_Fish _returnvalue))) 2.0) (.FishingLevel (Utilities|Struct|BreakF_Fish _returnvalue)) (.Rarity (Utilities|Struct|BreakF_Fish _returnvalue)) (Utilities|Array|Get(acopy) (.SpawnableDepths (Utilities|Struct|BreakF_Fish _returnvalue)) (Utilities|Array|LastIndex (.SpawnableDepths (Utilities|Struct|BreakF_Fish _returnvalue)))) (Utilities|Array|Get(acopy) (.SpawnableTimes (Utilities|Struct|BreakF_Fish _returnvalue)) (Utilities|Array|LastIndex (.SpawnableTimes (Utilities|Struct|BreakF_Fish _returnvalue)))) (.Difficulty (Utilities|Struct|BreakF_Fish _returnvalue)) "NewEnumerator1"))
        (switch Utilities|FlowControl|Switch|SwitchonE_FishRarity (.Rarity (Utilities|Struct|BreakF_Fish _returnvalue))
          (:NewEnumerator0
            (Utilities|Array|Add (LocalVariables|GetCommon) _sellvalue))
          (:NewEnumerator1
            (Utilities|Array|Add (LocalVariables|GetUncommon) _sellvalue))
          (:NewEnumerator2
            (Utilities|Array|Add (LocalVariables|GetRare) _sellvalue))
          (:NewEnumerator3
            (Utilities|Array|Add (LocalVariables|GetLegendary) _sellvalue))))))
  (bind _average (CallFunction|ArrayAverage (LocalVariables|GetCommon)))
  (bind _average_2 (CallFunction|ArrayAverage (LocalVariables|GetUncommon)))
  (bind _average_3 (CallFunction|ArrayAverage (LocalVariables|GetRare)))
  (bind _average_4 (CallFunction|ArrayAverage (LocalVariables|GetLegendary)))
  (return (Utilities|Map|MakeMap "NewEnumerator0" _average "NewEnumerator1" _average_2 "NewEnumerator2" _average_3 "NewEnumerator3" _average_4)))

(fn CalculateFishSellPrice
  (params (Weight :type Float%20%28double-precision%29) (Length :type Float%20%28double-precision%29) (FishingLevel :type Integer) (Rarity :type E_FishRarity%20Enum :default "NewEnumerator0") (Depth :type E_FishDepth%20Enum :default "NewEnumerator0") (Time :type E_FishTime%20Enum :default "NewEnumerator0") (Difficulty :type E_FishDifficulty%20Enum :default "NewEnumerator0") (Quality :type E_FishQuality%20Enum :default "NewEnumerator0"))
  (bind _returnvalue (Utilities|GetDataTableRow "/Game/DataAssets/DT_FishMath.DT_FishMath" "SellPrice")
    (:then
      (bind _rounded_value (CallFunction|RoundValue (* (+ Length (/ Weight (.Divisor (Utilities|Struct|BreakF_FishMathValues _returnvalue)))) (.Value (Utilities|Map|Find (.Rarities (Utilities|Struct|BreakF_FishMathValues _returnvalue)) Rarity)) (.Value (Utilities|Map|Find (.Times (Utilities|Struct|BreakF_FishMathValues _returnvalue)) Time)) (.Value (Utilities|Map|Find (.Qualities (Utilities|Struct|BreakF_FishMathValues _returnvalue)) Quality)) (.Multiplier (Utilities|Struct|BreakF_FishMathValues _returnvalue)) (+ (.Value (Utilities|Map|Find (.Depths (Utilities|Struct|BreakF_FishMathValues _returnvalue)) Depth)) (.Value (Utilities|Map|Find (.Difficulties (Utilities|Struct|BreakF_FishMathValues _returnvalue)) Difficulty)) (/ FishingLevel (.Divisor (Utilities|Struct|BreakF_FishMathValues _returnvalue))))) (Math|Conversions|ToFloat(Integer) (.Round (Utilities|Struct|BreakF_FishMathValues _returnvalue)))))
      (return _rounded_value))))

(fn ArrayAverage
  (params (ListOfNums :type Array%20of%20Floats%20%28double-precision%29))
  (for _array_element ListOfNums
    (LocalVariables|SetTotal (+ _array_element (LocalVariables|GetTotal))))
  (return (/ (LocalVariables|GetTotal) (Utilities|Array|Length ListOfNums))))