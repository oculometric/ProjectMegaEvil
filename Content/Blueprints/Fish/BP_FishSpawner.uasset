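; BP_FishSpawner populates the water around itself with BP_FishPawn shoals, using settings from DT_FishSpawning.
; A fast timer fills to the target population, while a rate-based timer tops it up.
; Each attempt traces downward at a random radial offset for depth, then filters DT_FishParameters by area, depth class and day-night segment.
; A rarity-weighted roll picks the species and a random shoal size; KillAllFish broadcasts removal.
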(event Custom|IncreasePopulation
  (bind _returnvalue (Math|Random|RandomFloat))
  (bind _returnvalue_2 (Math|Random|RandomFloat))
  (bind _returnvalue_3 (Transformation|GetActorLocation))
  (bind _minspawndepth (Variables|Default|GetMinSpawnDepth))
  (bind _maxspawnradius (Variables|Default|GetMaxSpawnRadius))
  (bind _returnvalue_4 (* _returnvalue 3.6e+02))
  (bind _returnvalue_5 (- _maxspawnradius _minspawndepth))
  (bind _returnvalue_6 (* _returnvalue_2 _returnvalue_5))
  (bind _returnvalue_7 (+ _returnvalue_6 _minspawndepth))
  (bind _returnvalue_8 (Math|Vector|RotateVectorAroundAxis (Math|Vector|MakeVector _returnvalue_7 0.0 0.0) _returnvalue_4 "0.000000,0.000000,1.000000"))
  (bind _returnvalue_9 (+ _returnvalue_3 _returnvalue_8))
  (bind (_x _y _z) (Math|Vector|BreakVector _returnvalue_9))
  (Utilities|FlowControl|Sequence
    (:then_0
      (bind _cyclesegment (Default|GetCurrentTime (Variables|Default|GetDayNightManager)))
      (bind (_outhit _returnvalue_10) (Collision|LineTraceForObjects (- _returnvalue_9 "0.000000,0.000000,50.000000") (- _returnvalue_9 "0.000000,0.000000,20000.000000") (Utilities|Array|MakeArray "ObjectTypeQuery1") false 0 "None"))
      (if _returnvalue_10
        (bind _fishdepth (Utilities|GetNearbyDepthClasses (.Distance (Collision|BreakHitResult _outhit)))
          (:Row%20Found
            (if (not (< (.Distance (Collision|BreakHitResult _outhit)) (Variables|Default|GetMinSpawnDepth)))
              (CallFunction|SpawnFish (Utilities|Select :Index (/ (Math|Float|%(Float) (+ _returnvalue_4 45.0) 3.6e+02) 9e+01) :Option%200 "NewEnumerator0" :Option%201 "NewEnumerator2" :Option%202 "NewEnumerator1" :Option%203 "NewEnumerator3") _fishdepth _cyclesegment (Math|Vector|MakeVector _x _y (+ (* (* (Math|Random|RandomFloat) (.Distance (Collision|BreakHitResult _outhit))) -1.0) _z))))))))
    (:then_1
      (if (>= (Variables|Default|GetTotalFish) (Variables|Default|GetTargetPopulation))
        (Utilities|Time|ClearandInvalidateTimerbyHandle (Variables|Default|GetSetupSpawnTimer))))))

(event Custom|TrySpawnFish
  (bind _returnvalue (Math|Random|RandomFloat))
  (bind _returnvalue_2 (Math|Random|RandomFloat))
  (bind _returnvalue_3 (Transformation|GetActorLocation))
  (bind _minspawndepth (Variables|Default|GetMinSpawnDepth))
  (bind _maxspawnradius (Variables|Default|GetMaxSpawnRadius))
  (bind _returnvalue_4 (* _returnvalue 3.6e+02))
  (bind _returnvalue_5 (- _maxspawnradius _minspawndepth))
  (bind _returnvalue_6 (* _returnvalue_2 _returnvalue_5))
  (bind _returnvalue_7 (+ _returnvalue_6 _minspawndepth))
  (bind _returnvalue_8 (Math|Vector|RotateVectorAroundAxis (Math|Vector|MakeVector _returnvalue_7 0.0 0.0) _returnvalue_4 "0.000000,0.000000,1.000000"))
  (bind _returnvalue_9 (+ _returnvalue_3 _returnvalue_8))
  (bind (_x _y _z) (Math|Vector|BreakVector _returnvalue_9))
  (if (< (Variables|Default|GetTotalFish) (Variables|Default|GetTargetPopulation))
    (bind _cyclesegment (Default|GetCurrentTime (Variables|Default|GetDayNightManager)))
    (bind (_outhit _returnvalue_10) (Collision|LineTraceForObjects (- _returnvalue_9 "0.000000,0.000000,50.000000") (- _returnvalue_9 "0.000000,0.000000,20000.000000") (Utilities|Array|MakeArray "ObjectTypeQuery1") false 0 "None"))
    (if _returnvalue_10
      (bind _fishdepth (Utilities|GetNearbyDepthClasses (.Distance (Collision|BreakHitResult _outhit)))
        (:Row%20Found
          (if (not (< (.Distance (Collision|BreakHitResult _outhit)) (Variables|Default|GetMinSpawnDepth)))
            (CallFunction|SpawnFish (Utilities|Select :Index (/ (Math|Float|%(Float) (+ _returnvalue_4 45.0) 3.6e+02) 9e+01) :Option%200 "NewEnumerator0" :Option%201 "NewEnumerator2" :Option%202 "NewEnumerator1" :Option%203 "NewEnumerator3") _fishdepth _cyclesegment (Math|Vector|MakeVector _x _y (+ (* (* (Math|Random|RandomFloat) (.Distance (Collision|BreakHitResult _outhit))) -1.0) _z)))))))))

(event Custom|KillAllFish
  (Default|CallKillFish))

(event EventBeginPlay
  (bind _returnvalue (Utilities|GetDataTableRow "/Game/DataAssets/DT_FishSpawning.DT_FishSpawning" "Row")
    (:then
      (Variables|Default|SetMinSpawnDepth (.minspawndepth _returnvalue))
      (Variables|Default|SetMaxSpawnRadius (.maxspawnradius _returnvalue))
      (bind _output_get (Variables|Default|SetSpawnRate (.spawnrate _returnvalue)))
      (Variables|Default|SetTargetPopulation (.targetpopulation _returnvalue))
      (bind _returnvalue_2 (Utilities|Time|SetTimerbyEvent (delegate Custom|IncreasePopulation) 0.01 true true))
      (Variables|Default|SetSetupSpawnTimer _returnvalue_2)
      (bind _returnvalue_3 (Utilities|Time|SetTimerbyEvent (delegate Custom|TrySpawnFish) (/ 1.0 _output_get) true true))
      (Variables|Default|SetSpawnTimer _returnvalue_3)
      (bind _returnvalue_4 (Actor|GetActorOfClass "/Game/Blueprints/Environment/BP_DayNightManager.BP_DayNightManager_C"))
      (Variables|Default|SetDayNightManager _returnvalue_4))))

(fn ConstructionScript)

(fn SpawnFish
  (params (Area :type E_FishArea%20Enum :default "NewEnumerator0") (Depth :type E_FishDepth%20Enum :default "NewEnumerator0") (Time :type E_FishTime%20Enum :default "NewEnumerator0") (Position :type Vector))
  (bind _fishspawnchances (LocalVariables|GetFishSpawnChances))
  (bind _spawnablefishnames (LocalVariables|GetSpawnableFishNames))
  (bind _outrownames (DataTable|GetDataTableRowNames "/Game/DataAssets/DT_FishParameters.DT_FishParameters"))
  (Utilities|Map|Clear (LocalVariables|GetSpawnableFishNames))
  (for _array_element _outrownames
    (bind _returnvalue (Utilities|GetDataTableRow "/Game/DataAssets/DT_FishParameters.DT_FishParameters" _array_element)
      (:then
        (if (Math|Boolean|ANDBoolean (Utilities|Array|ContainsItem (.SpawnableAreas (Utilities|Struct|BreakS_Fish _returnvalue)) Area) (Utilities|Array|ContainsItem (.SpawnableDepths (Utilities|Struct|BreakS_Fish _returnvalue)) Depth) (Utilities|Array|ContainsItem (.SpawnableTimes (Utilities|Struct|BreakS_Fish _returnvalue)) Time))
          (Utilities|Map|Add (LocalVariables|GetSpawnableFishNames) _array_element _returnvalue)))))
  (LocalVariables|SetTotalFishSpawnChance 0.0)
  (Utilities|Map|Clear _fishspawnchances)
  (bind _keys (Utilities|Map|Keys _spawnablefishnames))
  (for _array_element_2 _keys
    (Utilities|Map|Add (LocalVariables|GetFishSpawnChances) _array_element_2 (Utilities|Select :Index (.Rarity (Utilities|Struct|BreakS_Fish (.Value (Utilities|Map|Find _spawnablefishnames _array_element_2)))) :NewEnumerator0 0.55 :NewEnumerator1 0.3 :NewEnumerator2 0.148 :NewEnumerator3 0.02))
    (LocalVariables|SetTotalFishSpawnChance (+ (LocalVariables|GetTotalFishSpawnChance) (Utilities|Select :Index (.Rarity (Utilities|Struct|BreakS_Fish (.Value (Utilities|Map|Find _spawnablefishnames _array_element_2)))) :NewEnumerator0 0.55 :NewEnumerator1 0.3 :NewEnumerator2 0.148 :NewEnumerator3 0.02))))
  (bind _keys_2 (Utilities|Map|Keys _fishspawnchances))
  (LocalVariables|SetTrackedFishSpawnChance (* (Math|Random|RandomFloat) (LocalVariables|GetTotalFishSpawnChance)))
  (bind _array_element_3 (Utilities|Array|ForEachLoopwithBreak _keys_2 :!label _label)
    (:LoopBody
      (bind _output_get (LocalVariables|SetTrackedFishSpawnChance (- (LocalVariables|GetTrackedFishSpawnChance) (.Value (Utilities|Map|Find (LocalVariables|GetFishSpawnChances) _array_element_3)))))
      (if (<= _output_get 0.0)
        (LocalVariables|SetFishToSpawn _array_element_3)
        (goto _label Break)))
    (:Completed
      (for _index (range 0 (Math|Random|RandomInteger (.MaxShoalSize (Utilities|Struct|BreakS_Fish (.Value (Utilities|Map|Find (LocalVariables|GetSpawnableFishNames) (LocalVariables|GetFishToSpawn)))))))
        (Game|SpawnActorfromClass "/Game/Blueprints/Fish/BP_FishPawn.BP_FishPawn_C" (Math|Transform|MakeTransform Position (Math|Rotator|MakeRotator 0.0 0.0 (* (Math|Random|RandomFloat) 3.6e+02)) "1.000000,1.000000,1.000000") "Undefined" "MultiplyWithRoot" 0 self (.Value (Utilities|Map|Find (LocalVariables|GetSpawnableFishNames) (LocalVariables|GetFishToSpawn))) 0)
        (Math|Integer|IncrementInt (Variables|Default|GetTotalFish))))))