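; Fish AI component that drives its owning pawn through an enum state machine on Tick: wander, bait interest, return, catch minigame and flee.
; While fishing, random rolls lure fish to the Fisher's bobber, then decide between biting and returning to spawn.
; SwitchState picks each target, and movement lerps rotation toward it while directly setting location forward without sweep.
; MiniGame is an empty stub, and nothing here triggers Flee.
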(event EventBeginPlay
  (bind _output_get (Variables|Default|SetFishPawn (.AsPawn (Utilities|Casting|CastToPawn (Components|GetOwner)))))
  (Variables|Default|SetSpawnLocation (Transformation|GetActorLocation _output_get))
  (CallFunction|SwitchState "NewEnumerator0"))

(event EventTick
  (params (DeltaSeconds :type Float%20%28single-precision%29))
  (CallFunction|FSMLogic))

(fn FSMLogic
  (switch Utilities|FlowControl|Switch|SwitchonE_FishFSM (Variables|Default|GetFishFSM)
    (:NewEnumerator0
      (if (not (Variables|Default|GetFishing))
        (CallFunction|WandertoLocation :!label _label)
        (elif (>= (Math|Random|RandomFloat) (Variables|Default|GetLureChance))
          (goto _label)
          (else
            (CallFunction|SwitchState "NewEnumerator1")))))
    (:NewEnumerator1
      (if (Variables|Default|GetBIte)
        (CallFunction|SwitchState "NewEnumerator2")
        (else
          (CallFunction|InterestedinBait))))
    (:NewEnumerator4
      (CallFunction|Return))
    (:NewEnumerator2
      (CallFunction|MiniGame))
    (:NewEnumerator3
      (CallFunction|Flee)))
  (return))

(fn FindWanderLocation
  (bind _spawnlocation (Variables|Default|GetSpawnLocation))
  (bind _spawnlocation_2 (Variables|Default|GetSpawnLocation))
  (bind _spawnlocation_3 (Variables|Default|GetSpawnLocation))
  (bind _wanderradius (Variables|Default|GetWanderRadius))
  (bind _wanderheightradius (Variables|Default|GetWanderHeightRadius))
  (bind _wanderradius_2 (Variables|Default|GetWanderRadius))
  (Variables|Default|SetTargetLocation (Math|Vector|MakeVector (Math|Random|RandomFloatinRange (- _wanderradius_2 (.x _spawnlocation)) (+ _wanderradius_2 (.x _spawnlocation))) (Math|Random|RandomFloatinRange (- _wanderradius (.y _spawnlocation_3)) (+ _wanderradius (.y _spawnlocation_3))) (Math|Random|RandomFloatinRange (- _wanderheightradius (.z _spawnlocation_2)) (+ _wanderheightradius (.z _spawnlocation_2)))))
  (return))

(fn MovetoTargetLocation
  (if (Utilities|Operators|EqualEqual (Transformation|GetActorRotation (Variables|Default|GetFishPawn)) (Math|Rotator|FindLookatRotation (Transformation|GetActorLocation (Variables|Default|GetFishPawn)) (Variables|Default|GetTargetLocation)) 0.1)
    _
    (else
      (CallFunction|HandleRotation)))
  (CallFunction|HandleMovement)
  (return))

(fn Flee
  (if (<= (Math|Vector|Distance(Vector) (Transformation|GetActorLocation (Variables|Default|GetFishPawn)) (Variables|Default|GetTargetLocation)) (Variables|Default|GetAcceptanceRadius))
    (CallFunction|SwitchState "NewEnumerator0")
    (else
      (CallFunction|MovetoTargetLocation)))
  (return))

(fn MiniGame)

(fn Return
  (if (<= (Math|Vector|Distance(Vector) (Transformation|GetActorLocation (Variables|Default|GetFishPawn)) (Variables|Default|GetTargetLocation)) (Variables|Default|GetAcceptanceRadius))
    (CallFunction|SwitchState "NewEnumerator0")
    (else
      (CallFunction|MovetoTargetLocation)))
  (return))

(fn WandertoLocation
  (if (<= (Math|Vector|Distance(Vector) (Transformation|GetActorLocation (Variables|Default|GetFishPawn)) (Variables|Default|GetTargetLocation)) (Variables|Default|GetAcceptanceRadius))
    (CallFunction|FindWanderLocation))
  (CallFunction|MovetoTargetLocation)
  (return))

(fn InterestedinBait
  (if (not (Variables|Default|GetFishing))
    (CallFunction|SwitchState "NewEnumerator4")
    (return)
    (elif (<= (Math|Vector|Distance(Vector) (Variables|Default|GetTargetLocation) (Transformation|GetActorLocation (Variables|Default|GetFishPawn))) (Variables|Default|GetAcceptanceRadius))
      (if (and (Variables|Default|GetFishing) (>= (Math|Random|RandomFloat) 0.5))
        (CallFunction|SwitchState "NewEnumerator2")
        (Variables|Default|SetBIte true)
        (else
          (CallFunction|SwitchState "NewEnumerator4")))
      (return)
      (else
        (CallFunction|MovetoTargetLocation)
        (return)))))

(fn SwitchState
  (params (New%20State :type E_FishFSM%20Enum :default "NewEnumerator0"))
  (bind _fisher (Variables|Default|GetFisher))
  (bind _output_get (Variables|Default|SetFishFSM New%20State))
  (switch Utilities|FlowControl|Switch|SwitchonE_FishFSM _output_get
    (:NewEnumerator0
      (CallFunction|FindWanderLocation))
    (:NewEnumerator1
      (Variables|Default|SetTargetLocation (Transformation|GetWorldLocation (Components|GetChildComponent (Variables|/Game/Blueprints/FishingTest/BP_FisherTest.BP_FisherTest_C|GetBobber (Variables|Default|GetFisher)) 0))))
    (:NewEnumerator4
      (Variables|Default|SetTargetLocation (Variables|Default|GetSpawnLocation)))
    (:NewEnumerator3
      (Variables|Default|SetSpeed (* (Variables|Default|GetSpeed) 1e+01))
      (Variables|Default|SetTargetLocation (+ (Transformation|GetActorLocation _fisher) (* (Transformation|GetActorForwardVector _fisher) 1e+03)))))
  (return))

(fn HandleMovement
  (Transformation|SetActorLocation (Variables|Default|GetFishPawn) (+ (* (Transformation|GetActorForwardVector (Variables|Default|GetFishPawn)) (* (Utilities|Time|GetWorldDeltaSeconds) (Variables|Default|GetSpeed))) (Transformation|GetActorLocation (Variables|Default|GetFishPawn))) false false)
  (return))

(fn HandleRotation
  (Transformation|SetActorRotation (Variables|Default|GetFishPawn) (Math|Rotator|Lerp(Rotator) (Transformation|GetActorRotation (Variables|Default|GetFishPawn)) (Math|Rotator|FindLookatRotation (Transformation|GetActorLocation (Variables|Default|GetFishPawn)) (Variables|Default|GetTargetLocation)) (* (Utilities|Time|GetWorldDeltaSeconds) (Variables|Default|GetRotationSpeed)) true))
  (return))