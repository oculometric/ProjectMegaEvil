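; Player-driven boat pawn with steering, free-look and zoom camera, bobbing animation, and switching to a spawned fisher pawn outside no-fishing zones.
; Components handle health, attributes, mesh loading, weathering and movement, cross-linked on BeginPlay, which also attaches a fish spawner.
; Timelines drive bobbing, engine volume, zoom and timed camera return.
; Damage feeds health and effects; death shows a fade sequence, respawns the boat and resets the weekly quota.
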(event Custom|SetNoFishingZone
  (params (NoFIsh :type Boolean))
  (bind _output_get (Variables|Default|SetIn%20No%20Fishing%20Zone NoFIsh))
  (Development|PrintString (Utilities|String|SelectString "In No Fishing Zone!" "Leaving No Fishing Zone." _output_get))
  (if _output_get
    _))

(event Custom|Death
  (bind _playercontroller (Variables|Default|GetPlayerController))
  (bind _boathud (Variables|/Game/Blueprints/BP_FishingPlayerController.BP_FishingPlayerController_C|GetBoatHUD _playercontroller))
  ;[0.3281 0 0] Death Event
  (Utilities|FlowControl|DoOnce false :!label _label
    (:Completed
      (Default|ToggleControlsEnabled _playercontroller false)
      (Default|SetHUDVisibility _boathud false)
      (bind _returnvalue (UserInterface|CreateWidget "/Game/UI/MenuPrototypes/WBP_DeathScreen.WBP_DeathScreen_C"))
      (Class|UserWidget|PlayAnimationForward _returnvalue (Variables|/Game/UI/MenuPrototypes/WBP_DeathScreen.WBP_DeathScreen_C|GetFadeIn _returnvalue) 1.0 false)
      (UserInterface|Viewport|AddtoViewport _returnvalue 0)
      (Utilities|FlowControl|Delay 8.0)
      (bind _returnvalue_2 (UserInterface|CreateWidget "/Game/UI/MenuPrototypes/WBP_SimpleFade.WBP_SimpleFade_C"))
      (UserInterface|Viewport|AddtoViewport _returnvalue_2 0)
      (Default|FadetoBlack _returnvalue_2 0.75)
      (Utilities|FlowControl|Delay 1.0)
      (Widget|RemovefromParent _returnvalue)
      (CallFunction|Reset)
      (Default|FadefromBlack _returnvalue_2 1.0)
      (Utilities|FlowControl|Delay 0.75)
      (bind _returnvalue_3 (Actor|GetActorOfClass "/Game/Blueprints/BP_WeeklyQuotaManager.BP_WeeklyQuotaManager_C"))
      (Default|ResetWeek _returnvalue_3)
      (Default|SetHUDVisibility _boathud true)
      (Utilities|FlowControl|Delay 0.25)
      (Widget|RemovefromParent _returnvalue_2)
      (Default|ToggleControlsEnabled _playercontroller true)
      (goto _label Reset))))

(event Custom|Reset
  (Default|ResetPlayerHealth (Variables|Default|GetBPC_BoatHealth))
  (bind _returnvalue (Actor|GetActorOfClass "/Game/Blueprints/BP_BoatGameMode.BP_BoatGameMode_C"))
  (Transformation|SetActorLocation (Transformation|GetActorLocation (Class|GameModeBase|FindPlayerStart _returnvalue (Variables|Default|GetPlayerController))) false true)
  (Transformation|SetActorRotation "0, 0, 0" true))

(event Custom|ReturnCamera
  ;[1 1 1] Free Looking
  (bind _alpha (Timeline|CamReturnTimeline Play)
    (:Update
      (Transformation|SetRelativeRotation (Variables|Components|GetSpringArm) (Math|Rotator|Lerp(Rotator) (stale Input|EnhancedActionEvents|EnhancedInputActionIA_BoatLook _output_get) "-16.000000,0.000000,0.000000" _alpha) false false))))

(event Input|EnhancedActionEvents|EnhancedInputActionIA_BoatTurn
  (params (ActionValue :type Float%20%28double-precision%29) (ElapsedSeconds :type Float%20%28double-precision%29) (TriggeredSeconds :type Float%20%28double-precision%29) (InputAction :type Input%20Action%20Object%20Reference :default "/Game/Input/Boat/IA_BoatTurn.IA_BoatTurn"))
  ;[1 1 1] Left/Right Turning
  (if (Variables|Default|GetControlsEnabled)
    (Pawn|Input|AddControllerYawInput (* ActionValue (Variables|Default|GetSteeringMultiplier) (Utilities|Time|GetWorldDeltaSeconds) (Math|Float|SelectFloat -1.0 1.0 (Variables|Default|GetReversing))))))

(event Input|EnhancedActionEvents|EnhancedInputActionIA_BoatLook
  (params (ActionValue :type Vector%202D%20Structure) (ElapsedSeconds :type Float%20%28double-precision%29) (TriggeredSeconds :type Float%20%28double-precision%29) (InputAction :type Input%20Action%20Object%20Reference :default "/Game/Input/Boat/IA_BoatLook.IA_BoatLook"))
  (bind _springarm (Variables|Components|GetSpringArm))
  (bind _camspeedmultiplier (Variables|Default|GetCamSpeedMultiplier))
  (bind _relativerotation (Variables|/Script/Engine.SceneComponent|GetRelativeRotation _springarm))
  ;[1 1 1] Free Looking
  (Utilities|Time|ClearandInvalidateTimerbyHandle (Variables|Default|GetFreeLookReturnTimer))
  (Transformation|SetRelativeRotation _springarm (Math|Rotator|MakeRotator 0.0 (Math|Float|Clamp(Float) (+ (.pitch _relativerotation) (* (.y ActionValue) _camspeedmultiplier)) -45.0 45.0) (+ (.yaw _relativerotation) (* (.x ActionValue) _camspeedmultiplier) 0.0)) false false)
  (bind _output_get (Variables|Default|SetCamRotAfterLook (Variables|/Script/Engine.SceneComponent|GetRelativeRotation (Variables|Components|GetSpringArm))))
  (bind _returnvalue (Utilities|Time|SetTimerbyEvent (delegate Custom|ReturnCamera) (Variables|Default|GetCameraReturnTime)))
  (Variables|Default|SetFreeLookReturnTimer _returnvalue))

(event Input|EnhancedActionEvents|EnhancedInputActionIA_SwitchPerspective
  (params (ActionValue :type Boolean) (ElapsedSeconds :type Float%20%28double-precision%29) (TriggeredSeconds :type Float%20%28double-precision%29) (InputAction :type Input%20Action%20Object%20Reference :default "/Game/Input/IA_SwitchPerspective.IA_SwitchPerspective"))
  (bind _playercontroller (Variables|Default|GetPlayerController))
  (bind _playercontroller_2 (Variables|Default|GetPlayerController))
  (bind _fisher (Variables|Default|GetFisher))
  (bind _playercontroller_3 (Variables|Default|GetPlayerController))
  (bind _controlsenabled (Variables|Default|GetControlsEnabled))
  (bind _returnvalue (PlayerController|LocalPlayerSubsystems|GetEnhancedInputLocalPlayerSubsystem _playercontroller_2))
  (bind _boathud (Variables|/Game/Blueprints/BP_FishingPlayerController.BP_FishingPlayerController_C|GetBoatHUD _playercontroller))
  (bind _boathud_2 (Variables|/Game/Blueprints/BP_FishingPlayerController.BP_FishingPlayerController_C|GetBoatHUD _playercontroller_3))
  (bind _wbp_baitcounter (Variables|/Game/UI/BoatHUD/WBP_BoatHUD.WBP_BoatHUD_C|GetWBP_BaitCounter _boathud))
  (bind _wbp_baitcounter_2 (Variables|/Game/UI/BoatHUD/WBP_BoatHUD.WBP_BoatHUD_C|GetWBP_BaitCounter _boathud_2))
  ;[1 1 1] Change to Fisher Perspective
  (:Started
    (if _controlsenabled
      (Default|ButtonPressed _wbp_baitcounter_2)))
  (:Completed
    (if _controlsenabled
      (Default|ButtonReleased _wbp_baitcounter_2)
      (if (not (Variables|Default|GetIn%20No%20Fishing%20Zone))
        (Game|Player|SetViewTargetwithBlend _playercontroller_2 _fisher 0.5 "VTBlend_EaseInOut" 2.0 false)
        (Default|MakeVisible (Variables|/Game/Blueprints/Fishing/BP_FishingPawn.BP_FishingPawn_C|GetCastMeter _fisher))
        (Utilities|FlowControl|Delay 0.5)
        (Pawn|Possess _playercontroller_2 _fisher)
        (Utilities|IsValid _returnvalue
          (:Is%20Valid
            (Input|RemoveMappingContext _returnvalue "/Game/Input/Boat/IMC_Boat.IMC_Boat" "(bIgnoreAllPressedKeysUntilRelease=True,bForceImmediately=False,bNotifyUserSettings=False)")
            (Input|AddMappingContext _returnvalue "/Game/Input/Fishing/IMC_Fishing.IMC_Fishing" 0 "(bIgnoreAllPressedKeysUntilRelease=True,bForceImmediately=False,bNotifyUserSettings=False)")
            (Default|CollapsePrompt _wbp_baitcounter)
            (Default|DisplayPrompt _wbp_baitcounter "Drive" "E")))))))

(event Input|EnhancedActionEvents|EnhancedInputActionIA_BoatZoom
  (params (ActionValue :type Float%20%28double-precision%29) (ElapsedSeconds :type Float%20%28double-precision%29) (TriggeredSeconds :type Float%20%28double-precision%29) (InputAction :type Input%20Action%20Object%20Reference :default "/Game/Input/Boat/IA_BoatZoom.IA_BoatZoom"))
  ;[1 1 1] Camera Zoom
  (if (Variables|Default|GetControlsEnabled)
    (if (not (Variables|Default|GetZoomInProgress?))
      (Variables|Default|SetZoomInProgress? true)
      (bind _alpha (Timeline|Zoom PlayFromStart)
        (:Update
          (Variables|/Script/Engine.SpringArmComponent|SetTargetArmLength (Variables|Components|GetSpringArm) (Math|Float|Lerp (Variables|/Script/Engine.SpringArmComponent|GetTargetArmLength (Variables|Components|GetSpringArm)) (Math|Float|Clamp(Float) (- (Variables|/Script/Engine.SpringArmComponent|GetTargetArmLength (Variables|Components|GetSpringArm)) (* ActionValue (Variables|Default|GetZoomMultiplier))) (Variables|Default|GetMinCamLength) (Variables|Default|GetMaxCamLength)) _alpha)))
        (:Finished
          (Variables|Default|SetZoomInProgress? false))))))

(event Input|EnhancedActionEvents|EnhancedInputActionIA_BoatMove
  (params (ActionValue :type Float%20%28double-precision%29) (ElapsedSeconds :type Float%20%28double-precision%29) (TriggeredSeconds :type Float%20%28double-precision%29) (InputAction :type Input%20Action%20Object%20Reference :default "/Game/Input/Boat/IA_BoatMove.IA_BoatMove"))
  (bind _controlsenabled (Variables|Default|GetControlsEnabled))
  ;[1 1 1] Forward/Backward Movement
  (:Triggered
    (if _controlsenabled
      (Pawn|Input|AddMovementInput (Math|Vector|RotateVector (Math|Vector|MakeVector ActionValue 0.0 0.0) (Transformation|GetActorRotation)) (* (Variables|Default|GetMovementMultiplier) (Utilities|Time|GetWorldDeltaSeconds) (Variables|Default|GetMovement%20Debuff)) false)
      (Variables|Default|SetReversing (< ActionValue 0.0))
      (Variables|Default|SetisMoving true)
      (Utilities|FlowControl|DoOnce false :!label _label
        (:Completed
          (bind _scale (Timeline|BoatMoveSound Play)
            (:Update
              (Audio|Components|Audio|SetVolumeMultiplier (Variables|Default|GetBoatMoveSounds) (Math|Float|Lerp 0.2 1.0 _scale) :!class /Script/Engine.AudioComponent)))))))
  (:Completed
    (if _controlsenabled
      (Variables|Default|SetReversing false)
      (Variables|Default|SetisMoving false)
      (Utilities|FlowControl|Sequence
        (:then_0
          (Timeline|BoatMoveSound Reverse))
        (:then_1
          (goto _label Reset))))))

(event EventBeginPlay
  (bind _self self)
  (bind _self_2 self)
  (bind _bpc_boathealth (Variables|Default|GetBPC_BoatHealth))
  (bind _bpc_boatattributes (Variables|Default|GetBPC_BoatAttributes))
  (bind _fisherattachpoint (Variables|Components|GetFisherAttachPoint))
  (bind _boatattach (Variables|Default|GetBoatAttach))
  (Default|ResetPlayerHealth (Variables|Default|GetBPC_BoatHealth))
  (Default|LoadMesh (Variables|Components|GetBPC_BoatMeshManager) 0 0 0 (Variables|Default|GetBoatAttach))
  (Utilities|FlowControl|Sequence
    (:then_0
      ;[0 1 1] Spawn Fisher
      (bind _returnvalue (Game|SpawnActorfromClass "/Game/Blueprints/Fishing/BP_FishingPawn.BP_FishingPawn_C" (Transformation|GetWorldTransform _fisherattachpoint) "AlwaysSpawn" "MultiplyWithRoot" 0 0))
      (bind _output_get (Variables|Default|SetFisher _returnvalue))
      (Transformation|AttachComponentToComponent _output_get _fisherattachpoint "None" "SnapToTarget" "SnapToTarget" "SnapToTarget" true)
      (Variables|/Game/Blueprints/Fishing/BP_FishingPawn.BP_FishingPawn_C|SetBoat _output_get self)
      ;[1 1 1] Setting component references
      (Variables|/Game/Blueprints/Boats/BPC_BoatWeatheringComponent.BPC_BoatWeatheringComponent_C|SetBoat (Variables|Default|GetBPC_BoatWeatheringComponent) self)
      (Variables|/Game/Blueprints/Boats/BPC_BoatHealth.BPC_BoatHealth_C|SetBoatAttributes _bpc_boathealth _bpc_boatattributes)
      (Variables|/Game/Blueprints/Boats/BPC_BoatAttributes.BPC_BoatAttributes_C|SetBoatLoader _bpc_boatattributes (Variables|Components|GetBPC_BoatMeshManager))
      (Variables|/Game/Blueprints/Boats/BPC_BoatAttributes.BPC_BoatAttributes_C|SetBoat _bpc_boatattributes _self_2)
      (Variables|/Game/Blueprints/Boats/BPC_BoatHealth.BPC_BoatHealth_C|SetBoat _bpc_boathealth _self_2))
    (:then_1
      ;[0 0 1] Fish Spawning
      (bind _returnvalue_2 (Actor|GetActorOfClass "/Game/Blueprints/BP_FishSpawner.BP_FishSpawner_C"))
      (Utilities|IsValid _returnvalue_2
        (:Is%20Valid
          (Transformation|AttachActorToActor _returnvalue_2 _self "None" "SnapToTarget" "SnapToTarget" "SnapToTarget" false))
        (:Is%20Not%20Valid
          (bind _returnvalue_3 (Game|SpawnActorfromClass "/Game/Blueprints/BP_FishSpawner.BP_FishSpawner_C" (Transformation|GetActorTransform) "AlwaysSpawn" "MultiplyWithRoot" 0 0))
          (Transformation|AttachActorToActor _returnvalue_3 _self "None" "SnapToTarget" "SnapToTarget" "SnapToTarget" false))))
    (:then_2
      ;[0 0 0] Set Player Controller
      (bind _asbp_fishing_player_controller (Utilities|Casting|CastToBP_FishingPlayerController (Game|GetPlayerController 0)))
      (Variables|Default|SetPlayerController _asbp_fishing_player_controller)
      (Default|Initialise (Variables|Default|GetBPC_BoatMovement) _self))
    (:then_3
      (bind _updown (Timeline|Timeline PlayFromStart)
        (:Update
          (Transformation|SetRelativeLocation _boatattach (Math|Vector|MakeVector 0.0 0.0 (- (* _updown -3e+01) -5.0)) false false)
          (Transformation|SetRelativeRotation _boatattach (Math|Interpolation|Ease "EaseIn" (* (Utilities|Time|GetWorldDeltaSeconds) 3.0) (Variables|/Script/Engine.SceneComponent|GetRelativeRotation _boatattach) (Variables|Default|GetTargetAngles) true) false false))
        (:Finished
          (Timeline|Timeline PlayFromStart))
        (:SetTargetRotation
          (Variables|Default|SetTargetAngles (Class|KismetMathLibrary|MakeRotfromYZ (Class|KismetMathLibrary|VectorRight) (Math|Random|RandomUnitVectorinConeinDegrees "0.000000,0.000000,1.000000" 15.0))))))))

(event Game|Damage|EventAnyDamage
  (params (Damage :type Float%20%28single-precision%29) (DamageType :type Damage%20Type%20Object%20Reference) (InstigatedBy :type Controller%20Object%20Reference) (DamageCauser :type Actor%20Object%20Reference))
  ;[1 0 0] Damage
  (Default|HealthChanged (Variables|Default|GetBPC_BoatHealth) Damage)
  (if (> Damage 1e+01)
    (Niagara|SpawnSystematLocation "/Game/VFX/NS_Damage.NS_Damage" (Transformation|GetActorLocation))
    (Default|ShowDamageEffect (Variables|/Game/Blueprints/BP_FishingPlayerController.BP_FishingPlayerController_C|GetBoatHUD (Variables|Default|GetPlayerController)))))

(fn ConstructionScript)