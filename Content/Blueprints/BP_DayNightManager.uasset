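; Day/night cycle manager that advances game time, animates sky and sun, and tells the weekly quota manager when a cycle ends.
; DT_DayNightCycle supplies day and night lengths plus sun colour and power keyframes.
; Tick accumulates time, mapped to a 0–2 fraction so day and night can differ in length.
; Sky updates drive a dynamic material and sun rotation, blend keyframes through Lerp5, and broadcast the current time.
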(event Custom|UpdateSkyShader
  (bind _time (Utilities|GetCycleTime))
  (bind _nightlengthseconds (Variables|Default|GetNightLengthSeconds))
  (bind _suncolourdawn (Variables|Default|GetSunColourDawn))
  (bind _sunpowerdawn (Variables|Default|GetSunPowerDawn))
  (bind _sunlight (Variables|Default|GetSunLight))
  (bind _daylengthseconds (Variables|Default|GetDayLengthSeconds))
  (bind _returnvalue (Math|Conversions|ToVector(Float) _sunpowerdawn))
  (bind _returnvalue_2 (<= _time _daylengthseconds))
  (bind _returnvalue_3 (/ _time _daylengthseconds))
  (bind _returnvalue_4 (- _time _daylengthseconds))
  (bind _lightcomponent (Variables|/Script/Engine.Light|GetLightComponent _sunlight))
  (bind _returnvalue_5 (/ _returnvalue_4 _nightlengthseconds))
  (bind _returnvalue_6 (+ _returnvalue_5 1.0))
  (bind _returnvalue_7 (Math|Float|SelectFloat _returnvalue_3 _returnvalue_6 _returnvalue_2))
  (bind _returnvalue_8 (Math|Float|%(Float) _returnvalue_7 2.0))
  (bind _returnvalue_9 (/ _returnvalue_8 2.0))
  ;[1 1 1] Update the sky shader and lighting based on the time of day
  (Rendering|Material|SetScalarParameterValue (Variables|Default|GetSkyMaterial) "TimeFactor" _returnvalue_8 :!class /Script/Engine.MaterialInstanceDynamic)
  (Transformation|SetActorRotation _sunlight (Math|Conversions|RotationFromXVector (Math|Vector|RotateVector "0.000000,0.300000,-0.900000" (Math|Rotator|MakeRotator 0.0 (* (- (* _returnvalue_8 2.0) 1.0) -9e+01) 0.0))))
  (Rendering|Components|Light|SetLightColor _lightcomponent (Math|Conversions|ToLinearColor(Vector) (Utilities|Lerp5 _suncolourdawn (Variables|Default|GetSunColourMidday) (Variables|Default|GetSunColourDusk) (Variables|Default|GetSunColourMidnight) _suncolourdawn _returnvalue_9)) true)
  (Rendering|Components|Light|SetIntensity _lightcomponent (.x (Utilities|Lerp5 _returnvalue (Math|Conversions|ToVector(Float) (Variables|Default|GetSunPowerMidday)) (Math|Conversions|ToVector(Float) (Variables|Default|GetSunPowerDusk)) (Math|Conversions|ToVector(Float) (Variables|Default|GetSunPowerMidnight)) _returnvalue _returnvalue_9)))
  (bind (_elapsedtime _cyclesegment _fraction) (CallFunction|GetCurrentTime))
  (Default|CallDayTimeUpdated _elapsedtime _fraction _cyclesegment))

(event Custom|ReadDataTable
  ;[1 1 1] read day-cycle config
  (bind _returnvalue (Utilities|GetDataTableRow "/Game/DataAssets/DT_DayNightCycle.DT_DayNightCycle" (Variables|Default|GetDay))
    (:then
      (Utilities|FlowControl|Sequence
        (:then_0
          (Variables|Default|SetDayLengthSeconds (* (.cyclelengthseconds _returnvalue) (.dayfraction _returnvalue)))
          (Variables|Default|SetNightLengthSeconds (- (.cyclelengthseconds _returnvalue) (* (.cyclelengthseconds _returnvalue) (.dayfraction _returnvalue)))))
        (:then_1
          (Variables|Default|SetSunColourDawn (.suncolourdawn _returnvalue))
          (Variables|Default|SetSunPowerDawn (.sunpowerdawn _returnvalue)))
        (:then_2
          (Variables|Default|SetSunColourMidday (.suncolourmidday _returnvalue))
          (Variables|Default|SetSunPowerMidday (.sunpowermidday _returnvalue)))
        (:then_3
          (Variables|Default|SetSunColourDusk (.suncolourdusk _returnvalue))
          (Variables|Default|SetSunPowerDusk (.sunpowerdusk _returnvalue)))
        (:then_4
          (Variables|Default|SetSunColourMidnight (.suncolourmidnight _returnvalue))
          (Variables|Default|SetSunPowerMidnight (.sunpowermidnight _returnvalue)))))
    (:RowNotFound
      (Development|PrintString "data table row not found!!"))))

(event Custom|DayCycleFinish
  (bind _returnvalue (Actor|GetActorOfClass "/Game/Blueprints/BP_WeeklyQuotaManager.BP_WeeklyQuotaManager_C"))
  (Utilities|IsValid _returnvalue
    (:Is%20Valid
      (Default|NextDay _returnvalue false))))

(event Custom|SkipDay
  (CallFunction|SetDayFraction 0.1))

(event Custom|SetDayFraction
  (params (Fraction :type Float%20%28double-precision%29))
  (bind _returnvalue (Math|Float|%(Float) Fraction 2.0))
  (Variables|Default|SetDayTimer (+ (* (Math|Float|Clamp(Float) _returnvalue) (Variables|Default|GetDayLengthSeconds)) (* (Variables|Default|GetNightLengthSeconds) (Math|Float|Clamp(Float) (- _returnvalue 1.0))))))

(event EventBeginPlay
  (CallFunction|Initialise)
  (Utilities|Time|SetTimerbyEvent (EventDispatchers|CreateEvent :!event Custom|UpdateSkyShader) 0.1 true true)
  (CallFunction|SetDayFraction 0.1))

(event EventTick
  (params (DeltaSeconds :type Float%20%28single-precision%29))
  (bind _daylengthseconds (Variables|Default|GetDayLengthSeconds))
  (bind _nightlengthseconds (Variables|Default|GetNightLengthSeconds))
  (bind _returnvalue (+ _daylengthseconds _nightlengthseconds))
  (bind _output_get (Variables|Default|SetDayTimer (+ DeltaSeconds (Variables|Default|GetDayTimer))))
  (if (>= _output_get _returnvalue)
    (Variables|Default|SetDayTimer (- _output_get _returnvalue))
    (CallFunction|DayCycleFinish)))

(fn ConstructionScript
  (CallFunction|Initialise))

(fn GetCurrentTime
  (bind _time (Utilities|GetCycleTime))
  (bind _time_2 (Utilities|GetCycleTime))
  (bind _daylengthseconds (Variables|Default|GetDayLengthSeconds))
  (return _time (select (> _time (Variables|Default|GetDayLengthSeconds)) "NewEnumerator1" "NewEnumerator0") (Math|Float|%(Float) (Math|Float|SelectFloat (/ _time_2 _daylengthseconds) (+ (/ (- _time_2 _daylengthseconds) (Variables|Default|GetNightLengthSeconds)) 1.0) (<= _time_2 _daylengthseconds)) 2.0)))

(fn Initialise
  (CallFunction|ReadDataTable)
  (bind _returnvalue (Rendering|Material|CreateDynamicMaterialInstance "/Game/Materials/M_SimpleSky.M_SimpleSky" "None" "None" :!class /Script/Engine.KismetMaterialLibrary))
  (bind _output_get (Variables|Default|SetSkyMaterial _returnvalue))
  (Rendering|Material|SetMaterial (Actor|GetComponentbyClass (Variables|Default|GetSkySphere) "/Script/Engine.StaticMeshComponent") 0 _output_get))