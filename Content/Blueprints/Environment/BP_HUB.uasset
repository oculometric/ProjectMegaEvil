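; BP_HUB is the harbour hub actor, with a no-fishing zone and a pier interaction for ending the day.
; When enabled, NoFishZone overlaps toggle the boat's no-fishing state and swap the HUD's Fish prompt.
; InteractBox overlaps set the player controller's CanInteract and show or clear the End Day prompt.
; Tick rotates Spinner and scales it from DayNightManager's time, so it appears only around one time of day.
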(event OnComponentBeginOverlap(NoFishZone)
  (params (OverlappedComponent :type Primitive%20Component%20Object%20Reference) (OtherActor :type Actor%20Object%20Reference) (OtherComp :type Primitive%20Component%20Object%20Reference) (OtherBodyIndex :type Integer) (bFromSweep :type Boolean) (SweepResult :type Hit%20Result%20Structure%20%28by%20ref%29))
  (bind _player_controller (Variables|Default|GetPlayer%20Controller))
  (bind _boathud (Variables|/Game/Blueprints/BP_FishingPlayerController.BP_FishingPlayerController_C|GetBoatHUD _player_controller))
  (bind _wbp_baitcounter (Variables|/Game/UI/BoatHUD/WBP_BoatHUD.WBP_BoatHUD_C|GetWBP_BaitCounter _boathud))
  ;[1 1 1] NoFishingZone
  (if (Variables|Default|GetEnabled)
    (bind _asbp_boat_pawn (Utilities|Casting|CastToBP_BoatPawn OtherActor))
    (Default|SetNoFishingZone _asbp_boat_pawn true)
    (Utilities|FlowControl|Delay 0.2)
    (Default|CollapsePrompt _wbp_baitcounter)
    (Default|DisplayPrompt _wbp_baitcounter)))

(event OnComponentEndOverlap(NoFishZone)
  (params (OverlappedComponent :type Primitive%20Component%20Object%20Reference) (OtherActor :type Actor%20Object%20Reference) (OtherComp :type Primitive%20Component%20Object%20Reference) (OtherBodyIndex :type Integer))
  (bind _player_controller (Variables|Default|GetPlayer%20Controller))
  (bind _boathud (Variables|/Game/Blueprints/BP_FishingPlayerController.BP_FishingPlayerController_C|GetBoatHUD _player_controller))
  (bind _wbp_baitcounter (Variables|/Game/UI/BoatHUD/WBP_BoatHUD.WBP_BoatHUD_C|GetWBP_BaitCounter _boathud))
  ;[1 1 1] NoFishingZone
  (if (Variables|Default|GetEnabled)
    (bind _asbp_boat_pawn (Utilities|Casting|CastToBP_BoatPawn OtherActor))
    (Default|SetNoFishingZone _asbp_boat_pawn false)
    (Default|CollapsePrompt _wbp_baitcounter)
    (Default|DisplayPrompt _wbp_baitcounter "Fish" "E")))

(event OnComponentBeginOverlap(InteractBox)
  (params (OverlappedComponent :type Primitive%20Component%20Object%20Reference) (OtherActor :type Actor%20Object%20Reference) (OtherComp :type Primitive%20Component%20Object%20Reference) (OtherBodyIndex :type Integer) (bFromSweep :type Boolean) (SweepResult :type Hit%20Result%20Structure%20%28by%20ref%29))
  ;[1 1 1] Interact With Pier
  (Variables|/Game/Blueprints/BP_FishingPlayerController.BP_FishingPlayerController_C|SetbCanInteract (Variables|Default|GetPlayer%20Controller) true)
  (Default|DisplayPrompt (Variables|/Game/UI/BoatHUD/WBP_BoatHUD.WBP_BoatHUD_C|GetWBP_BaitCounter (Variables|/Game/Blueprints/BP_FishingPlayerController.BP_FishingPlayerController_C|GetBoatHUD (Variables|Default|GetPlayer%20Controller))) "End Day" "F"))

(event OnComponentEndOverlap(InteractBox)
  (params (OverlappedComponent :type Primitive%20Component%20Object%20Reference) (OtherActor :type Actor%20Object%20Reference) (OtherComp :type Primitive%20Component%20Object%20Reference) (OtherBodyIndex :type Integer))
  ;[1 1 1] Interact With Pier
  (Variables|/Game/Blueprints/BP_FishingPlayerController.BP_FishingPlayerController_C|SetbCanInteract (Variables|Default|GetPlayer%20Controller) false)
  (Default|DisplayPrompt (Variables|/Game/UI/BoatHUD/WBP_BoatHUD.WBP_BoatHUD_C|GetWBP_BaitCounter (Variables|/Game/Blueprints/BP_FishingPlayerController.BP_FishingPlayerController_C|GetBoatHUD (Variables|Default|GetPlayer%20Controller)))))

(event EventBeginPlay
  (bind _asbp_fishing_player_controller (Utilities|Casting|CastToBP_FishingPlayerController (Game|GetPlayerController 0)))
  (Variables|Default|SetPlayer%20Controller _asbp_fishing_player_controller)
  (bind _returnvalue (Actor|GetActorOfClass "/Game/Blueprints/BP_DayNightManager.BP_DayNightManager_C"))
  (Variables|Default|SetDayNightManager _returnvalue))

(event EventTick
  (params (DeltaSeconds :type Float%20%28single-precision%29))
  (bind _spinner (Variables|Default|GetSpinner))
  (Transformation|AddLocalRotation _spinner (Math|Rotator|MakeRotator 0.0 0.0 (* DeltaSeconds 25.0)) false false)
  (bind _fraction (Default|GetCurrentTime (Variables|Default|GetDayNightManager)))
  (Transformation|SetWorldScale3D _spinner (Math|Conversions|ToVector(Float) (- 1.0 (Math|Float|Clamp(Float) (+ (/ (Math|Float|Absolute(Float) (- 1.5 _fraction)) 0.2) -0.5))))))

(fn ConstructionScript)