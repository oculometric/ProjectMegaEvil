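; BP_Buoy is an environment buoy that fakes floating with looping bob and sway motion.
; A Timeline started on BeginPlay drives the mesh's relative Z from its UpDown track and restarts itself when finished.
; Its event track picks a random tilt within a cone around world up, and each update eases the mesh rotation toward that target, scaled by delta time.
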(event EventBeginPlay
  (bind _sm_buoy (Variables|Default|GetSM_Buoy))
  (bind _updown (Timeline|Timeline Play)
    (:Update
      (Transformation|SetRelativeLocation _sm_buoy (Math|Vector|MakeVector 0.0 0.0 (- (* _updown -8e+01) 5e+01)) false false)
      (Transformation|SetRelativeRotation _sm_buoy (Math|Interpolation|Ease "EaseIn" (* (Utilities|Time|GetWorldDeltaSeconds) 3.0) (Variables|/Script/Engine.SceneComponent|GetRelativeRotation (Variables|Default|GetSM_Buoy)) (Variables|Default|GetTargetAngles) true) false false))
    (:Finished
      (Timeline|Timeline PlayFromStart))
    (:SetTargetRotation
      (Variables|Default|SetTargetAngles (Math|Rotator|MakeRotfromZX (Math|Random|RandomUnitVectorinConeinDegrees "0.000000,0.000000,1.000000" 3e+01) (Class|KismetMathLibrary|VectorRight))))))

(fn ConstructionScript)