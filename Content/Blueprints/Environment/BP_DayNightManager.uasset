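; Day/night manager that animates the sky and sun over a looping cycle and advances BP_WeeklyQuotaManager's day when each cycle ends.
; BeginPlay and SkipDay load the Day0 row of DT_DayNightCycle, start timers and apply a dynamic sky material.
; A fast timer maps cycle-timer progress to sky TimeFactor, sun rotation, and Lerp5-blended sun colour and intensity.
; GetCurrentTime exposes elapsed time and the day or night segment.
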(event Custom|UpdateSkyShader
  (bind _suncolourdawn (Variables|Default|GetSunColourDawn))
  (bind _sunpowerdawn (Variables|Default|GetSunPowerDawn))
  (bind _daycycletimer (Variables|Default|GetDayCycleTimer))
  (bind _daylengthseconds (Variables|Default|GetDayLengthSeconds))
  (bind _nightlengthseconds (Variables|Default|GetNightLengthSeconds))
  (bind _sunlight (Variables|Default|GetSunLight))
  (bind _returnvalue (Math|Conversions|ToVector(Float) _sunpowerdawn))
  (bind _returnvalue_2 (Class|KismetSystemLibrary|GetTimerElapsedTimeHandle _daycycletimer))
  (bind _lightcomponent (Variables|/Script/Engine.Light|GetLightComponent _sunlight))
  (bind _returnvalue_3 (<= _returnvalue_2 _daylengthseconds))
  (bind _returnvalue_4 (/ _returnvalue_2 _daylengthseconds))
  (bind _returnvalue_5 (- _returnvalue_2 _daylengthseconds))
  (bind _returnvalue_6 (/ _returnvalue_5 _nightlengthseconds))
  (bind _returnvalue_7 (+ _returnvalue_6 1.0))
  (bind _returnvalue_8 (Math|Float|SelectFloat _returnvalue_4 _returnvalue_7 _returnvalue_3))
  (bind _returnvalue_9 (Math|Float|%(Float) _returnvalue_8 2.0))
  (bind _returnvalue_10 (/ _returnvalue_9 2.0))
  (Rendering|Material|SetScalarParameterValue (Variables|Default|GetSkyMaterial) "TimeFactor" _returnvalue_9 :!class /Script/Engine.MaterialInstanceDynamic)
  (Transformation|SetActorRotation _sunlight (Math|Conversions|RotationFromXVector (Math|Vector|RotateVector "0.000000,0.300000,-0.900000" (Math|Rotator|MakeRotator 0.0 (* (- (* _returnvalue_9 2.0) 1.0) -9e+01) 0.0))))
  (Rendering|Components|Light|SetLightColor _lightcomponent (Math|Conversions|ToLinearColor(Vector) (Utilities|Lerp5 _suncolourdawn (Variables|Default|GetSunColourMidday) (Variables|Default|GetSunColourDusk) (Variables|Default|GetSunColourMidnight) _suncolourdawn _returnvalue_10)) true)
  (Rendering|Components|Light|SetIntensity _lightcomponent (.x (Utilities|Lerp5 _returnvalue (Math|Conversions|ToVector(Float) (Variables|Default|GetSunPowerMidday)) (Math|Conversions|ToVector(Float) (Variables|Default|GetSunPowerDusk)) (Math|Conversions|ToVector(Float) (Variables|Default|GetSunPowerMidnight)) _returnvalue _returnvalue_10))))

(event Custom|ReadDataTable
  (params (RowName :type Name))
  (bind _returnvalue (Utilities|GetDataTableRow "/Game/DataAssets/DT_DayNightCycle.DT_DayNightCycle" RowName)
    (:then
      (Utilities|FlowControl|Sequence
        (:then_0
          (Variables|Default|SetDayLengthSeconds (* (.cyclelengthseconds _returnvalue) (.dayfraction _returnvalue)))
          (Variables|Default|SetNightLengthSeconds (- (.cyclelengthseconds _returnvalue) (* (.cyclelengthseconds _returnvalue) (.dayfraction _returnvalue)))))
        (:then_1
          (Variables|Default|SetSunColourDawn (.suncolourdawn _returnvalue))
          (Variables|Default|SetSunPowerDawn (.sunpowerdawn _returnvalue)))
        (:then_2
          (Variables|Default|SetSunColourMidday (.suncolourmidday _returnvalue))
          (Variables|Default|SetSunPowerMidday (.sunpowermidday _returnvalue)))
        (:then_3
          (Variables|Default|SetSunColourDusk (.suncolourdusk _returnvalue))
          (Variables|Default|SetSunPowerDusk (.sunpowerdusk _returnvalue)))
        (:then_4
          (Variables|Default|SetSunColourMidnight (.suncolourmidnight _returnvalue))
          (Variables|Default|SetSunPowerMidnight (.sunpowermidnight _returnvalue)))))
    (:RowNotFound
      (Development|PrintString "data table row not found!!"))))

(event Custom|DayCycleFinish
  (Development|PrintString "it is now tomorrow")
  (bind _returnvalue (Actor|GetActorOfClass "/Game/Blueprints/WeeklyQuota/BP_WeeklyQuotaManager.BP_WeeklyQuotaManager_C"))
  (Default|AdvanceDay _returnvalue))

(event Custom|SkipDay
  (CallFunction|ReadDataTable "Day0")
  (Utilities|Time|SetTimerbyEvent (delegate Custom|UpdateSkyShader) 0.1 true true)
  (bind _returnvalue (Utilities|Time|SetTimerbyEvent (delegate Custom|DayCycleFinish) (+ (Variables|Default|GetDayLengthSeconds) (Variables|Default|GetNightLengthSeconds)) true))
  (Variables|Default|SetDayCycleTimer _returnvalue)
  (bind _returnvalue_2 (Rendering|Material|CreateDynamicMaterialInstance "/Game/Materials/M_SimpleSky.M_SimpleSky" "None" "None" :!class /Script/Engine.KismetMaterialLibrary))
  (bind _output_get (Variables|Default|SetSkyMaterial _returnvalue_2))
  (Rendering|Material|SetMaterial (Actor|GetComponentbyClass (Variables|Default|GetSkySphere) "/Script/Engine.StaticMeshComponent") 0 _output_get))

(event EventBeginPlay
  (CallFunction|ReadDataTable "Day0")
  (Utilities|Time|SetTimerbyEvent (delegate Custom|UpdateSkyShader) 0.1 true true)
  (bind _returnvalue (Utilities|Time|SetTimerbyEvent (delegate Custom|DayCycleFinish) (+ (Variables|Default|GetDayLengthSeconds) (Variables|Default|GetNightLengthSeconds)) true))
  (Variables|Default|SetDayCycleTimer _returnvalue)
  (bind _returnvalue_2 (Rendering|Material|CreateDynamicMaterialInstance "/Game/Materials/M_SimpleSky.M_SimpleSky" "None" "None" :!class /Script/Engine.KismetMaterialLibrary))
  (bind _output_get (Variables|Default|SetSkyMaterial _returnvalue_2))
  (Rendering|Material|SetMaterial (Actor|GetComponentbyClass (Variables|Default|GetSkySphere) "/Script/Engine.StaticMeshComponent") 0 _output_get))

(fn ConstructionScript)

(fn GetCurrentTime
  (bind _daycycletimer (Variables|Default|GetDayCycleTimer))
  (bind _returnvalue (Class|KismetSystemLibrary|GetTimerElapsedTimeHandle _daycycletimer))
  (return _returnvalue (select (> _returnvalue (Variables|Default|GetDayLengthSeconds)) "NewEnumerator1" "NewEnumerator0")))