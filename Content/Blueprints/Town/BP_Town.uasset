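; BP_Town is a town where overlapping its Box trigger opens the shop and halts the boat.
; On overlap it creates WB_ShopUI, calls ShopCreated on it, then zeroes the BP_Boat's floating-movement speed and steering and stops it immediately.
; A ShopClosed event restores speed and steering to hard-coded values.
; The overlap does not check which actor entered, and the boat is found by class lookup.
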(event OnComponentBeginOverlap(Box)
  (params (OverlappedComponent :type Primitive%20Component%20Object%20Reference) (OtherActor :type Actor%20Object%20Reference) (OtherComp :type Primitive%20Component%20Object%20Reference) (OtherBodyIndex :type Integer) (bFromSweep :type Boolean) (SweepResult :type Hit%20Result%20Structure%20%28by%20ref%29))
  (bind _output_get (Variables|Default|SetPlayer%20Ref (Game|GetPlayerController 0)))
  (bind _returnvalue (UserInterface|CreateWidget "/Game/UI/WB_ShopUI.WB_ShopUI_C" _output_get))
  (bind _output_get_2 (Variables|Default|SetShop%20UI _returnvalue))
  (Default|ShopCreated _output_get_2 _returnvalue)
  (bind _returnvalue_2 (Actor|GetActorOfClass "/Game/Blueprints/Boat/BP_Boat.BP_Boat_C"))
  (bind _returnvalue_3 (AddComponent|AddFloatingPawnMovement _returnvalue_2))
  (Variables|/Script/Engine.FloatingPawnMovement|SetMaxSpeed _returnvalue_3 0.0)
  (Variables|/Game/Blueprints/Boat/BP_Boat.BP_Boat_C|SetSteeringMultiplier _returnvalue_2 0.0)
  (Components|Movement|StopMovementImmediately _returnvalue_3))

(event Custom|Shop%20Closed
  (Variables|/Script/Engine.FloatingPawnMovement|SetMaxSpeed (stale OnComponentBeginOverlap(Box) _returnvalue_3) 1.2e+03)
  (Variables|/Game/Blueprints/Boat/BP_Boat.BP_Boat_C|SetSteeringMultiplier (stale OnComponentBeginOverlap(Box) _returnvalue_2) 15.0))

(fn ConstructionScript)