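; Boat attributes component that applies speed, armour and storage levels to the boat's max speed and mesh.
; It caches base max speed a tick after BeginPlay, and on stat updates scales it by SpeedLevel.
; A nested threshold chain picks a DT_BoatType row by propulsion and material; storage tiers share rows.
; GetName re-finds the row name by mesh match for BoatLoader to load.
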(event Custom|UpdateStats
  (Variables|/Script/Engine.FloatingPawnMovement|SetMaxSpeed (Variables|/Game/Blueprints/BP_BoatPawn.BP_BoatPawn_C|GetFloatingPawnMovement (Variables|Default|GetBoat)) (* (Variables|Default|GetSpeedLevel) (Variables|Default|GetMax%20Speed)))
  (if (Math|Boolean|ANDBoolean (>= (Variables|Default|GetSpeedLevel) 2.0) (>= (Variables|Default|GetArmourLevel) 3.0) (>= (Variables|Default|GetStorageLevel) 1.5e+02))
    (bind _returnvalue (Utilities|GetDataTableRow "/Game/DataAssets/DT_BoatType.DT_BoatType" "MetalExhaust")
      (:then
        (bind _name (CallFunction|GetName _returnvalue))
        (Default|LoadMesh (Variables|Default|GetBoatLoader) _name)))
    (else
      ;[1 1 1] 3,2,2
      (if (Math|Boolean|ANDBoolean (>= (Variables|Default|GetSpeedLevel) 2.0) (>= (Variables|Default|GetArmourLevel) 3.0) (>= (Variables|Default|GetStorageLevel) 1e+02))
        (bind _returnvalue_2 (Utilities|GetDataTableRow "/Game/DataAssets/DT_BoatType.DT_BoatType" "MetalExhaust")
          (:then
            (bind _name_2 (CallFunction|GetName _returnvalue_2))
            (Default|LoadMesh (Variables|Default|GetBoatLoader) _name_2)))
        (else
          ;[1 1 1] 3,2,1
          (if (Math|Boolean|ANDBoolean (>= (Variables|Default|GetSpeedLevel) 2.0) (>= (Variables|Default|GetArmourLevel) 3.0) (>= (Variables|Default|GetStorageLevel) 5e+01))
            (bind _returnvalue_3 (Utilities|GetDataTableRow "/Game/DataAssets/DT_BoatType.DT_BoatType" "MetalExhaust")
              (:then
                (bind _name_3 (CallFunction|GetName _returnvalue_3))
                (Default|LoadMesh (Variables|Default|GetBoatLoader) _name_3)))
            (else
              ;[1 1 1] 3,1,3
              (if (Math|Boolean|ANDBoolean (>= (Variables|Default|GetSpeedLevel) 2.0) (>= (Variables|Default|GetArmourLevel) 0.0) (>= (Variables|Default|GetStorageLevel) 1.5e+02))
                (bind _returnvalue_4 (Utilities|GetDataTableRow "/Game/DataAssets/DT_BoatType.DT_BoatType" "WoodenExhaust")
                  (:then
                    (bind _name_4 (CallFunction|GetName _returnvalue_4))
                    (Default|LoadMesh (Variables|Default|GetBoatLoader) _name_4)))
                (else
                  ;[1 1 1] 3,1,2
                  (if (Math|Boolean|ANDBoolean (>= (Variables|Default|GetSpeedLevel) 2.0) (>= (Variables|Default|GetArmourLevel) 0.0) (>= (Variables|Default|GetStorageLevel) 1e+02))
                    (bind _returnvalue_5 (Utilities|GetDataTableRow "/Game/DataAssets/DT_BoatType.DT_BoatType" "WoodenExhaust")
                      (:then
                        (bind _name_5 (CallFunction|GetName _returnvalue_5))
                        (Default|LoadMesh (Variables|Default|GetBoatLoader) _name_5)))
                    (else
                      ;[1 1 1] 3,1,1
                      (if (Math|Boolean|ANDBoolean (>= (Variables|Default|GetSpeedLevel) 2.0) (>= (Variables|Default|GetArmourLevel) 0.0) (>= (Variables|Default|GetStorageLevel) 5e+01))
                        (bind _returnvalue_6 (Utilities|GetDataTableRow "/Game/DataAssets/DT_BoatType.DT_BoatType" "WoodenExhaust")
                          (:then
                            (bind _name_6 (CallFunction|GetName _returnvalue_6))
                            (Default|LoadMesh (Variables|Default|GetBoatLoader) _name_6)))
                        (else
                          ;[1 1 1] 2,2,3
                          (if (Math|Boolean|ANDBoolean (>= (Variables|Default|GetSpeedLevel) 1.5) (>= (Variables|Default|GetArmourLevel) 3.0) (>= (Variables|Default|GetStorageLevel) 1.5e+02))
                            (bind _returnvalue_7 (Utilities|GetDataTableRow "/Game/DataAssets/DT_BoatType.DT_BoatType" "MetalEngine")
                              (:then
                                (bind _name_7 (CallFunction|GetName _returnvalue_7))
                                (Default|LoadMesh (Variables|Default|GetBoatLoader) _name_7)))
                            (else
                              ;[1 1 1] 2,2,2
                              (if (Math|Boolean|ANDBoolean (>= (Variables|Default|GetSpeedLevel) 1.5) (>= (Variables|Default|GetArmourLevel) 3.0) (>= (Variables|Default|GetStorageLevel) 1e+02))
                                (bind _returnvalue_8 (Utilities|GetDataTableRow "/Game/DataAssets/DT_BoatType.DT_BoatType" "MetalEngine")
                                  (:then
                                    (bind _name_8 (CallFunction|GetName _returnvalue_8))
                                    (Default|LoadMesh (Variables|Default|GetBoatLoader) _name_8)))
                                (else
                                  ;[1 1 1] 2,2,1
                                  (if (Math|Boolean|ANDBoolean (>= (Variables|Default|GetSpeedLevel) 1.5) (>= (Variables|Default|GetArmourLevel) 3.0) (>= (Variables|Default|GetStorageLevel) 5e+01))
                                    (bind _returnvalue_9 (Utilities|GetDataTableRow "/Game/DataAssets/DT_BoatType.DT_BoatType" "MetalEngine")
                                      (:then
                                        (bind _name_9 (CallFunction|GetName _returnvalue_9))
                                        (Default|LoadMesh (Variables|Default|GetBoatLoader) _name_9)))
                                    (else
                                      ;[1 1 1] 2,1,3
                                      (if (Math|Boolean|ANDBoolean (>= (Variables|Default|GetSpeedLevel) 1.5) (>= (Variables|Default|GetArmourLevel) 0.0) (>= (Variables|Default|GetStorageLevel) 1.5e+02))
                                        (bind _returnvalue_10 (Utilities|GetDataTableRow "/Game/DataAssets/DT_BoatType.DT_BoatType" "WoodenEngine")
                                          (:then
                                            (bind _name_10 (CallFunction|GetName _returnvalue_10))
                                            (Default|LoadMesh (Variables|Default|GetBoatLoader) _name_10)))
                                        (else
                                          ;[1 1 1] 2,1,2
                                          (if (Math|Boolean|ANDBoolean (>= (Variables|Default|GetSpeedLevel) 1.5) (>= (Variables|Default|GetArmourLevel) 0.0) (>= (Variables|Default|GetStorageLevel) 1e+02))
                                            (bind _returnvalue_11 (Utilities|GetDataTableRow "/Game/DataAssets/DT_BoatType.DT_BoatType" "WoodenEngine")
                                              (:then
                                                (bind _name_11 (CallFunction|GetName _returnvalue_11))
                                                (Default|LoadMesh (Variables|Default|GetBoatLoader) _name_11)))
                                            (else
                                              ;[1 1 1] 2,1,1
                                              (if (Math|Boolean|ANDBoolean (>= (Variables|Default|GetSpeedLevel) 1.5) (>= (Variables|Default|GetArmourLevel) 0.0) (>= (Variables|Default|GetStorageLevel) 5e+01))
                                                (bind _returnvalue_12 (Utilities|GetDataTableRow "/Game/DataAssets/DT_BoatType.DT_BoatType" "WoodenEngine")
                                                  (:then
                                                    (bind _name_12 (CallFunction|GetName _returnvalue_12))
                                                    (Default|LoadMesh (Variables|Default|GetBoatLoader) _name_12)))
                                                (else
                                                  ;[1 1 1] 1,2,3
                                                  (if (Math|Boolean|ANDBoolean (>= (Variables|Default|GetSpeedLevel) 1.0) (>= (Variables|Default|GetArmourLevel) 3.0) (>= (Variables|Default|GetStorageLevel) 1.5e+02))
                                                    (bind _returnvalue_13 (Utilities|GetDataTableRow "/Game/DataAssets/DT_BoatType.DT_BoatType" "MetalOars")
                                                      (:then
                                                        (bind _name_13 (CallFunction|GetName _returnvalue_13))
                                                        (Default|LoadMesh (Variables|Default|GetBoatLoader) _name_13)))
                                                    (else
                                                      ;[1 1 1] 1,2,2
                                                      (if (Math|Boolean|ANDBoolean (>= (Variables|Default|GetSpeedLevel) 1.0) (>= (Variables|Default|GetArmourLevel) 3.0) (>= (Variables|Default|GetStorageLevel) 1e+02))
                                                        (bind _returnvalue_14 (Utilities|GetDataTableRow "/Game/DataAssets/DT_BoatType.DT_BoatType" "MetalOars")
                                                          (:then
                                                            (bind _name_14 (CallFunction|GetName _returnvalue_14))
                                                            (Default|LoadMesh (Variables|Default|GetBoatLoader) _name_14)))
                                                        (else
                                                          ;[1 1 1] 1,2,1
                                                          (if (Math|Boolean|ANDBoolean (>= (Variables|Default|GetSpeedLevel) 1.0) (>= (Variables|Default|GetArmourLevel) 3.0) (>= (Variables|Default|GetStorageLevel) 5e+01))
                                                            (bind _returnvalue_15 (Utilities|GetDataTableRow "/Game/DataAssets/DT_BoatType.DT_BoatType" "MetalOars")
                                                              (:then
                                                                (bind _name_15 (CallFunction|GetName _returnvalue_15))
                                                                (Default|LoadMesh (Variables|Default|GetBoatLoader) _name_15)))
                                                            (else
                                                              ;[1 1 1] 1,1,3
                                                              (if (Math|Boolean|ANDBoolean (>= (Variables|Default|GetSpeedLevel) 1.0) (>= (Variables|Default|GetArmourLevel) 0.0) (>= (Variables|Default|GetStorageLevel) 1.5e+02))
                                                                (bind _returnvalue_16 (Utilities|GetDataTableRow "/Game/DataAssets/DT_BoatType.DT_BoatType" "WoodenOars")
                                                                  (:then
                                                                    (bind _name_16 (CallFunction|GetName _returnvalue_16))
                                                                    (Default|LoadMesh (Variables|Default|GetBoatLoader) _name_16)))
                                                                (else
                                                                  ;[1 1 1] 1,1,2
                                                                  (if (Math|Boolean|ANDBoolean (>= (Variables|Default|GetSpeedLevel) 1.0) (>= (Variables|Default|GetArmourLevel) 0.0) (>= (Variables|Default|GetStorageLevel) 1e+02))
                                                                    (bind _returnvalue_17 (Utilities|GetDataTableRow "/Game/DataAssets/DT_BoatType.DT_BoatType" "WoodenOars")
                                                                      (:then
                                                                        (bind _name_17 (CallFunction|GetName _returnvalue_17))
                                                                        (Default|LoadMesh (Variables|Default|GetBoatLoader) _name_17)))
                                                                    (else
                                                                      ;[1 1 1] 1,1,1
                                                                      (if (Math|Boolean|ANDBoolean (>= (Variables|Default|GetSpeedLevel) 1.0) (>= (Variables|Default|GetArmourLevel) 0.0) (>= (Variables|Default|GetStorageLevel) 5e+01))
                                                                        (bind _returnvalue_18 (Utilities|GetDataTableRow "/Game/DataAssets/DT_BoatType.DT_BoatType" "WoodenOars")
                                                                          (:then
                                                                            (bind _name_18 (CallFunction|GetName _returnvalue_18))
                                                                            (Default|LoadMesh (Variables|Default|GetBoatLoader) _name_18)))))))))))))))))))))))))))))))))))))))

(event EventBeginPlay
  (EventDispatchers|BindEventtoUpdatedStats (delegate Custom|UpdateStats))
  (Utilities|FlowControl|DelayUntilNextTick)
  (Variables|Default|SetMax%20Speed (Variables|/Script/Engine.FloatingPawnMovement|GetMaxSpeed (Variables|/Game/Blueprints/BP_BoatPawn.BP_BoatPawn_C|GetFloatingPawnMovement (Variables|Default|GetBoat)))))

(fn GetName
  (params (BoatType :type F%20Boat%20Type%20Structure))
  (bind _outrownames (DataTable|GetDataTableRowNames "/Game/DataAssets/DT_BoatType.DT_BoatType"))
  (for _array_element _outrownames
    (bind _returnvalue (Utilities|GetDataTableRow "/Game/DataAssets/DT_BoatType.DT_BoatType" _array_element)
      (:then
        (if (== (Utilities|Struct|BreakF_BoatType _returnvalue) (Utilities|Struct|BreakF_BoatType BoatType))
          (return _array_element))))))