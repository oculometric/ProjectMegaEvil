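; Boat mesh actor base that changes the boat's look to match its speed, storage and armour upgrade levels.
; An Initialise event takes the three levels, then toggles component visibility and swaps materials.
; Speed swaps oars for an engine, later adds an exhaust, and changes the top from wood to metal.
; Armour turns the base metal, and each storage level reveals another bucket.
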(event Custom|Initialise
  (params (SpeedLevel :type Integer) (StorageLevel :type Integer) (ArmourLevel :type Integer))
  (Utilities|FlowControl|Sequence
    (:then_0
      (Development|SetHiddeninGame (Variables|Default|GetSM_Exhaust) (< SpeedLevel 2) false)
      (Development|SetHiddeninGame (Variables|Default|GetSM_BoatEngine) (< SpeedLevel 1) false)
      (Development|SetHiddeninGame (Variables|Default|GetSM_BoatOar) (> SpeedLevel 0) false)
      (Rendering|Material|SetMaterial (Variables|Default|GetSM_BoatTop) 0 (select (> SpeedLevel 0) "/Game/Materials/Boat/MI_BoatMetalTop.MI_BoatMetalTop" "/Game/Materials/Boat/MI_BoatWoodTop.MI_BoatWoodTop")))
    (:then_1
      (Rendering|Material|SetMaterial (Variables|Default|GetSM_BoatBase) 0 (select (> ArmourLevel 0) "/Game/Materials/Boat/MI_BoatMetalBase.MI_BoatMetalBase" "/Game/Materials/Boat/MI_BoatWoodBase.MI_BoatWoodBase")))
    (:then_2
      (Development|SetHiddeninGame (Variables|Default|GetSM_Bucket1) (< StorageLevel 1) false)
      (Development|SetHiddeninGame (Variables|Default|GetSM_Bucket2) (< StorageLevel 2) false)
      (Development|SetHiddeninGame (Variables|Default|GetSM_Bucket3) (< StorageLevel 3) false))))

(fn ConstructionScript)