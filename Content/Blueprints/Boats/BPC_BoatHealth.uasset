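; Boat health component that tracks current and maximum health for a boat pawn and broadcasts updates when it changes.
; HealthChanged scales positive damage down by the owner's armour level with diminishing returns, lets negative amounts through as healing, then clamps the result.
; Armour comes from the boat pawn's attributes component, cached on BeginPlay as a temporary link.
; Reset and getter functions are provided, while the death check is an empty stub.
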(event Custom|HealthChanged
  (params (Health%20Change%20Amount :type Float%20%28double-precision%29))
  (bind _maxhealth (Variables|Default|GetMaxHealth))
  ;[1 1 1] Health Logic
  (bind _reduceddamage (CallFunction|ApplyDamageReduction Health%20Change%20Amount))
  (bind _output_get (Variables|Default|SetCurrentHealth (Math|Float|Clamp(Float) (- (Variables|Default|GetCurrentHealth) _reduceddamage) 0.0 _maxhealth)))
  (Default|CallEHealthUpdated _output_get _maxhealth)
  (Development|PrintString (Utilities|String|ToString(Float) _output_get))
  (CallFunction|IsDead))

(event Custom|isDead
  (if (< (Variables|Default|GetCurrentHealth) 0.0)
    _))

(event EventBeginPlay
  ;[1 0 0.2847] attach reference to attributes in boat, this is temporary
  (Variables|Default|SetBoatAttributes (Variables|/Game/Blueprints/BP_BoatPawn.BP_BoatPawn_C|GetBPC_BoatAttributes (.AsBP%20Boat%20Pawn (Utilities|Casting|CastToBP_BoatPawn (Components|GetOwner))))))

(fn ResetPlayerHealth
  (Variables|Default|SetCurrentHealth (Variables|Default|GetMaxHealth))
  (return))

(fn ApplyDamageReduction
  (params (Damage :type Float%20%28double-precision%29))
  (if (< Damage 0.0)
    (return Damage)
    (else
      (bind _rounded_value (CallFunction|RoundValue (* Damage (- 1.0 (- 1.0 (/ 1.0 (+ (* 0.5 (Variables|/Game/Blueprints/Boats/BPC_BoatAttributes.BPC_BoatAttributes_C|GetArmourLevel (Variables|Default|GetBoatAttributes))) 1.0))))) 2.0))
      (return _rounded_value))))

(fn GetHealthValues
  (return (Variables|Default|GetCurrentHealth) (Variables|Default|GetMaxHealth)))