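; Boat component for weathering damage that scales with the water depth beneath the boat.
; BeginPlay loads depth thresholds and damage settings from the fish spawning and boat weathering data tables, then starts a one-second looping timer.
; Weathering traces below the boat, buckets the hit distance by depth, and applies base damage times that band's multiplier.
; The damage timer's setup is unreachable, and the pause check uses a constant condition.
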(event Custom|Weathering
  (bind _boat (Variables|Default|GetBoat))
  (bind _returnvalue (Transformation|GetActorLocation _boat))
  (bind (_outhit _returnvalue_2) (Collision|LineTraceForObjects _returnvalue (+ _returnvalue (* (Math|Vector|NegateVector (Transformation|GetActorUpVector _boat)) "1.000000,1.000000,1500.000000")) (Utilities|Array|MakeArray "ObjectTypeQuery1") false 0 "ForOneFrame"))
  (if _returnvalue_2
    (if (> (.Distance (Collision|BreakHitResult _outhit)) (Variables|Default|GetMediumStartHeight))
      (Variables|Default|SetDepth "NewEnumerator0")
      (elif (> (.Distance (Collision|BreakHitResult _outhit)) (Variables|Default|GetDeepStartHeight))
        (Variables|Default|SetDepth "NewEnumerator1")
        (elif (> (.Distance (Collision|BreakHitResult _outhit)) (Variables|Default|GetDeepestStartHeight))
          (Variables|Default|SetDepth "NewEnumerator2")
          (else
            (Variables|Default|SetDepth "NewEnumerator3")))))
    (Game|Damage|ApplyDamage (Variables|Default|GetBoat) (* (Variables|Default|GetBaseDamage) (.Value (Utilities|Map|Find (Variables|Default|GetDepth%20Damage%20Map) (Variables|Default|GetDepth)))) 0 (Variables|Default|GetBoat))))

(event Custom|Timer
  (bind _damagetimer (Variables|Default|GetDamageTimer))
  (bind _returnvalue (Class|KismetSystemLibrary|IsTimerPausedHandle _damagetimer))
  (if (not false)
    (if (not _returnvalue)
      (Utilities|Time|PauseTimerbyHandle (Variables|Default|GetDamageTimer)))
    (elif _returnvalue
      (Utilities|Time|UnpauseTimerbyHandle (Variables|Default|GetDamageTimer)))))

(event EventBeginPlay
  (bind _returnvalue (Utilities|GetDataTableRow "/Game/DataAssets/DT_FishSpawning.DT_FishSpawning" "Row")
    (:then
      (Variables|Default|SetMediumStartHeight (.ShallowMediumTransitionDepth (Utilities|Struct|BreakS_FishSpawning _returnvalue)))
      (Variables|Default|SetDeepStartHeight (.MediumDeepTransitionDepth (Utilities|Struct|BreakS_FishSpawning _returnvalue)))
      (Variables|Default|SetDeepestStartHeight (.DeepDeepestTransitionDepth (Utilities|Struct|BreakS_FishSpawning _returnvalue)))
      (Variables|Default|SetBoat (.AsBP%20Boat%20Pawn (Utilities|Casting|CastToBP_BoatPawn (Components|GetOwner))))
      (bind _returnvalue_2 (Utilities|GetDataTableRow "/Game/DataAssets/DT_BoatWeathering.DT_BoatWeathering" "Default")
        (:then
          (Variables|Default|SetWeatheringRate (.weatheringrate _returnvalue_2))
          (Variables|Default|SetBaseDamage (.baseweatheringdamage _returnvalue_2))
          (Variables|Default|SetDepth%20Damage%20Map (.depthdamagemult _returnvalue_2))
          (Utilities|Time|SetTimerbyEvent (EventDispatchers|CreateEvent :!event Custom|Timer) 1.0 true))))))