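; Boat movement Blueprint that pushes a physics body with acceleration-change forces from player input.
; The IA_BoatMove Ongoing event scales the constant forward vector by the action value and Speed, while a raw S key press applies a reverse push at half Speed.
; Both forces target PhysicsHandle, whose only setter in this graph is disconnected; Tick is empty.
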(event Input|EnhancedActionEvents|EnhancedInputActionIA_BoatMove
  (params (ActionValue :type Float%20%28double-precision%29) (ElapsedSeconds :type Float%20%28double-precision%29) (TriggeredSeconds :type Float%20%28double-precision%29) (InputAction :type Input%20Action%20Object%20Reference :default "/Game/Input/IA_BoatMove.IA_BoatMove"))
  (:Ongoing
    (Physics|AddForce (Variables|Default|GetPhysics%20Handle) (* (Class|KismetMathLibrary|VectorForward) (* ActionValue (Variables|Default|GetSpeed))) true)))

(event EventTick
  (params (DeltaSeconds :type Float%20%28single-precision%29)))

(event Input|KeyboardEvents|S
  (params (Key :type Key%20Structure))
  (:Pressed
    (Physics|AddForce (Variables|Default|GetPhysics%20Handle) (/ (* (Math|Vector|NegateVector (Class|KismetMathLibrary|VectorForward)) (Variables|Default|GetSpeed)) 2.0) true)))