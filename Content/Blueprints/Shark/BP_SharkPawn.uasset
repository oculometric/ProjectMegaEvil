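; Shark pawn driven by an enum state machine on Tick, which wanders, reacts to the boat and makes overlapped fish flee.
; Wander lerps rotation toward random 3D targets, flipping direction components against distance and depth limits.
; Boat overlap with the agro radius starts Circle, which immediately switches to Pursue, and exit switches to ReturnToWanderRange.
; Pursue, return, attack and reset logic are empty stubs, and a debug line shows the target.
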(event OnComponentBeginOverlap(FishCollider)
  (params (OverlappedComponent :type Primitive%20Component%20Object%20Reference) (OtherActor :type Actor%20Object%20Reference) (OtherComp :type Primitive%20Component%20Object%20Reference) (OtherBodyIndex :type Integer) (bFromSweep :type Boolean) (SweepResult :type Hit%20Result%20Structure%20%28by%20ref%29))
  (bind (_asbp_fish_pawn _bsuccess) (Utilities|Casting|CastToBP_FishPawn OtherActor))
  ;[0 0.5186 1] Fish Flee Behaviour
  (if _bsuccess
    (Default|FleefromTarget _asbp_fish_pawn self)))

(event OnComponentBeginOverlap(AgroRadius)
  (params (OverlappedComponent :type Primitive%20Component%20Object%20Reference) (OtherActor :type Actor%20Object%20Reference) (OtherComp :type Primitive%20Component%20Object%20Reference) (OtherBodyIndex :type Integer) (bFromSweep :type Boolean) (SweepResult :type Hit%20Result%20Structure%20%28by%20ref%29))
  ;[1 0.00828 0] Shark Agro
  (if (and (== OtherActor (Variables|Default|GetBoat)) (Utilities|Enum|Equal(Enum) (Variables|Default|GetSharkFSM) "NewEnumerator0"))
    (CallFunction|SwitchState "NewEnumerator3")))

(event OnComponentEndOverlap(AgroRadius)
  (params (OverlappedComponent :type Primitive%20Component%20Object%20Reference) (OtherActor :type Actor%20Object%20Reference) (OtherComp :type Primitive%20Component%20Object%20Reference) (OtherBodyIndex :type Integer))
  ;[1 0.1071 0.09716] Shark de-agro
  (if (and (== OtherActor (Variables|Default|GetBoat)) (not (Utilities|Enum|Equal(Enum) (Variables|Default|GetSharkFSM) "NewEnumerator0")))
    (CallFunction|SwitchState "NewEnumerator4")))

(event Custom|BeginSharkBehaviour
  ;[1 1 1] Starts SharkBehaviour - to be called each day
  (CallFunction|ResetSharkState)
  (CallFunction|SwitchState "NewEnumerator0"))

(event EventBeginPlay
  ;[0 1 0.3169] Initialise Shark
  (bind _returnvalue (Actor|GetActorOfClass "/Game/Blueprints/BP_DayNightManager.BP_DayNightManager_C"))
  (Variables|Default|SetDayNightCycle _returnvalue)
  (Variables|Default|SetSpawnPosition (Transformation|GetActorLocation))
  (bind _returnvalue_2 (Actor|GetActorOfClass "/Game/Blueprints/BP_BoatPawn.BP_BoatPawn_C"))
  (Variables|Default|SetBoat _returnvalue_2)
  (CallFunction|BeginSharkBehaviour))

(event EventTick
  (params (DeltaSeconds :type Float%20%28single-precision%29))
  ;[1 1 1] Runs FSM
  (CallFunction|FSMLogic)
  (Rendering|Debug|DrawDebugLine :LineStart (Transformation|GetActorLocation) :LineEnd (Variables|Default|GetTargetPosition))
  (Variables|Default|SetDIstance (Math|Vector|VectorLength (Transformation|GetActorLocation))))

(fn ConstructionScript)

(fn FSMLogic
  (switch Utilities|FlowControl|Switch|SwitchonE_SharkFSM (Variables|Default|GetSharkFSM)
    (:NewEnumerator0
      (CallFunction|WanderState))
    (:NewEnumerator1
      (CallFunction|PursuitState))
    (:NewEnumerator3
      (CallFunction|CirclePlayerState))
    (:NewEnumerator4
      (CallFunction|ReturntoWanderRadiusState))
    (:NewEnumerator5
      _))
  (return))

(fn SwitchState
  (params (New%20State :type E_SharkFSM%20Enum :default "NewEnumerator0"))
  (bind _output_get (Variables|Default|SetSharkFSM New%20State))
  (switch Utilities|FlowControl|Switch|SwitchonE_SharkFSM _output_get
    (:NewEnumerator0
      (CallFunction|FindWanderLocation))
    (:NewEnumerator1
      (Variables|Default|SetTargetPosition (Transformation|GetActorLocation (Variables|Default|GetBoat))))
    (:NewEnumerator3
      _)
    (:NewEnumerator4
      _)
    (:NewEnumerator5
      _))
  (return))

(fn WanderState
  (if (<= (Math|Vector|Distance(Vector) (Transformation|GetWorldLocation (Variables|Default|GetSharkCollider)) (Variables|Default|GetTargetPosition)) (Variables|Default|GetAcceptanceRadius))
    (CallFunction|FindWanderLocation))
  (CallFunction|MovetoTargetPosition)
  (return))

(fn AttackState)

(fn PursuitState)

(fn CirclePlayerState
  (if true
    (CallFunction|SwitchState "NewEnumerator1")
    (else
      (CallFunction|HandleMovetoVector (Math|Vector|CrossProduct (Math|Vector|Normalize (* (- (Transformation|GetActorLocation (Variables|Default|GetBoat)) (Transformation|GetActorLocation)) "1.000000,1.000000,0.000000")) "0.000000,0.000000,1.000000"))))
  (return))

(fn ReturntoWanderRadiusState)

(fn ResetSharkState)

(fn UpdateRadi
  (Components|Sphere|SetSphereRadius (Variables|Default|GetAgroRadius) 0.0 true))

(fn MovetoTargetPosition
  (if (Utilities|Operators|EqualEqual (Transformation|GetActorRotation) (Math|Rotator|FindLookatRotation (Transformation|GetActorLocation) (Variables|Default|GetTargetPosition)) 0.1)
    _
    (else
      (CallFunction|HandleRotation)))
  (CallFunction|HandleMovement))

(fn FindWanderLocation
  (bind _returnvalue (Math|Random|RandomUnitVector))
  (bind _returnvalue_2 (Transformation|GetActorLocation))
  (bind _wanderradius (Variables|Default|GetWanderRadius))
  (bind _returnvalue_3 (* _returnvalue _wanderradius "1.000000,1.000000,0.100000"))
  (bind _returnvalue_4 (+ _returnvalue_3 _returnvalue_2))
  (bind _z (Math|Vector|BreakVector _returnvalue_4))
  (bind _returnvalue_5 (Math|Vector|VectorLength _returnvalue_4))
  (Variables|Default|SetTargetPosition (+ (* (* _returnvalue (* (Math|Vector|SelectVector "-1.000000,-1.000000,1.000000" "1.000000,1.000000,1.000000" (Class|KismetMathLibrary|XORBoolean (> _returnvalue_5 (Variables|Default|GetMaxHubWanderDist)) (< _returnvalue_5 (Variables|Default|GetMinWanderDistance)))) (Math|Vector|SelectVector "1.000000,1.000000,-1.000000" "1.000000,1.000000,1.000000" (Class|KismetMathLibrary|XORBoolean (> _z 0.0) (< _z -7e+02))))) (Variables|Default|GetWanderRadius) "1.000000,1.000000,0.100000") (Transformation|GetActorLocation)))
  (return))

(fn HandleMovement
  (Transformation|SetActorLocation (+ (* (Transformation|GetActorForwardVector) (* (Utilities|Time|GetWorldDeltaSeconds) (Variables|Default|GetSpeed))) (Transformation|GetActorLocation)) false false))

(fn HandleRotation
  (Transformation|SetActorRotation (Math|Rotator|Lerp(Rotator) (Transformation|GetActorRotation) (Math|Rotator|FindLookatRotation (Transformation|GetActorLocation) (Variables|Default|GetTargetPosition)) (* (Utilities|Time|GetWorldDeltaSeconds) 2.0) true)))

(fn HandleMovetoVector
  (params (Input%20Vector :type Vector))
  (bind _returnvalue (Transformation|GetActorLocation))
  (bind _returnvalue_2 (Utilities|Time|GetWorldDeltaSeconds))
  (bind _speed (Variables|Default|GetSpeed))
  (bind _returnvalue_3 (* _returnvalue_2 _speed 18.0))
  (bind _returnvalue_4 (* Input%20Vector _returnvalue_3))
  (bind _returnvalue_5 (+ _returnvalue_4 _returnvalue))
  (Transformation|SetActorLocation _returnvalue_5 false false)
  (Transformation|SetActorRotation (Math|Rotator|FindLookatRotation (Transformation|GetActorLocation) _returnvalue_5)))