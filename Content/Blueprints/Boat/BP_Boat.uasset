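; Player-driven boat pawn that carries a fisher character and lets the player switch over to control it.
; On BeginPlay it spawns BP_FisherTest, attaches it to FisherAttachPoint and passes it a boat reference.
; Enhanced Input drives throttle, yaw steering and timeline-eased, clamped spring-arm zoom, while a Q key event creates the shop widget.
; Switching perspective possesses the fisher and swaps the boat mapping context for the fishing one.
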(event Input|EnhancedActionEvents|EnhancedInputActionIA_Accelerate
  (params (ActionValue :type Float%20%28double-precision%29) (ElapsedSeconds :type Float%20%28double-precision%29) (TriggeredSeconds :type Float%20%28double-precision%29) (InputAction :type Input%20Action%20Object%20Reference :default "/Game/Blueprints/Boat/Input/IA_Accelerate.IA_Accelerate"))
  ;[1 1 1] Forward/Backward Movement
  (Pawn|Input|AddMovementInput (Math|Vector|RotateVector (Math|Vector|MakeVector ActionValue 0.0 0.0) (Transformation|GetActorRotation)) (* (Variables|Default|GetMovementMultiplier) (Utilities|Time|GetWorldDeltaSeconds)) true))

(event Input|EnhancedActionEvents|EnhancedInputActionIA_Steer
  (params (ActionValue :type Float%20%28double-precision%29) (ElapsedSeconds :type Float%20%28double-precision%29) (TriggeredSeconds :type Float%20%28double-precision%29) (InputAction :type Input%20Action%20Object%20Reference :default "/Game/Blueprints/Boat/Input/IA_Steer.IA_Steer"))
  ;[1 1 1] Left/Right Turning
  (Pawn|Input|AddControllerYawInput (* ActionValue (Variables|Default|GetSteeringMultiplier) (Utilities|Time|GetWorldDeltaSeconds))))

(event Input|EnhancedActionEvents|EnhancedInputActionIA_Zoom
  (params (ActionValue :type Float%20%28double-precision%29) (ElapsedSeconds :type Float%20%28double-precision%29) (TriggeredSeconds :type Float%20%28double-precision%29) (InputAction :type Input%20Action%20Object%20Reference :default "/Game/Blueprints/Boat/Input/IA_Zoom.IA_Zoom"))
  ;[1 1 1] Camera Zoom
  (if (not (Variables|Default|GetZoomInProgress?))
    (Variables|Default|SetZoomInProgress? true)
    (bind _alpha (Timeline|Zoom PlayFromStart)
      (:Update
        (Variables|/Script/Engine.SpringArmComponent|SetTargetArmLength (Variables|Default|GetSpringArm) (Math|Float|Lerp (Variables|/Script/Engine.SpringArmComponent|GetTargetArmLength (Variables|Default|GetSpringArm)) (Math|Float|Clamp(Float) (- (Variables|/Script/Engine.SpringArmComponent|GetTargetArmLength (Variables|Default|GetSpringArm)) (* ActionValue (Variables|Default|GetZoomMultiplier))) (Variables|Default|GetMinCamLength) (Variables|Default|GetMaxCamLength)) _alpha)))
      (:Finished
        (Variables|Default|SetZoomInProgress? false)))))

(event Input|EnhancedActionEvents|EnhancedInputActionIA_SwitchPerspective
  (params (ActionValue :type Boolean) (ElapsedSeconds :type Float%20%28double-precision%29) (TriggeredSeconds :type Float%20%28double-precision%29) (InputAction :type Input%20Action%20Object%20Reference :default "/Game/Blueprints/Boat/Input/IA_SwitchPerspective.IA_SwitchPerspective"))
  (bind _returnvalue (Game|GetPlayerController 0))
  (bind _returnvalue_2 (PlayerController|LocalPlayerSubsystems|GetEnhancedInputLocalPlayerSubsystem _returnvalue))
  ;[1 1 1] Change to Fisher Perspective
  (Utilities|IsValid _returnvalue
    (:Is%20Valid
      (Pawn|Possess _returnvalue (Variables|Default|GetFisher))
      (Utilities|IsValid _returnvalue_2
        (:Is%20Valid
          (Input|RemoveMappingContext _returnvalue_2 "/Game/Blueprints/Boat/Input/IMC_Boat.IMC_Boat" "(bIgnoreAllPressedKeysUntilRelease=True,bForceImmediately=False,bNotifyUserSettings=False)")
          (Input|AddMappingContext _returnvalue_2 "/Game/Blueprints/FishingTest/Control/IMC_Fishing.IMC_Fishing" 0 "(bIgnoreAllPressedKeysUntilRelease=True,bForceImmediately=False,bNotifyUserSettings=False)"))))))

(event EventBeginPlay
  (bind _fisherattachpoint (Variables|Default|GetFisherAttachPoint))
  ;[1 1 1] Spawn Fisher
  (bind _returnvalue (Game|SpawnActorfromClass "/Game/Blueprints/FishingTest/BP_FisherTest.BP_FisherTest_C" (Transformation|GetWorldTransform _fisherattachpoint) "AlwaysSpawn" "MultiplyWithRoot" 0 0))
  (bind _output_get (Variables|Default|SetFisher _returnvalue))
  (Transformation|AttachComponentToComponent _output_get _fisherattachpoint "None" "SnapToTarget" "SnapToTarget" "SnapToTarget" true)
  (Variables|/Game/Blueprints/FishingTest/BP_FisherTest.BP_FisherTest_C|SetBoat _output_get self))

(event Input|KeyboardEvents|Q
  (params (Key :type Key%20Structure :default "None"))
  (:Pressed
    (bind _returnvalue (UserInterface|CreateWidget "/Game/UI/WB_ShopUI.WB_ShopUI_C" (Game|GetPlayerController 0)))
    (Default|ShopCreated _returnvalue _returnvalue)))

(fn ConstructionScript)