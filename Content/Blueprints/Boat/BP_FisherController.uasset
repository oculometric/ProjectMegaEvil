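; Player controller for the fishing boat game that adds the boat input mapping, runs the pause menu and tracks a weekly earnings quota.
; Earnings adds income to the quota struct, and AdvanceDay steps days, checking the quota at week's end over four weeks.
; Success raises week and quota without resetting day or earnings, while failure restarts the week.
; Debug keys trigger both functions, with feedback via PrintString.
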(event Custom|Weekly%20Quota%20Message
  (bind _weeklyquota (Variables|Default|GetWeeklyQuota))
  (bind (_weeklyquota_2 _currentday _currentweek _daysoftheweek) (Utilities|Struct|BreakS_WeeklyQuota _weeklyquota))
  ;[1 1 1] Presents the Day, The week and the current earnings.
  (Development|PrintString (Utilities|String|Append "The day is: " (Utilities|Array|Get(acopy) _daysoftheweek _currentday) ", The week is: " (Utilities|String|ToString(Integer) _currentweek) ", The weekly quota is:  " (Utilities|String|ToString(Integer) _weeklyquota_2)) true true "(R=0.000000,G=0.660000,B=1.000000,A=1.000000)" 5.0))

(event Input|EnhancedActionEvents|EnhancedInputActionIA_Pause
  (params (ActionValue :type Boolean) (ElapsedSeconds :type Float%20%28double-precision%29) (TriggeredSeconds :type Float%20%28double-precision%29) (InputAction :type Input%20Action%20Object%20Reference :default "/Game/Input/IA_Pause.IA_Pause"))
  (bind _pausemenu (Variables|Default|GetPauseMenu))
  (:Started
    (Widget|SetVisibility _pausemenu "Visible")
    (Game|SetGamePaused true)
    (Input|SetInputModeUIOnly self _pausemenu "DoNotLock" true)
    (Variables|Default|SetbShowMouseCursor true)))

(event EventBeginPlay
  (bind _returnvalue (PlayerController|LocalPlayerSubsystems|GetEnhancedInputLocalPlayerSubsystem))
  (Utilities|IsValid _returnvalue
    (:Is%20Valid
      (Input|AddMappingContext _returnvalue "/Game/Blueprints/Boat/Input/IMC_Boat.IMC_Boat" 0 "(bIgnoreAllPressedKeysUntilRelease=True,bForceImmediately=False,bNotifyUserSettings=False)")
      (bind _returnvalue_2 (UserInterface|CreateWidget "/Game/UI/WBP_Pause.WBP_Pause_C" self))
      (bind _output_get (Variables|Default|SetPauseMenu _returnvalue_2))
      (UserInterface|Viewport|AddtoViewport _output_get 0)
      (Widget|SetVisibility _output_get "Hidden")
      (CallFunction|WeeklyQuotaMessage))))

(event Input|KeyboardEvents|8
  (params (Key :type Key%20Structure :default "None"))
  ;[1 1 1] Weekly Quota Test
  (:Pressed
    (CallFunction|AdvanceDay)))

(event Input|KeyboardEvents|7
  (params (Key :type Key%20Structure :default "None"))
  ;[1 1 1] Weekly Quota Test
  (:Pressed
    (CallFunction|Earnings 2000)
    (Development|PrintString (Utilities|String|ToString(Integer) (.CurrentEarnings (Utilities|Struct|BreakS_WeeklyQuota (Variables|Default|GetWeeklyQuota)))))))

(fn ConstructionScript)

(fn AdvanceDay
  (bind _weeklyquota (Variables|Default|GetWeeklyQuota))
  (bind _weeklyquota_2 (Variables|Default|GetWeeklyQuota))
  (bind (_weeklyquota_3 _currentearnings _currentday _maxdays _currentweek _daysoftheweek) (Utilities|Struct|BreakS_WeeklyQuota _weeklyquota))
  (bind _currentweek_2 (Utilities|Struct|BreakS_WeeklyQuota _weeklyquota_2))
  ;[1 1 1] Keeps track of what day it is (Using day/night cycle made by Jacob) Checks everytime a new day has happened if they have met their weekly quota.
  (if (<= _currentweek 4)
    (Development|PrintString (Utilities|Array|Get(acopy) _daysoftheweek (- _currentday -1)))
    (if (> _currentday _maxdays)
      (if (>= _currentearnings _weeklyquota_3)
        (Development|PrintString "Quota Met!")
        ;;[1 1 1] Resets the day back to 1 (Monday) Resets current earnings so the player has a harder challenge (I assume actual money will be stored elsewhere) Increments the week and sets weekly quota to x by what week it is (Placeholder)
        (bind _result (Math|Integer|IncrementInt _currentweek)
          (:%20%20
            (Utilities|Struct|SetmembersinS_WeeklyQuota _weeklyquota_2 (* _result _weeklyquota_3) 0 0 _result)))
        (else
          (Development|PrintString "Quota Not Met!")
          ;;[1 1 1] Resets the week (For now)
          (Utilities|Struct|SetmembersinS_WeeklyQuota (Variables|Default|GetWeeklyQuota))))
      (if (<= _currentweek_2 4)
        (Development|PrintString (Utilities|String|Append "Your new weekly quota: " (Utilities|String|ToString(Integer) _weeklyquota_3)) true true "(R=1.000000,G=0.000000,B=0.026310,A=1.000000)" 5.0)
        (Development|PrintString (Utilities|String|Append "Week: " (Utilities|String|ToString(Integer) _currentweek_2)) true true "(R=0.218262,G=0.219380,B=0.776042,A=1.000000)" 5.0))
      (else
        (Math|Integer|IncrementInt _currentday)))
    (else
      (Development|PrintString "4 weeks done!"))))

(fn Earnings
  (params (NewEarnings :type Integer))
  (bind _weeklyquota (Variables|Default|GetWeeklyQuota))
  ;[1 1 1] Can be called to update the earnings for the weekly quota.
  (Utilities|Struct|SetmembersinS_WeeklyQuota _weeklyquota (+ (Utilities|Struct|BreakS_WeeklyQuota _weeklyquota) NewEarnings)))