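; BP_WeeklyQuotaManager tracks days, weeks and earnings against a weekly quota that rises linearly with the week index.
; NextDay optionally skips the day through DayNightManager, then at week's end either advances the week or resets it on a missed quota.
; Event dispatchers signal quota met, quota failed and game completion after the last week.
; The UI widget passed into Initialise is refreshed directly as earnings, days and weeks change.
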(event Custom|NextDay
  (params (Skipped :type Boolean))
  (if Skipped
    (Default|SkipDay (Variables|Default|GetDayNightManager)))
  (bind _result (Math|Integer|IncrementInt (Variables|Default|GetDayIndex))
    (:%20%20
      (if (>= _result (Variables|Default|GetDaysPerWeek))
        (if (>= (Variables|Default|GetCurrentWeekEarned) (Variables|Default|GetCurrentWeekQuota))
          (Default|CallQuotaMet)
          (CallFunction|NextWeek)
          (else
            (Default|CallQuotaFailed)
            (CallFunction|ResetWeek)))
        (else
          (CallFunction|UpdateUI))))))

(event Custom|CalculateQuota
  (Variables|Default|SetCurrentWeekQuota (+ (* (Variables|Default|GetWeekIndex) 250) 500)))

(event Custom|ResetWeek
  (Variables|Default|SetDayIndex 0)
  (Variables|Default|SetCurrentWeekEarned 0)
  (CallFunction|UpdateUI))

(event Custom|Initialise
  (params (UI :type WBP%20Boat%20HUD%20Object%20Reference))
  ;[1 1 1] Initalises UI
  (Variables|Default|SetWeekly%20Quota%20UI UI)
  (CallFunction|CalculateQuota)
  (CallFunction|UpdateUI))

(event Custom|AddEarnings
  (params (Amount :type Integer))
  (Variables|Default|SetCurrentWeekEarned (+ Amount (Variables|Default|GetCurrentWeekEarned)))
  (CallFunction|UpdateUI))

(event Custom|NextWeek
  (Variables|Default|SetDayIndex 0)
  (bind _result (Math|Integer|IncrementInt (Variables|Default|GetWeekIndex))
    (:%20%20
      (if (>= _result (Variables|Default|GetWeeksPerGame))
        (Default|CallGameCompleted))
      (Variables|Default|SetCurrentWeekEarned 0)
      (CallFunction|CalculateQuota)
      (CallFunction|UpdateUI))))

(event Custom|UpdateUI
  (bind _weekly_quota_ui (Variables|Default|GetWeekly%20Quota%20UI))
  ;[1 1 1] Updates UI
  (Utilities|FlowControl|Sequence
    (:then_0
      (Default|UpdateEarnings _weekly_quota_ui (Variables|Default|GetCurrentWeekEarned))
      (Default|UpdateQuota _weekly_quota_ui (Variables|Default|GetCurrentWeekQuota)))
    (:then_1
      (Default|UpdateDays _weekly_quota_ui (Variables|Default|GetDayIndex) (Variables|Default|GetDaysPerWeek))
      (Default|UpdateWeeks _weekly_quota_ui (Variables|Default|GetWeekIndex)))))

(fn ConstructionScript)