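; Player boat pawn steered with the mouse, with an early fishing state and debug drawing.
; Until fishing, Tick turns the collider toward the cursor, found by intersecting a camera-to-mouse line with a horizontal plane at boat height.
; Right click adds Speed-scaled force along the mouse ray if its deprojected origin is near the boat in XY.
; Left click sets IsFishing, never cleared here, and draws a debug arrow.
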(event EventTick
  (params (DeltaSeconds :type Float%20%28single-precision%29))
  (bind _returnvalue (Transformation|GetActorLocation))
  (bind _cameraman (Variables|Default|GetCameraMan))
  (bind _playercontroller (Variables|Default|GetPlayerController))
  (bind _returnvalue_2 (Transformation|GetActorLocation _cameraman))
  (bind (_worldlocation _worlddirection) (Game|Player|ConvertMouseLocationToWorldSpace _playercontroller))
  (bind _returnvalue_3 (* _worlddirection 5e+03))
  (bind _returnvalue_4 (+ _worldlocation _returnvalue_3))
  (bind _intersection (Class|KismetMathLibrary|LinePlaneIntersectionOriginNormal _returnvalue_2 _returnvalue_4 _returnvalue "0.000000,0.000000,1.000000"))
  ;[1 1 1] Boat Rotation
  (if (not (Variables|Default|GetisFishing))
    (Transformation|SetWorldRotation (Variables|Default|GetCollider) (Math|Rotator|FindLookatRotation _returnvalue _intersection) false false)
    (Rendering|Debug|DrawDebugSphere _intersection 25.0 8 "(R=1.000000,G=1.000000,B=1.000000,A=1.000000)" 0.0)))

(event EventBeginPlay
  ;[1 1 1] Initialise variables
  (Variables|Default|SetCameraMan (Game|GetPlayerCameraManager 0))
  (Variables|Default|SetPlayerController (Game|GetPlayerController 0)))

(event Input|MouseEvents|RightMouseButton
  (params (Key :type Key%20Structure :default "None"))
  (bind _returnvalue (Transformation|GetActorLocation))
  (bind _playercontroller (Variables|Default|GetPlayerController))
  (bind (_worldlocation _worlddirection) (Game|Player|ConvertMouseLocationToWorldSpace _playercontroller))
  (:Pressed
    (if (<= (Math|Vector|Distance(Vector) (Math|Vector|MakeVector (.x _returnvalue) (.y _returnvalue) 0.0) (Math|Vector|MakeVector (.x _worldlocation) (.y _worldlocation) 0.0)) 3e+01)
      (Physics|AddForce (Variables|Default|GetCollider) (* (Math|Vector|Normalize _worlddirection) (Variables|Default|GetSpeed)) "None" false))))

(event Input|MouseEvents|LeftMouseButton
  (params (Key :type Key%20Structure :default "None"))
  (:Pressed
    (Variables|Default|SetisFishing true)
    (Rendering|Debug|DrawDebugArrow :LineStart (Transformation|GetActorLocation) :LineEnd (Math|Vector|ProjectVectorontoPlane (.WorldLocation (Game|Player|ConvertMouseLocationToWorldSpace (Variables|Default|GetPlayerController))) "0, 0, 0") :ArrowSize 1.0 :Duration 2.0 :Thickness 0.1)))

(fn ConstructionScript)